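; Helper pivot actor for the bulk icon generator that lets a capture mesh actor rotate around its center of mass.
; AttachMesh unhides the mesh, moves this actor to its center of mass (bounds origin for skeletal meshes), matches rotation, attaches it, then moves both to the mesh's original location.
; DetachMesh releases the mesh, puts the attached one at the pivot's location and zeroes the pivot's rotation.
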(fn `AttachMesh`
  (params (Mesh :type "/Game/BulkIconGenerator/Blueprints/CaptureActor_BP Object Reference (by ref)"))
  (if (not (== Mesh (`self.AttachedCaptureActor`)))
    ;[1 1 1] Remember the original transform
    (set `self.OldActorLocation` (`self.K2_GetActorLocation` Mesh))
    (set `self.OldActorRotation` (`self.K2_GetActorRotation` Mesh))
    (bind _output_get (set `self.AttachedCaptureActor` Mesh))
    (`self.SetActorHiddenInGame` _output_get false)
    (`self.K2_SetActorLocation` (select `bool` (== (`SkinnedMeshComponent.SkeletalMesh` (`/Game/BulkIconGenerator/Blueprints/CaptureActor_BP.SkeletalMesh` Mesh)) null) :`false` (`self.GetActorBounds` Mesh false) :`true` (`PrimitiveComponent.GetCenterOfMass` (`/Game/BulkIconGenerator/Blueprints/CaptureActor_BP.StaticMesh` Mesh) "None"))) ; Set center of COM actor location to the COM location of the mesh
    (`self.K2_SetActorRotation` (`self.OldActorRotation`)) ; Apply the rotation of Mesh
    (`self.K2_AttachToActor` (`self.AttachedCaptureActor`) self "None" "KeepWorld" "KeepWorld" "KeepWorld" true) ; Finally attach the mesh to the COM actor - pivot will now be at the COM
    (`self.K2_SetActorLocation` (`self.OldActorLocation`)) ; Set COM actor location the original location
  ))

(fn `DetachMesh`
  (params (Mesh :type "/Game/BulkIconGenerator/Blueprints/CaptureActor_BP Object Reference (by ref)"))
  ;[1 1 1] Detach the current mesh and set it's transform to the one it had before attaching
  (`/Engine/EditorBlueprintResources/StandardMacros.IsValid` Mesh
    (:`Is Valid`
      (`self.K2_DetachFromActor` Mesh "KeepWorld" "KeepWorld" "KeepWorld")
      (if (== (`self.AttachedCaptureActor`) Mesh)
        (`self.K2_SetActorLocation` Mesh (`self.K2_GetActorLocation`) false false))
      (`self.K2_SetActorRotation` (struct))
      (set `self.AttachedCaptureActor` null))))

(fn `UserConstructionScript`)