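; Inventory combine rule for the Remington 870 rifle that decides what happens when another item is combined with it.
; It extends a parent CombineItems and switches on the slave item's ID, accepting only the shellbox and rejecting everything else.
; A shellbox triggers CombineMag, which runs BasicCharge to load the weapon.
; On success, the master item's actor bridge syncs the observable weapon with its item data.
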(fn `CombineItems`
  (params (MasterItemIndex :type Integer) (SlaveItemIndex :type Integer) (BP_InventoryComonent :type "/Game/Blueprints/Components/Player/BP_InventoryComponent Object Reference"))
  (returns (CombineSucceeded :type Boolean))
  (locals (L_CombineSucceded :type Boolean :default false))
  (`parent.CombineItems` MasterItemIndex SlaveItemIndex BP_InventoryComonent)
  (`|ExecutionSequence`
    (:`then_0`
      (switch `string` (`.ID_33_C85DBAA343F73909462E21B0374A3722` (break `/Game/Data/Structs/S_InventoryItemData` (`/Game/Blueprints/Components/Player/BP_InventoryComponent.GetItem` (`self.BP_InventoryComponent`) (`self.SlaveItemIndex`))))
        (:`Default`
          (return false))
        (:`item_shellbox`
          (bind _combinesucceded (`self.CombineMag`))
          (set `local.L_CombineSucceded` _combinesucceded))))
    (:`then_1`
      (if (`local.L_CombineSucceded`)
        (`/Game/Blueprints/Inventory/ActorBridges/BP_Base_ActorBridge.SyncObservableWithItemData` (`.ActorBridge_46_C59038FE4D701770074A409246A41738` (break `/Game/Data/Structs/S_InventoryItemData` (`/Game/Blueprints/Components/Player/BP_InventoryComponent.GetItem` (`self.BP_InventoryComponent`) (`self.MasterItemIndex`)))))
        (return (`local.L_CombineSucceded`))))))

(fn `CombineMag`
  (returns (CombineSucceded :type Boolean))
  (bind _combinesucceeded (`self.BasicCharge`))
  (return _combinesucceeded))