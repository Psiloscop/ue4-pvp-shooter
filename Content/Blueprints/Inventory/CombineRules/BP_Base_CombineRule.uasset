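; Base combine rule for inventory items, covering the merge of a slave item into a master item.
; CombineItems stores both item indices and the inventory component, then returns false by default.
; BasicCharge is a reusable helper that moves slave charge into the master, capped by the master's remaining ChargeLimit.
; It adjusts the slave's amount and charge, writes both items back through RewriteItem and reports success.
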(fn `BasicCharge`
  (returns (CombineSucceeded :type Boolean))
  (locals (L_Amount :type Integer :default 0) (L_Charge :type Integer) (L_MasterItemData :type "/Game/Data/Structs/S_InventoryItemData Structure") (L_SlaveItemData :type "/Game/Data/Structs/S_InventoryItemData Structure"))
  (bind (_id _name _description _type _image _cells _placement _isstackable _chargelimit _charge) (break `/Game/Data/Structs/S_InventoryItemData` (`local.L_SlaveItemData`)))
  (bind (_id_2 _name_2 _description_2 _type_2 _image_2 _cells_2 _placement_2 _isstackable_2 _chargelimit_2 _charge_2) (break `/Game/Data/Structs/S_InventoryItemData` (`local.L_MasterItemData`)))
  (bind (_id_3 _name_3 _description_3 _type_3 _image_3 _cells_3 _placement_3 _isstackable_3 _chargelimit_3 _charge_3 _amount) (break `/Game/Data/Structs/S_InventoryItemData` (`local.L_SlaveItemData`)))
  (bind (_id_4 _name_4 _description_4 _type_4 _image_4 _cells_4 _placement_4 _isstackable_4 _chargelimit_4 _charge_4 _amount_2) (break `/Game/Data/Structs/S_InventoryItemData` (`local.L_SlaveItemData`)))
  (bind (_out _found) (`/Game/Blueprints/Components/Player/BP_InventoryComponent.GetItem` (`self.BP_InventoryComponent`) (`self.SlaveItemIndex`)))
  (bind (_out_2 _found_2) (`/Game/Blueprints/Components/Player/BP_InventoryComponent.GetItem` (`self.BP_InventoryComponent`) (`self.MasterItemIndex`)))
  (bind _returnvalue (- _chargelimit_2 _charge_2))
  (bind _returnvalue_2 (* _charge_3 _amount))
  (bind _returnvalue_3 (`KismetMathLibrary.SelectInt` (`KismetMathLibrary.SelectInt` _amount _returnvalue (< _amount _returnvalue)) (/ _returnvalue _charge_3) (== _charge_3 1)))
  (bind _returnvalue_4 (`KismetMathLibrary.SelectInt` 0 _returnvalue_3 (< _returnvalue_3 0)))
  (set `local.L_MasterItemData` _out_2)
  (set `local.L_SlaveItemData` _out)
  (if (and _found_2 _found)
    (if (> (`.Charge_12_3F5CFC6849447618911FE689586EBF3B` (break `/Game/Data/Structs/S_InventoryItemData` (`local.L_SlaveItemData`))) 0)
      (`|ExecutionSequence`
        (:`then_0`
          ;[1 1 1] Calculate quantity for both charge and amount to decrease
          (set `local.L_Amount` (`KismetMathLibrary.SelectInt` _amount _returnvalue_4 (< _amount _returnvalue_4)))
          (set `local.L_Charge` (`KismetMathLibrary.SelectInt` _returnvalue_2 _returnvalue (< _returnvalue_2 _returnvalue))))
        (:`then_1`
          ;[1 1 1] Increse master's both amount and charge
          (setmembers `/Game/Data/Structs/S_InventoryItemData` :`StructRef` (`local.L_MasterItemData`) :`Charge` (+ (`local.L_Charge`) (`.Charge_12_3F5CFC6849447618911FE689586EBF3B` (break `/Game/Data/Structs/S_InventoryItemData` (`local.L_MasterItemData`))))))
        (:`then_2`
          ;[1 1 1] Descrease both charge and amount from slave
          (setmembers `/Game/Data/Structs/S_InventoryItemData` :`StructRef` (`local.L_SlaveItemData`) :`Amount` (- (`.Amount_16_1F1E155B4AA399D443274FA1A73C83C4` (break `/Game/Data/Structs/S_InventoryItemData` (`local.L_SlaveItemData`))) (`local.L_Amount`)))
          (if (< (`local.L_Charge`) _chargelimit)
            (setmembers `/Game/Data/Structs/S_InventoryItemData` :`StructRef` (`local.L_SlaveItemData`) :`Charge` (- _charge (`local.L_Charge`)))))
        (:`then_3`
          ;[1 1 1] Set slave item amount to zero if charge is zero
          (if (and (== _charge_4 0) (== _amount_2 1))
            (setmembers `/Game/Data/Structs/S_InventoryItemData` :`StructRef` (`local.L_SlaveItemData`) :`Amount` 0)))
        (:`then_4`
          ;[1 1 1] Update itemdata
          (`/Game/Blueprints/Components/Player/BP_InventoryComponent.RewriteItem` (`self.BP_InventoryComponent`) (`self.MasterItemIndex`) (`local.L_MasterItemData`))
          (`/Game/Blueprints/Components/Player/BP_InventoryComponent.RewriteItem` (`self.BP_InventoryComponent`) (`self.SlaveItemIndex`) (`local.L_SlaveItemData`)))
        (:`then_5`
          (return true)))
      (else
        (return false)))
    (else
      (return false))))

(fn `CombineItems`
  (params (MasterItemIndex :type Integer) (SlaveItemIndex :type Integer) (BP_InventoryComonent :type "/Game/Blueprints/Components/Player/BP_InventoryComponent Object Reference"))
  (returns (CombineSucceeded :type Boolean))
  (set `self.MasterItemIndex` MasterItemIndex)
  (set `self.SlaveItemIndex` SlaveItemIndex)
  (set `self.BP_InventoryComponent` BP_InventoryComonent)
  (return false))