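; Inventory actor bridge that keeps a BP_Firearm's bullet count in step with the Charge field of its inventory item.
; On assignment it unbinds from any previous firearm, caches the new one, binds to its FireHappened event and refreshes the slot display.
; Firing writes the bullet amount back into the item data and updates the slot, while syncing copies the stored Charge onto the firearm.
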(event `self.AssignObservable`
  (params (Actor :type "Actor Object Reference") (ItremIndex :type Integer) (InventoryComponent :type "/Game/Blueprints/Components/Player/BP_InventoryComponent Object Reference"))
  (`parent.AssignObservable` Actor ItremIndex InventoryComponent)
  (`|ExecutionSequence`
    (:`then_0`
      (`/Engine/EditorBlueprintResources/StandardMacros.IsValid` (`self.Firearm`)
        (:`Is Valid`
          (remove `/Game/Blueprints/Weapons/BP_Firearm.FireHappened` (`self.Firearm`) (`|CreateDelegate` :!event `OnFireHappened`)))))
    (:`then_1`
      (bind _asbp_firearm (cast `/Game/Blueprints/Weapons/BP_Firearm` Actor))
      (set `self.Firearm` _asbp_firearm))
    (:`then_2`
      (add `/Game/Blueprints/Weapons/BP_Firearm.FireHappened` (`self.Firearm`) (`|CreateDelegate` :!event `OnFireHappened`)))
    (:`then_3`
      (`self.UpdateSlotDisplayInfo`))))

(event `self.SyncObservableWithItemData`
  (if (`KismetSystemLibrary.IsValid` (`self.Firearm`))
    (set `/Game/Blueprints/Weapons/BP_Firearm.BulletAmount` (`.Charge_12_3F5CFC6849447618911FE689586EBF3B` (break `/Game/Data/Structs/S_InventoryItemData` (`/Game/Blueprints/Components/Player/BP_InventoryComponent.GetItem` (`self.BP_InventoryComponent`) (`self.ItemIndex`)))) (`self.Firearm`))))

(fn `OnFireHappened`
  (params (BulletAmount :type Integer))
  (bind _itemindex (`self.ItemIndex`))
  (bind (_out _found) (`/Game/Blueprints/Components/Player/BP_InventoryComponent.GetItem` (`self.BP_InventoryComponent`) _itemindex))
  (if _found
    (bind _structout (setmembers `/Game/Data/Structs/S_InventoryItemData` :`StructRef` _out :`Charge` BulletAmount))
    (`/Game/Blueprints/Components/Player/BP_InventoryComponent.RewriteItem` (`self.BP_InventoryComponent`) _itemindex _structout)
    (`self.UpdateSlotDisplayInfo`)))