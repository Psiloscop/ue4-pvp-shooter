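; Base actor bridge that links an inventory item, by index and inventory component, to the widgets that display it.
; It keeps a unique list of registered slot widgets and an optional status bar, refreshing slot info plus the bar's weapon and armor slots on update.
; Syncing and removing the observable are empty stubs, and assignment ignores the passed actor, storing only the index and component.
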(fn `AddSlot`
  (params (In :type "/Game/UI/Inventory/W_InventorySlot Object Reference"))
  (`KismetArrayLibrary.Array_AddUnique` (`self.W_InventorySlot`) In))

(fn `AssignObservable`
  (params (Actor :type "Actor Object Reference") (ItremIndex :type Integer) (InventoryComponent :type "/Game/Blueprints/Components/Player/BP_InventoryComponent Object Reference"))
  (set `self.ItemIndex` ItremIndex)
  (set `self.BP_InventoryComponent` InventoryComponent))

(fn `AssignStatusBarWidget`
  (params (In :type "/Game/UI/HUD/W_HUD_StatusBar Object Reference"))
  (set `self.W_StatusBar` In))

(fn `RemoveObservable`)

(fn `RemoveSlot`
  (params (In :type "/Game/UI/Inventory/W_InventorySlot Object Reference"))
  (`KismetArrayLibrary.Array_RemoveItem` (`self.W_InventorySlot`) In))

(fn `SyncObservableWithItemData`)

(fn `UpdateSlotDisplayInfo`
  (`|ExecutionSequence`
    (:`then_0`
      (for _array_element (`self.W_InventorySlot`)
        (`/Game/UI/Inventory/W_InventorySlot.UpdateDisplayInfo` _array_element)))
    (:`then_1`
      (`/Engine/EditorBlueprintResources/StandardMacros.IsValid` (`self.W_StatusBar`)
        (:`Is Valid`
          (`/Game/UI/HUD/W_HUD_StatusBar.UpdateWeaponSlot` (`self.W_StatusBar`))
          (`/Game/UI/HUD/W_HUD_StatusBar.UpdateArmorSlot` (`self.W_StatusBar`)))))))