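; Inventory actor bridge for chest armor that reduces bullet damage taken by the observed BP_Base_Character.
; On assign and removal it swaps OnTakePointDamage bindings on the character.
; OnTakeBulletDamage picks a damage divider and wear rate from the armor tier, lowers the item's Charge and refreshes the slot display.
; It forwards the hit to the character's OnTakeBulletDamage, at full damage once Charge is depleted.
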(event `self.AssignObservable`
  (params (Actor :type "Actor Object Reference") (ItremIndex :type Integer) (InventoryComponent :type "/Game/Blueprints/Components/Player/BP_InventoryComponent Object Reference"))
  (`parent.AssignObservable` Actor ItremIndex InventoryComponent)
  (`|ExecutionSequence`
    (:`then_0`
      (`/Engine/EditorBlueprintResources/StandardMacros.IsValid` (`self.BaseCharacter`)
        (:`Is Valid`
          (add `Actor.OnTakePointDamage` (`self.BaseCharacter`) (`|CreateDelegate` (`self.BaseCharacter`) :!event `OnTakeBulletDamage`))
          (remove `Actor.OnTakePointDamage` (`self.BaseCharacter`) (`|CreateDelegate` :!event `OnTakeBulletDamage`)))))
    (:`then_1`
      (bind _asbp_base_character (cast `/Game/Blueprints/Characters/BP_Base_Character` Actor))
      (set `self.BaseCharacter` _asbp_base_character))
    (:`then_2`
      (remove `Actor.OnTakePointDamage` (`self.BaseCharacter`) (`|CreateDelegate` (`self.BaseCharacter`) :!event `OnTakeBulletDamage`))
      (add `Actor.OnTakePointDamage` (`self.BaseCharacter`) (`|CreateDelegate` :!event `OnTakeBulletDamage`)))))

(event `self.RemoveObservable`
  (`/Engine/EditorBlueprintResources/StandardMacros.IsValid` (`self.BaseCharacter`)
    (:`Is Valid`
      (add `Actor.OnTakePointDamage` (`self.BaseCharacter`) (`|CreateDelegate` (`self.BaseCharacter`) :!event `OnTakeBulletDamage`))
      (remove `Actor.OnTakePointDamage` (`self.BaseCharacter`) (`|CreateDelegate` :!event `OnTakeBulletDamage`))
      (set `self.BaseCharacter` null))))

(fn `OnTakeBulletDamage`
  (params (DamagedActor :type "Actor Object Reference") (Damage :type "Float (double-precision)") (InstigatedBy :type "Controller Object Reference") (HitLocation :type "Vector Structure") (FHitComponent :type "PrimitiveComponent Object Reference") (BoneName :type Name) (ShotFromDirection :type "Vector Structure") (DamageType :type "DamageType Object Reference") (DamageCauser :type "Actor Object Reference"))
  (locals (L_DamageDivider :type "Float (double-precision)" :default 1.0) (L_ReceivedDamage :type "Float (double-precision)") (L_ItemIndex :type Integer :default 0) (L_DamageDividerMultiplyer :type Integer) (L_ArmorDamageCoefficient :type Integer))
  (bind _out (`/Game/Blueprints/Components/Player/BP_InventoryComponent.GetItem` (`self.BP_InventoryComponent`) (`local.L_ItemIndex`)))
  (bind _output (`|GetArrayItem` (`self.W_InventorySlot`)))
  (bind (_id _name _description _type _image _cells _placement _isstackable _chargelimit _charge) (break `/Game/Data/Structs/S_InventoryItemData` _out))
  (bind _returnvalue (- _charge (`local.L_ArmorDamageCoefficient`)))
  (set `local.L_ReceivedDamage` Damage)
  (set `local.L_DamageDividerMultiplyer` 3)
  (`/Engine/EditorBlueprintResources/StandardMacros.IsValid` _output
    (:`Is Valid`
      (set `local.L_ItemIndex` (`/Game/UI/Inventory/W_InventorySlot.ItemIndex` _output)))
    (:`Is Not Valid`
      (set `local.L_ItemIndex` (`self.ItemIndex`))))
  (switch `string` _id
    (:`Default`
      (set `local.L_DamageDivider` 1.0)
      (set `local.L_ArmorDamageCoefficient` 0))
    (:`item_chest_armor_weak`
      (set `local.L_DamageDivider` 1.5)
      (set `local.L_ArmorDamageCoefficient` 10))
    (:`item_chest_armor_medium`
      (set `local.L_DamageDivider` 2.0)
      (set `local.L_ArmorDamageCoefficient` 5))
    (:`item_chest_armor_strong`
      (set `local.L_DamageDivider` 2.5)
      (set `local.L_ArmorDamageCoefficient` 3)))
  (if (> _charge 0)
    (bind _structout (setmembers `/Game/Data/Structs/S_InventoryItemData` :`StructRef` _out :`Charge` (select `bool` (< _returnvalue 0) :`false` _returnvalue)))
    (`/Game/Blueprints/Components/Player/BP_InventoryComponent.RewriteItem` (`self.BP_InventoryComponent`) (`local.L_ItemIndex`) _structout)
    (`self.UpdateSlotDisplayInfo`)
    (`/Game/Blueprints/Characters/BP_Base_Character.OnTakeBulletDamage` (`self.BaseCharacter`) DamagedActor (/ (`local.L_ReceivedDamage`) (* (`local.L_DamageDividerMultiplyer`) (`local.L_DamageDivider`))) InstigatedBy HitLocation FHitComponent BoneName ShotFromDirection DamageType DamageCauser)
    (else
      (`/Game/Blueprints/Characters/BP_Base_Character.OnTakeBulletDamage` (`self.BaseCharacter`) DamagedActor (`local.L_ReceivedDamage`) InstigatedBy HitLocation FHitComponent BoneName ShotFromDirection DamageType DamageCauser))))