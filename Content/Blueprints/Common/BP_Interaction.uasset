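; Base interaction Blueprint that registers itself as an AI sight stimulus and tracks which controller is interacting with it.
; When the interaction controller changes, it moves its action-hand-displayed HUD binding from the old controller to the new one, skipping AI controllers.
; ApplyAction and OnActionHandDisplayed are empty hooks, and GetType returns a default enum value, apparently for child Blueprints to override.
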(event `self.ReceiveBeginPlay`
  ;[1 1 1] Need for AI sight detection
  (`AIPerceptionSystem.RegisterPerceptionStimuliSource` "/Script/AIModule.AISense_Sight" self))

(event `/Game/Blueprints/Interfaces/BP_Intercation_Interface.AssingInteractionController`
  (params (In :type "Controller Object Reference"))
  (bind _returnvalue (not (`.bSuccess` (cast `AIController` (`self.InteractionController`) :!pure true))))
  (if (!= In (`self.InteractionController`))
    (`|ExecutionSequence`
      (:`then_0`
        (if (and _returnvalue (`KismetSystemLibrary.IsValid` (`self.InteractionController`)))
          (remove `/Game/Base/Blueprints/BP_HUD_Base.ActionHandDisplayed` (`/Game/Libs/BP_GlobalGetters.GetHudByController` (`self.InteractionController`)) (`|CreateDelegate` :!event `OnActionHandDisplayed`))))
      (:`then_1`
        (bind _output_get (set `self.InteractionController` In))
        (if _returnvalue
          (add `/Game/Base/Blueprints/BP_HUD_Base.ActionHandDisplayed` (`/Game/Libs/BP_GlobalGetters.GetHudByController` _output_get) (`|CreateDelegate` :!event `OnActionHandDisplayed`)))))))

(event `/Game/Blueprints/Interfaces/BP_Intercation_Interface.ApplyAction`)

(fn `GetType`
  (returns (Out :type "/Game/Data/Enums/E_ObjectType Enum"))
  (return "NewEnumerator0"))

(fn `OnActionHandDisplayed`
  (params (ActonHand :type "/Game/Data/Enums/E_ActionHandType Enum" :default "NewEnumerator0")))

(fn `UserConstructionScript`)