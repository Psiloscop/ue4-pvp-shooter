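; Spawner actor that places a random rifle with two matching magazines at its spawn point.
; On BeginPlay it fills parallel weapon and magazine class lists, spawns once, then retries on a looping timer set by TimeSpawnInterval.
; A new weapon spawns only when the previous reference is invalid.
; Matching magazines, picked by the same index and offset beside it, spawn then only if both previous magazines are also invalid.
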(event `self.ReceiveBeginPlay`
  (`parent.ReceiveBeginPlay`)
  (set `self.WeaponList` (`|MakeArray` "/Game/Blueprints/Items/Weapons/BP_Item_ak47.BP_Item_ak47_C" "/Game/Blueprints/Items/Weapons/BP_Item_ak74u.BP_Item_ak74u_C" "/Game/Blueprints/Items/Weapons/BP_Item_ar15a4.BP_Item_ar15a4_C" "/Game/Blueprints/Items/Weapons/BP_Item_asval.BP_Item_asval_C" "/Game/Blueprints/Items/Weapons/BP_Item_m4a1.BP_Item_m4a1_C" :!type "/Game/Blueprints/Items/Common/BP_Item_Base Class Reference"))
  (set `self.AmmoList` (`|MakeArray` "/Game/Blueprints/Items/Weapons/BP_Item_ak47_mag.BP_Item_ak47_mag_C" "/Game/Blueprints/Items/Weapons/BP_Item_ak74u_mag.BP_Item_ak74u_mag_C" "/Game/Blueprints/Items/Weapons/BP_Item_ar15a4_mag.BP_Item_ar15a4_mag_C" "/Game/Blueprints/Items/Weapons/BP_Item_asval_mag.BP_Item_asval_mag_C" "/Game/Blueprints/Items/Weapons/BP_Item_m4a1_mag.BP_Item_m4a1_mag_C" :!type "/Game/Blueprints/Items/Common/BP_Item_Base Class Reference"))
  (`self.SpawnWeaponAndMag`)
  (`KismetSystemLibrary.K2_SetTimer` null "SpawnWeaponAndMag" (`self.TimeSpawnInterval`) true))

(fn `SpawnWeaponAndMag`
  (locals (LWeaponIndex :type Integer :default 0) (L_MagLOcation :type "Vector Structure" :default (0.0 0.0 0.0)))
  (bind (_returnvalue_location _returnvalue_rotation _returnvalue_scale) (`KismetMathLibrary.BreakTransform` (`SceneComponent.K2_GetComponentToWorld` (`self.SpawnPoint`))))
  (bind _returnvalue (+ _returnvalue_location (-20.0 0.0 0.0)))
  (if (not (`KismetSystemLibrary.IsValid` (`self.SpawnedWeapon`)))
    (set `local.LWeaponIndex` (`KismetMathLibrary.RandomIntegerInRange` 0 (- (`KismetArrayLibrary.Array_Length` (`self.WeaponList`)) 1)))
    (`|ExecutionSequence`
      (:`then_0`
        (bind _returnvalue_2 (`|SpawnActorFromClass` (`|GetArrayItem` (`self.WeaponList`) (`local.LWeaponIndex`)) (`SceneComponent.K2_GetComponentToWorld` (`self.SpawnPoint`)) "Undefined" "OverrideRootScale" null null))
        (set `self.SpawnedWeapon` _returnvalue_2))
      (:`then_1`
        (if (and (not (`KismetSystemLibrary.IsValid` (`self.SpawnedMag1`))) (not (`KismetSystemLibrary.IsValid` (`self.SpawnedMag2`))))
          (set `local.L_MagLOcation` _returnvalue)
          (bind _returnvalue_3 (`|SpawnActorFromClass` (`|GetArrayItem` (`self.AmmoList`) (`local.LWeaponIndex`)) (`KismetMathLibrary.MakeTransform` _returnvalue _returnvalue_rotation _returnvalue_scale) "Undefined" "OverrideRootScale" null null))
          (set `self.SpawnedMag1` _returnvalue_3)
          (bind _returnvalue_4 (`|SpawnActorFromClass` (`|GetArrayItem` (`self.AmmoList`) (`local.LWeaponIndex`)) (`KismetMathLibrary.MakeTransform` (+ (`local.L_MagLOcation`) (0.0 5.0 0.0)) _returnvalue_rotation _returnvalue_scale) "Undefined" "OverrideRootScale" null null))
          (set `self.SpawnedMag2` _returnvalue_4))))))

(fn `UserConstructionScript`
  (`parent.UserConstructionScript`))