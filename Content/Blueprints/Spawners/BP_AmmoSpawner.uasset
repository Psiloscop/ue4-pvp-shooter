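; BP_AmmoSpawner is a spawner that keeps two slots stocked with a random type of rifle magazine.
; BeginPlay fills the magazine class list and starts a looping timer that calls SpawnAmmo.
; Each call picks one random class and spawns it into any slot whose tracked actor is no longer valid.
; Items spawn at the SpawnPoint transform, with the second slot offset along world Y.
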(event `self.ReceiveBeginPlay`
  (`parent.ReceiveBeginPlay`)
  (set `self.AmmoList` (`|MakeArray` "/Game/Blueprints/Items/Weapons/BP_Item_ak47_mag.BP_Item_ak47_mag_C" "/Game/Blueprints/Items/Weapons/BP_Item_ak74u_mag.BP_Item_ak74u_mag_C" "/Game/Blueprints/Items/Weapons/BP_Item_ar15a4_mag.BP_Item_ar15a4_mag_C" "/Game/Blueprints/Items/Weapons/BP_Item_asval_mag.BP_Item_asval_mag_C" "/Game/Blueprints/Items/Weapons/BP_Item_m4a1_mag.BP_Item_m4a1_mag_C" :!type "/Game/Blueprints/Items/Common/BP_Item_Base Class Reference"))
  (set `self.AmmoAmount` 2)
  (`KismetSystemLibrary.K2_SetTimer` null "SpawnAmmo" (`self.TimeInterval`) true))

(fn `SpawnAmmo`
  (locals (L_AmmoToSpawn :type "/Game/Blueprints/Items/Common/BP_Item_Base Class Reference"))
  (bind _spawnpoint (`self.SpawnPoint`))
  (set `local.L_AmmoToSpawn` (`|GetArrayItem` (`self.AmmoList`) (`KismetMathLibrary.RandomIntegerInRange` 0 (- (`KismetArrayLibrary.Array_Length` (`self.AmmoList`)) 1))))
  (for _index (range 1 (+ (`self.AmmoAmount`) 1))
    (`/Engine/EditorBlueprintResources/StandardMacros.IsValid` (`KismetMathLibrary.SelectObject` (`self.SpawnedAmmo1`) (`self.SpawnedAmmo2`) (== _index 1))
      (:`Is Not Valid`
        (bind _returnvalue (`|SpawnActorFromClass` (`local.L_AmmoToSpawn`) (`KismetMathLibrary.MakeTransform` (+ (`SceneComponent.K2_GetComponentLocation` _spawnpoint) (`KismetMathLibrary.MakeVector` 0.0 (* (- _index 1) (`self.AmmoItemOffset`)))) (`SceneComponent.K2_GetComponentRotation` _spawnpoint) (`SceneComponent.K2_GetComponentScale` _spawnpoint)) "Undefined" "OverrideRootScale" null null))
        (switch `int` _index
          (:`1`
            (set `self.SpawnedAmmo1` _returnvalue))
          (:`2`
            (set `self.SpawnedAmmo2` _returnvalue)))))))

(fn `UserConstructionScript`
  (`parent.UserConstructionScript`))