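; Spawner actor that places a random chest armor pickup in the level at its spawn point.
; On BeginPlay it fills a list with weak, medium and strong armor classes, spawns one immediately, then starts a looping timer on the spawn interval.
; Each tick of the timer spawns a new, uniformly random piece only if the previous one is no longer valid, so at most one tracked armor exists at a time.
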(event `self.ReceiveBeginPlay`
  (`parent.ReceiveBeginPlay`)
  (set `self.ArmorList` (`|MakeArray` "/Game/Blueprints/Items/Armor/BP_Item_ChestArmor_Weak.BP_Item_ChestArmor_Weak_C" "/Game/Blueprints/Items/Armor/BP_Item_ChestArmor_Medium.BP_Item_ChestArmor_Medium_C" "/Game/Blueprints/Items/Armor/BP_Item_ChestArmor_Strong.BP_Item_ChestArmor_Strong_C" :!type "/Game/Blueprints/Items/Common/BP_Item_Base Class Reference"))
  (`self.SpawnArmor`)
  (`KismetSystemLibrary.K2_SetTimer` null "SpawnArmor" (`self.TimeSpawnInterval`) true))

(fn `SpawnArmor`
  (if (not (`KismetSystemLibrary.IsValid` (`self.SpawnedArmor`)))
    (bind _returnvalue (`|SpawnActorFromClass` (`|GetArrayItem` (`self.ArmorList`) (`KismetMathLibrary.RandomIntegerInRange` 0 (- (`KismetArrayLibrary.Array_Length` (`self.ArmorList`)) 1))) (`SceneComponent.K2_GetComponentToWorld` (`self.SpawnPoint`)) "Undefined" "OverrideRootScale" null null))
    (set `self.SpawnedArmor` _returnvalue)))

(fn `UserConstructionScript`
  (`parent.UserConstructionScript`))