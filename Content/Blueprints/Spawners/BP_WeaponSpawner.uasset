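; BP_WeaponSpawner is a spawner actor that places a random rifle pickup at its SpawnPoint component.
; BeginPlay fills WeaponList with a hardcoded set of weapon item classes and starts a looping timer at TimeInterval.
; Each tick of that timer calls SpawnWeapon, which spawns a random class from the list only when SpawnedWeapon is no longer valid, keeping one tracked weapon at a time.
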(event `self.ReceiveBeginPlay`
  (`parent.ReceiveBeginPlay`)
  (set `self.WeaponList` (`|MakeArray` "/Game/Blueprints/Items/Weapons/BP_Item_ak47.BP_Item_ak47_C" "/Game/Blueprints/Items/Weapons/BP_Item_ak74u.BP_Item_ak74u_C" "/Game/Blueprints/Items/Weapons/BP_Item_ar15a4.BP_Item_ar15a4_C" "/Game/Blueprints/Items/Weapons/BP_Item_asval.BP_Item_asval_C" "/Game/Blueprints/Items/Weapons/BP_Item_m4a1.BP_Item_m4a1_C" :!type "/Game/Blueprints/Items/Common/BP_Item_Base Class Reference"))
  (`KismetSystemLibrary.K2_SetTimer` null "SpawnWeapon" (`self.TimeInterval`) true))

(fn `SpawnWeapon`
  (if (not (`KismetSystemLibrary.IsValid` (`self.SpawnedWeapon`)))
    (bind _returnvalue (`|SpawnActorFromClass` (`|GetArrayItem` (`self.WeaponList`) (`KismetMathLibrary.RandomIntegerInRange` 0 (- (`KismetArrayLibrary.Array_Length` (`self.WeaponList`)) 1))) (`SceneComponent.K2_GetComponentToWorld` (`self.SpawnPoint`)) "Undefined" "OverrideRootScale" null null))
    (set `self.SpawnedWeapon` _returnvalue)))

(fn `UserConstructionScript`
  (`parent.UserConstructionScript`))