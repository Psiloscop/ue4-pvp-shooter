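; Medkit spawner actor that keeps at most one randomly chosen weak, medium or strong medkit at its spawn point.
; It spawns one on BeginPlay, then a looping timer retries at a set interval.
; Each call spawns a replacement only if the previous medkit is no longer valid, so the wait after removal depends on the timer's phase.
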(event `self.ReceiveBeginPlay`
  (`parent.ReceiveBeginPlay`)
  (set `self.MedkitList` (`|MakeArray` "/Game/Blueprints/Items/Medkit/BP_Item_Medkit_Weak.BP_Item_Medkit_Weak_C" "/Game/Blueprints/Items/Medkit/BP_Item_Medkit_Medium.BP_Item_Medkit_Medium_C" "/Game/Blueprints/Items/Medkit/BP_Item_Medkit_Strong.BP_Item_Medkit_Strong_C" :!type "/Game/Blueprints/Items/Common/BP_Item_Base Class Reference"))
  (`self.SpawnMedkit`)
  (`KismetSystemLibrary.K2_SetTimer` null "SpawnMedkit" (`self.TimeSpawnInterval`) true))

(fn `SpawnMedkit`
  (if (not (`KismetSystemLibrary.IsValid` (`self.SpawnedMedkit`)))
    (bind _returnvalue (`|SpawnActorFromClass` (`|GetArrayItem` (`self.MedkitList`) (`KismetMathLibrary.RandomIntegerInRange` 0 (- (`KismetArrayLibrary.Array_Length` (`self.MedkitList`)) 1))) (`SceneComponent.K2_GetComponentToWorld` (`self.SpawnPoint`)) "Undefined" "OverrideRootScale" null null))
    (set `self.SpawnedMedkit` _returnvalue)))

(fn `UserConstructionScript`
  (`parent.UserConstructionScript`))