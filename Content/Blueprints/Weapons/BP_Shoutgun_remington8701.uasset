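; Remington 870 shotgun Blueprint that fills in weapon-specific events and functions on top of its parent class.
; Skeletal sockets on the gun mesh drive shot origin, muzzle effect and sound, handguard transform, and bushing (shell) ejection along the right vector.
; Shoot delegates to MakeShot from the fireshot socket, while magazine attachment snaps to target.
; Muzzle effect and sound reuse AK-47 assets; the debug aim trace is disconnected from Tick.
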(event `self.ReceiveBeginPlay`
  (`parent.ReceiveBeginPlay`))

(event `self.ReceiveTick`
  (params (DeltaSeconds :type "Float (single-precision)"))
  ;[1 1 1] Draws line from fireshot location to what's fireshot is facing to
)

(event `AttachMagazineActor`
  (`self.K2_AttachToComponent` (`self.Magazine`) null "None" "SnapToTarget" "SnapToTarget" "SnapToTarget" true))

(event `/Game/Blueprints/Interfaces/BP_SpecificFirearmWeapon_Interface.PlayFireshotEffect`
  (`GameplayStatics.SpawnEmitterAttached` "/Game/Assets/Weapons/AK47/Particle/P_ak47_shot.P_ak47_shot" (`self.Firearm_remington870`) "fireshot" (0.0 0.0 0.0) (struct) (0.3 0.3 0.3) "KeepRelativeOffset" true "AutoRelease"))

(event `/Game/Blueprints/Interfaces/BP_SpecificFirearmWeapon_Interface.PlayFireshotSound`
  (`GameplayStatics.PlaySoundAtLocation` "/Game/Assets/Weapons/AK47/Sound/S_ak47_shot.S_ak47_shot" (`SceneComponent.GetSocketLocation` (`self.Firearm_remington870`) "fireshot") (struct) 1.0 1.0 0.0 null null null))

(event `/Game/Blueprints/Interfaces/BP_SpecificFirearmWeapon_Interface.SpawnBushingActor`
  (bind _firearm_remington870 (`self.Firearm_remington870`))
  (`self.SpawnBushingProjectile` (`SceneComponent.GetSocketLocation` _firearm_remington870 "split_gearbox") (`SceneComponent.GetRightVector` _firearm_remington870)))

(fn `GetFireRate`
  (returns (Out :type "Float (double-precision)"))
  (return (`self.FireRate`)))

(fn `GetFireshotTransform`
  (returns (Out :type "Transform Structure"))
  (return (`SceneComponent.GetSocketTransform` (`self.Firearm_remington870`) "fireshot" "RTS_World")))

(fn `GetHandguardTransform`
  (returns (Out :type "Transform Structure"))
  (return (`SceneComponent.GetSocketTransform` (`self.Firearm_remington870`) "handguard" "RTS_World")))

(fn `Shoot`
  (returns (ShootHappened :type Boolean))
  (bind _shothappened (`self.MakeShot` (`SceneComponent.GetSocketLocation` (`self.Firearm_remington870`) "fireshot")))
  (return _shothappened))

(fn `UserConstructionScript`
  (`parent.UserConstructionScript`))