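; Firearm Blueprint that handles ammo, bullet spawning with scatter, and bushing ejection.
; Fire decrements ammo and calls FireHappened, leaving rate limiting to animation cooldown; the timer cooldown and automatic refire are disabled.
; SpawnBulletProjectile aims from the muzzle at the attach parent's destination point, or a forward-vector fallback, randomly rotated by ScatterAngle, passing damage and owner.
; SpawnBushingProjectile randomizes ejection pitch and yaw using the random stream.
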(fn `CalculateBulletDestination`
  (returns (Out :type "Vector Structure"))
  (locals (L_CrosshairLocation :type "Vector Structure"))
  (bind _scatterangle (`self.ScatterAngle`))
  (bind _scatterangle_2 (`self.ScatterAngle`))
  (bind _returnvalue (`KismetMathLibrary.Conv_VectorToRotator` (`local.L_CrosshairLocation`)))
  (bind _out (`/Game/Libs/BP_WeaponFunctions.GetBulletDestinationPoint` (`self.GetAttachParentActor`)))
  (`|ExecutionSequence`
    (:`then_0`
      (if (!= _out (0.0 0.0 0.0) :`ErrorTolerance` 0.0)
        (set `local.L_CrosshairLocation` _out)
        (else
          (set `local.L_CrosshairLocation` (* (`self.GetActorForwardVector`) 10000)))))
    (:`then_1`
      (return (`KismetMathLibrary.RotateAngleAxis` (`KismetMathLibrary.RotateAngleAxis` (`local.L_CrosshairLocation`) (`KismetMathLibrary.RandomFloatInRangeFromStream` (* -1.0 _scatterangle_2) _scatterangle_2 (`self.RandomStream`)) (`KismetMathLibrary.GetRightVector` _returnvalue)) (`KismetMathLibrary.RandomFloatInRangeFromStream` (* -1.0 _scatterangle) _scatterangle (`self.RandomStream`)) (`KismetMathLibrary.GetUpVector` _returnvalue))))))

(fn `Cooldown`
  (`KismetSystemLibrary.K2_ClearAndInvalidateTimerHandle` (`self.CooldownTimer`))
  (if (and (`self.IsAbleToFire`) (`self.IsAutomatic`) false)
    (`self.Fire`)))

(fn `Fire`
  (returns (FireHappened :type Boolean))
  (if (`self.IsAbleToFire`)
    (bind _result (`/Engine/EditorBlueprintResources/StandardMacros.DecrementInt` (`self.BulletAmount`))
      (:`  `
        (`self.FireHappened` _result)
        (return true)))
    (else
      (return false))))

(fn `IsAbleToFire`
  (returns (Out :type Boolean))
  (return (and (> (`self.BulletAmount`) 0) true)))

(fn `SpawnBulletProjectile`
  (bind _muzzlelocation (`self.MuzzleLocation`))
  (`|SpawnActorFromClass` (`self.BulletClass`) (`KismetMathLibrary.MakeTransform` _muzzlelocation (`KismetMathLibrary.FindLookAtRotation` _muzzlelocation (`self.CalculateBulletDestination`))) "AlwaysSpawn" "OverrideRootScale" null (`self.Damage`) (`self.WeaponOwner`) null))

(fn `SpawnBushingProjectile`
  (params (SplitGearboxLocation :type "Vector Structure") (SplitGearboxDirection :type "Vector Structure"))
  (bind _pitch (.pitch (`KismetMathLibrary.Conv_VectorToRotator` SplitGearboxDirection)))
  (bind _yaw (.yaw (`KismetMathLibrary.Conv_VectorToRotator` SplitGearboxDirection)))
  (`|SpawnActorFromClass` (`self.BushingClass`) (`KismetMathLibrary.MakeTransform` SplitGearboxLocation (`KismetMathLibrary.MakeRotator` (.roll (`KismetMathLibrary.Conv_VectorToRotator` SplitGearboxDirection)) (`KismetMathLibrary.RandomFloatInRangeFromStream` (- _pitch 10.0) (+ _pitch 10.0) (`self.RandomStream`)) (`KismetMathLibrary.RandomFloatInRangeFromStream` (- _yaw 10.0) (+ _yaw 10.0) (`self.RandomStream`)))) "AlwaysSpawn" "OverrideRootScale" null null))

(fn `UserConstructionScript`)