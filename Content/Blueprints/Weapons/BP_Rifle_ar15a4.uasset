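; AR-15A4 rifle Blueprint that supplies the weapon-specific magazine, effects, sound and socket locations to its parent firearm class.
; On BeginPlay it spawns a BP_Mag_ar15a4 magazine and attaches it at the magazine snap point.
; Mesh sockets drive the parent's shot and bushing-projectile calls, muzzle effect and sound, and the handguard and fireshot transform getters.
; Tick is empty, leaving a debug muzzle line trace disconnected.
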(event `self.ReceiveBeginPlay`
  (`parent.ReceiveBeginPlay`)
  (bind _out (`/Game/Blueprints/Interfaces/BP_WeaponWithMagazine_Interface.SpawnMagazineActor` (`SceneComponent.K2_GetComponentToWorld` (`self.MagazineSnapLocation`))))
  (`self.K2_AttachToComponent` _out (`self.MagazineSnapLocation`) "None" "KeepWorld" "KeepWorld" "KeepWorld" true))

(event `self.ReceiveTick`
  (params (DeltaSeconds :type "Float (single-precision)"))
  ;[1 1 1] Draws line from fireshot location to what's fireshot is facing to
)

(event `/Game/Blueprints/Interfaces/BP_WeaponWithMagazine_Interface.AttachMagazineActor`
  (`self.K2_AttachToComponent` (`self.Magazine`) (`self.MagazineSnapLocation`) "None" "SnapToTarget" "SnapToTarget" "SnapToTarget" true))

(event `/Game/Blueprints/Interfaces/BP_SpecificFirearmWeapon_Interface.PlayFireshotEffect`
  (`GameplayStatics.SpawnEmitterAttached` "/Game/Assets/Weapons/M15A4/Particles/P_m15a4_shot.P_m15a4_shot" (`self.Firearm_AR15A4`) "fireshot" (0.0 0.0 0.0) (struct) (0.6 0.6 0.6)))

(event `/Game/Blueprints/Interfaces/BP_SpecificFirearmWeapon_Interface.PlayFireshotSound`
  (`GameplayStatics.PlaySoundAtLocation` "/Game/Assets/Weapons/M15A4/Sound/S_m15a4_shot.S_m15a4_shot" (`SceneComponent.GetSocketLocation` (`self.Firearm_AR15A4`) "fireshot") (struct) 1.0 1.0 0.0 null null null))

(event `/Game/Blueprints/Interfaces/BP_SpecificFirearmWeapon_Interface.SpawnBushingActor`
  (bind _firearm_ar15a4 (`self.Firearm_AR15A4`))
  (`self.SpawnBushingProjectile` (`SceneComponent.GetSocketLocation` _firearm_ar15a4 "split_gearbox") (`SceneComponent.GetRightVector` _firearm_ar15a4)))

(fn `GetFireRate`
  (returns (Out :type "Float (double-precision)"))
  (return (`self.FireRate`)))

(fn `GetFireshotTransform`
  (returns (Out :type "Transform Structure"))
  (return (`SceneComponent.GetSocketTransform` (`self.Firearm_AR15A4`) "fireshot" "RTS_World")))

(fn `GetHandguardTransform`
  (returns (Out :type "Transform Structure"))
  (return (`SceneComponent.GetSocketTransform` (`self.Firearm_AR15A4`) "handguard" "RTS_World")))

(fn `GetMagazineActor`
  (returns (Out :type "Actor Object Reference"))
  (return (`self.Magazine`)))

(fn `Shoot`
  (returns (ShootHappened :type Boolean))
  (bind _shothappened (`self.MakeShot` (`SceneComponent.GetSocketLocation` (`self.Firearm_AR15A4`) "fireshot")))
  (return _shothappened))

(fn `SpawnMagazineActor`
  (params (WhereTo :type "Transform Structure"))
  (returns (Out :type "Actor Object Reference"))
  (bind _returnvalue (`|SpawnActorFromClass` "/Game/Blueprints/Weapons/BP_mag_ar15a4.BP_Mag_ar15a4_C" (`KismetMathLibrary.MakeTransform` (.location WhereTo) (.rotation (`SceneComponent.K2_GetComponentToWorld` (`self.MagazineSnapLocation`))) (.scale (`SceneComponent.K2_GetComponentToWorld` (`self.MagazineSnapLocation`)))) "Undefined" "OverrideRootScale" null null))
  (bind _output_get (set `self.Magazine` _returnvalue))
  (return _output_get))

(fn `UserConstructionScript`
  (`parent.UserConstructionScript`))