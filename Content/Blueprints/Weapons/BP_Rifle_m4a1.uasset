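; M4A1 rifle Blueprint that fills in weapon-specific behavior on top of its parent class.
; BeginPlay spawns an M4A1 magazine and attaches it at the snap location, with an event to re-snap it.
; Mesh sockets drive shooting, muzzle particles, sound, bushing ejection and handguard transform, while shot and projectile logic is delegated to functions defined elsewhere.
; Tick is empty; its debug line trace is disconnected.
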(event `self.ReceiveBeginPlay`
  (`parent.ReceiveBeginPlay`)
  (bind _out (`self.SpawnMagazineActor` (`SceneComponent.K2_GetComponentToWorld` (`self.MagazineSnapLocation`))))
  (`self.K2_AttachToComponent` _out (`self.MagazineSnapLocation`) "None" "KeepWorld" "KeepWorld" "KeepWorld" true))

(event `self.ReceiveTick`
  (params (DeltaSeconds :type "Float (single-precision)"))
  ;[1 1 1] Draws line from fireshot location to what's fireshot is facing to
)

(event `self.AttachMagazineActor`
  (`self.K2_AttachToComponent` (`self.Magazine`) (`self.MagazineSnapLocation`) "None" "SnapToTarget" "SnapToTarget" "SnapToTarget" true))

(event `/Game/Blueprints/Interfaces/BP_SpecificFirearmWeapon_Interface.PlayFireshotEffect`
  (`GameplayStatics.SpawnEmitterAttached` "/Game/Assets/Weapons/M4A1/Particles/P_m4a1_shot.P_m4a1_shot" (`self.Firearm_M4A1`) "fireshot" (0.0 0.0 0.0) (struct) (0.7 0.7 0.7)))

(event `/Game/Blueprints/Interfaces/BP_SpecificFirearmWeapon_Interface.PlayFireshotSound`
  (`GameplayStatics.PlaySoundAtLocation` "/Game/Assets/Weapons/M4A1/Sound/S_M4a1_Shot.S_m4a1_shot" (`SceneComponent.GetSocketLocation` (`self.Firearm_M4A1`) "fireshot") (struct) 1.0 1.0 0.0 null null null))

(event `/Game/Blueprints/Interfaces/BP_SpecificFirearmWeapon_Interface.SpawnBushingActor`
  (bind _firearm_m4a1 (`self.Firearm_M4A1`))
  (`self.SpawnBushingProjectile` (`SceneComponent.GetSocketLocation` _firearm_m4a1 "split_gearbox") (`SceneComponent.GetRightVector` _firearm_m4a1)))

(fn `GetFireRate`
  (returns (Out :type "Float (double-precision)"))
  (return (`self.FireRate`)))

(fn `GetFireshotTransform`
  (returns (Out :type "Transform Structure"))
  (return (`SceneComponent.GetSocketTransform` (`self.Firearm_M4A1`) "fireshot" "RTS_World")))

(fn `GetHandguardTransform`
  (returns (Out :type "Transform Structure"))
  (return (`SceneComponent.GetSocketTransform` (`self.Firearm_M4A1`) "handguard" "RTS_World")))

(fn `GetMagazineActor`
  (returns (Out :type "Actor Object Reference"))
  (return (`self.Magazine`)))

(fn `Shoot`
  (returns (ShootHappened :type Boolean))
  (bind _shothappened (`self.MakeShot` (`SceneComponent.GetSocketLocation` (`self.Firearm_M4A1`) "fireshot")))
  (return _shothappened))

(fn `SpawnMagazineActor`
  (params (WhereTo :type "Transform Structure"))
  (returns (Out :type "Actor Object Reference"))
  (bind _returnvalue (`|SpawnActorFromClass` "/Game/Blueprints/Weapons/BP_mag_m4a1.BP_Mag_m4a1_C" (`KismetMathLibrary.MakeTransform` (.location WhereTo) (.rotation WhereTo) (.scale (`SceneComponent.K2_GetComponentToWorld` (`self.MagazineSnapLocation`)))) "Undefined" "OverrideRootScale" null null))
  (bind _output_get (set `self.Magazine` _returnvalue))
  (return _output_get))

(fn `UserConstructionScript`
  (`parent.UserConstructionScript`))