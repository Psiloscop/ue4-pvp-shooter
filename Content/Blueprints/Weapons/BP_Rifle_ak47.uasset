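; AK-47 rifle Blueprint that supplies weapon-specific assets, sockets and overrides to its parent firearm class.
; On BeginPlay it spawns a BP_Mag_ak47 and attaches it at the magazine snap location, with an event to snap it back in place.
; Mesh sockets drive shot origin, muzzle effect and sound, handguard transform, and bushing projectile ejection.
; A debug muzzle line trace remains disconnected from Tick.
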(event `self.ReceiveBeginPlay`
  (`parent.ReceiveBeginPlay`)
  (bind _out (`/Game/Blueprints/Interfaces/BP_WeaponWithMagazine_Interface.SpawnMagazineActor` (`SceneComponent.K2_GetComponentToWorld` (`self.MagazineSnapLocation`))))
  (`self.K2_AttachToComponent` _out (`self.MagazineSnapLocation`) "None" "KeepWorld" "KeepWorld" "KeepWorld" true))

(event `self.ReceiveTick`
  (params (DeltaSeconds :type "Float (single-precision)"))
  ;[1 1 1] Draws line from fireshot location to what's fireshot is facing to
)

(event `/Game/Blueprints/Interfaces/BP_WeaponWithMagazine_Interface.AttachMagazineActor`
  (`self.K2_AttachToComponent` (`self.Magazine`) (`self.MagazineSnapLocation`) "None" "SnapToTarget" "SnapToTarget" "SnapToTarget" true))

(event `/Game/Blueprints/Interfaces/BP_SpecificFirearmWeapon_Interface.PlayFireshotEffect`
  (`GameplayStatics.SpawnEmitterAttached` "/Game/Assets/Weapons/AK47/Particle/P_ak47_shot.P_ak47_shot" (`self.Firearm_AK47`) "fireshot" (0.0 0.0 0.0) (struct) (0.3 0.3 0.3) "KeepRelativeOffset" true "AutoRelease"))

(event `/Game/Blueprints/Interfaces/BP_SpecificFirearmWeapon_Interface.PlayFireshotSound`
  (`GameplayStatics.PlaySoundAtLocation` "/Game/Assets/Weapons/AK47/Sound/S_ak47_shot.S_ak47_shot" (`SceneComponent.GetSocketLocation` (`self.Firearm_AK47`) "fireshot") (struct) 1.0 1.0 0.0 null null null))

(event `/Game/Blueprints/Interfaces/BP_SpecificFirearmWeapon_Interface.SpawnBushingActor`
  (bind _firearm_ak47 (`self.Firearm_AK47`))
  (`self.SpawnBushingProjectile` (`SceneComponent.GetSocketLocation` _firearm_ak47 "split_gearbox") (`SceneComponent.GetRightVector` _firearm_ak47)))

(fn `GetFireRate`
  (returns (Out :type "Float (double-precision)"))
  (return (`self.FireRate`)))

(fn `GetFireshotTransform`
  (returns (Out :type "Transform Structure"))
  (return (`SceneComponent.GetSocketTransform` (`self.Firearm_AK47`) "fireshot" "RTS_World")))

(fn `GetHandguardTransform`
  (returns (Out :type "Transform Structure"))
  (return (`SceneComponent.GetSocketTransform` (`self.Firearm_AK47`) "handguard" "RTS_World")))

(fn `GetMagazineActor`
  (returns (Out :type "Actor Object Reference"))
  (return (`self.Magazine`)))

(fn `Shoot`
  (returns (ShootHappened :type Boolean))
  (bind _shothappened (`self.MakeShot` (`SceneComponent.GetSocketLocation` (`self.Firearm_AK47`) "fireshot")))
  (return _shothappened))

(fn `SpawnMagazineActor`
  (params (WhereTo :type "Transform Structure"))
  (returns (Out :type "Actor Object Reference"))
  (bind _returnvalue (`|SpawnActorFromClass` "/Game/Blueprints/Weapons/BP_Mag_ak47.BP_Mag_ak47_C" (`KismetMathLibrary.MakeTransform` (.location WhereTo) (.rotation WhereTo) (.scale (`SceneComponent.K2_GetComponentToWorld` (`self.MagazineSnapLocation`)))) "Undefined" "OverrideRootScale" null null))
  (bind _output_get (set `self.Magazine` _returnvalue))
  (return _output_get))

(fn `UserConstructionScript`
  (`parent.UserConstructionScript`))