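; BP_Rifle is a rifle weapon Blueprint that builds on a parent class and spawns bullet projectiles when it fires.
; On BeginPlay it binds a handler to the FireHappened event, while OnShotHappened spawns a bullet projectile.
; MakeShot stores the given muzzle location, then calls Fire and returns its result.
; GetHandguardTransform is an empty stub, and the construction script only calls the parent.
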(event `self.ReceiveBeginPlay`
  (`parent.ReceiveBeginPlay`)
  (add `self.FireHappened` (`|CreateDelegate` :!event `OnShotHappened`)))

(fn `GetHandguardTransform`
  (returns (Out :type "Transform Structure"))
  (return))

(fn `MakeShot`
  (params (MuzzleLocation :type "Vector Structure"))
  (returns (ShotHappened :type Boolean))
  (set `self.MuzzleLocation` MuzzleLocation)
  (bind _firehappened (`self.Fire`))
  (return _firehappened))

(fn `OnShotHappened`
  (params (BulletAmount :type Integer))
  (`self.SpawnBulletProjectile`))

(fn `UserConstructionScript`
  (`parent.UserConstructionScript`))