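; Remington 870 shotgun weapon Blueprint that fills in a parent firearm class's effect, firing and query hooks.
; Sockets on the firearm component place the muzzle flash, shot sound, handguard transform and bushing (casing) projectile, which ejects along the weapon's right vector.
; Shoot passes the muzzle socket location to MakeShot and returns its result.
; GetFireRate exposes the FireRate variable, while GetFireshotTransform returns no wired value.
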(event `/Game/Blueprints/Interfaces/BP_SpecificFirearmWeapon_Interface.PlayFireshotEffect`
  (`GameplayStatics.SpawnEmitterAttached` "/Game/Assets/Weapons/Remington870/Particles/P_remington870_shot.P_remington870_shot" (`self.Firearm_remingron870`) "fireshot" (0.0 0.0 0.0) (struct) (0.4 0.4 0.4)))

(event `/Game/Blueprints/Interfaces/BP_SpecificFirearmWeapon_Interface.PlayFireshotSound`
  (`GameplayStatics.PlaySoundAtLocation` "/Game/Assets/Weapons/Remington870/Sound/S_remington870_shot.S_remington870_shot" (`SceneComponent.GetSocketLocation` (`self.Firearm_remingron870`) "fireshot") (struct) 1.0 1.0 0.0 null null null))

(event `/Game/Blueprints/Interfaces/BP_SpecificFirearmWeapon_Interface.SpawnBushingActor`
  (bind _firearm_remingron870 (`self.Firearm_remingron870`))
  (`self.SpawnBushingProjectile` (`SceneComponent.GetSocketLocation` _firearm_remingron870 "split_gearbox") (`SceneComponent.GetRightVector` _firearm_remingron870)))

(fn `GetFireRate`
  (returns (Out :type "Float (double-precision)"))
  (return (`self.FireRate`)))

(fn `GetFireshotTransform`
  (returns (Out :type "Transform Structure"))
  (return))

(fn `GetHandguardTransform`
  (returns (Out :type "Transform Structure"))
  (return (`SceneComponent.GetSocketTransform` (`self.Firearm_remingron870`) "handguard" "RTS_World")))

(fn `Shoot`
  (returns (ShootHappened :type Boolean))
  (bind _shothappened (`self.MakeShot` (`SceneComponent.GetSocketLocation` (`self.Firearm_remingron870`) "fireshot")))
  (return _shothappened))

(fn `UserConstructionScript`
  (`parent.UserConstructionScript`))