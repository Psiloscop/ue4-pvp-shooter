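; Player component that detects interactable BP_Interaction actors in view and triggers their action on request.
; While interaction mode is enabled, Tick line-traces from the owner's camera toward an end point offset from the HUD action-hand location.
; Target changes update outline and controller assignment and notify detected or ignored.
; Combat state changes can disable the mode, whose RepNotify clears the outline and target when off.
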(event `self.ReceiveBeginPlay`
  (add `/Game/Blueprints/Components/Player/BP_CombatComponent.CombatStateChanged` (`/Game/Blueprints/Characters/Player/BP_Character.BP_CombatComponent` (`/Game/Libs/BP_GlobalGetters.GetCharacterByActor` (`self.GetOwner`))) (`|CreateDelegate` :!event `OnCombatStateChanged`)))

(event `self.ReceiveTick`
  (params (DeltaSeconds :type "Float (single-precision)"))
  (if (`self.InteractionModeEnabled`)
    (`self.TraceForInteractionActor`)))

(fn `ApplyActionToDetectedActor`
  (`/Engine/EditorBlueprintResources/StandardMacros.IsValid` (`self.DetectedInteractableActor`)
    (:`Is Valid`
      (`/Game/Blueprints/Common/BP_Interaction.ApplyAction` (`self.DetectedInteractableActor`)))))

(fn `OnCombatStateChanged`
  (params (In :type "/Game/Data/Enums/E_CharacterAnimState Enum" :default "NewEnumerator0"))
  (if (`|EnumInequality` In "NewEnumerator0")
    (set `self.InteractionModeEnabled` false)))

(fn `OnRep_InteractionModeEnabled`
  (if (and (not (`self.InteractionModeEnabled`)) (`KismetSystemLibrary.IsValid` (`self.DetectedInteractableActor`)))
    (`/Game/Blueprints/Common/BP_Interaction.ToggleOutline` (`self.DetectedInteractableActor`) false)
    (set `self.DetectedInteractableActor` null)))

(fn `ToggleInteractionMode`
  (params (Enable :type Boolean))
  (bind _output_get (set `self.InteractionModeEnabled` Enable))
  (`self.InteractionModeToggled` _output_get))

(fn `TraceForInteractionActor`
  (bind _camera (`/Game/Blueprints/Characters/Player/BP_Character.Camera` (`/Game/Libs/BP_GlobalGetters.GetCharacterByActor` (`self.GetOwner`))))
  (bind _outhit (`KismetSystemLibrary.LineTraceSingleForObjects` (`SceneComponent.K2_GetComponentLocation` _camera) (+ (`/Game/Base/Blueprints/BP_HUD_Base.GetActionHandLocation` (`/Game/Libs/BP_GlobalGetters.GetHudByActor` (`self.GetOwner`))) (* (`SceneComponent.GetForwardVector` _camera) 350)) (`|MakeArray` "ObjectTypeQuery1" :!type "EObjectTypeQuery Enum")))
  (bind _asbp_interaction (cast `/Game/Blueprints/Common/BP_Interaction` (`.HitActor` (`GameplayStatics.BreakHitResult` _outhit)))
    (:`then`
      (if (!= _asbp_interaction (`self.DetectedInteractableActor`))
        (`|ExecutionSequence`
          (:`then_0`
            (`/Engine/EditorBlueprintResources/StandardMacros.IsValid` (`self.DetectedInteractableActor`)
              (:`Is Valid`
                (`/Game/Blueprints/Common/BP_Interaction.AssingInteractionController` (`self.DetectedInteractableActor`) null)
                (`/Game/Blueprints/Common/BP_Interaction.ToggleOutline` (`self.DetectedInteractableActor`) false))))
          (:`then_1`
            (bind _output_get (set `self.DetectedInteractableActor` _asbp_interaction))
            (`/Game/Blueprints/Common/BP_Interaction.AssingInteractionController` (`self.DetectedInteractableActor`) (`/Game/Libs/BP_GlobalGetters.GetControllerByCharacter` (`/Game/Libs/BP_GlobalGetters.GetCharacterByActor` (`self.GetOwner`))))
            (`/Game/Blueprints/Common/BP_Interaction.ToggleOutline` (`self.DetectedInteractableActor`) true)
            (`self.InteractableActorDetected` _output_get)))))
    (:`CastFailed`
      (`self.InteractableActorIgnored`)
      (`/Engine/EditorBlueprintResources/StandardMacros.IsValid` (`self.DetectedInteractableActor`)
        (:`Is Valid`
          (`/Game/Blueprints/Common/BP_Interaction.AssingInteractionController` (`self.DetectedInteractableActor`) null)
          (`/Game/Blueprints/Common/BP_Interaction.ToggleOutline` (`self.DetectedInteractableActor`) false)
          (set `self.DetectedInteractableActor` null))))))