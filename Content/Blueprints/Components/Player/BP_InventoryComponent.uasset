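; Player inventory component that stores item data by slot index and tracks equipped rifles, handgun and armor.
; Adding and removing items syncs with the HUD inventory widget, whose equipment slot events, bound by a self-disabling Tick once the widget exists, update slot indices.
; Combining delegates to each item's CombineRule, then splits off any stack remainder.
; Dropped items spawn at the first unobstructed point found by radial line traces around the owner.
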(event `self.ReceiveTick`
  (params (DeltaSeconds :type "Float (single-precision)"))
  (`/Engine/EditorBlueprintResources/StandardMacros.IsValid` (`/Game/Libs/BP_GlobalGetters.GetHudByActor` (`self.GetOwner`))
    (:`Is Valid`
      (`/Engine/EditorBlueprintResources/StandardMacros.IsValid` (`/Game/Base/Blueprints/BP_HUD_Base.Inventory_Widget` (`/Game/Libs/BP_GlobalGetters.GetHudByActor` (`self.GetOwner`)))
        (:`Is Valid`
          (`KismetSystemLibrary.Delay` 0.1) ; Need to avoid "Init subscription" failure
          (`self.InitSubscriptions`)
          (`self.SetComponentTickEnabled` false))))))

(fn `AddItem`
  (params (ItemData :type "/Game/Data/Structs/S_InventoryItemData Structure"))
  (returns (ItemAdded :type Boolean))
  (locals (L_SlotIndex :type Integer :default 0) (L_W_Inventory :type "/Game/UI/Inventory/W_Inventory Object Reference") (L_ItemData :type "/Game/Data/Structs/S_InventoryItemData Structure") (L_W_SelectedSlot :type "/Game/UI/Inventory/W_InventorySlot Object Reference") (L_W_StatusBar :type "/Game/UI/HUD/W_HUD_StatusBar Object Reference"))
  (bind (_id _name _description _type _image _cells _placement _isstackable _chargelimit _charge _amount _actions _realitemclass _inventoryitemclass _actorbridge) (break `/Game/Data/Structs/S_InventoryItemData` (`local.L_ItemData`)))
  (bind (_id_2 _name_2 _description_2 _type_2 _image_2 _cells_2 _placement_2 _isstackable_2 _chargelimit_2 _charge_2 _amount_2) (break `/Game/Data/Structs/S_InventoryItemData` (`local.L_ItemData`)))
  (bind _out (`/Game/Libs/BP_GlobalGetters.GetHudByActor` (`self.GetOwner`)))
  (set `local.L_ItemData` ItemData)
  (set `local.L_W_Inventory` (`/Game/Base/Blueprints/BP_HUD_Base.Inventory_Widget` _out))
  (set `local.L_W_StatusBar` (`/Game/UI/HUD/W_HUD.W_HUD_StatusBar` (`/Game/Base/Blueprints/BP_HUD_Base.HUD_Widget` _out)))
  (bind (_slotindex _itemplaced _actiontoplace) (`/Game/UI/Inventory/W_Inventory.AddItem` (`local.L_W_Inventory`) (`local.L_ItemData`)))
  (set `local.L_SlotIndex` _slotindex)
  (if _itemplaced
    (set `local.L_W_SelectedSlot` (`/Game/UI/Inventory/W_Inventory.GetSlot` (`local.L_W_Inventory`) (`local.L_SlotIndex`)))
    (`|ExecutionSequence`
      (:`then_0`
        (`/Engine/EditorBlueprintResources/StandardMacros.IsValid` _actorbridge
          (:`Is Valid`
            (`/Game/Blueprints/Inventory/ActorBridges/BP_Base_ActorBridge.AddSlot` _actorbridge (`local.L_W_SelectedSlot`))
            (`/Game/Blueprints/Inventory/ActorBridges/BP_Base_ActorBridge.AssignStatusBarWidget` _actorbridge (`local.L_W_StatusBar`)))))
      (:`then_1`
        (switch `/Game/Data/Enums/E_InventorySlotModifyOption` _actiontoplace
          (:`NewEnumerator2`
            (return false))
          (:`NewEnumerator3`
            (`BlueprintMapLibrary.Map_Add` (`self.Items`) (`local.L_SlotIndex`) (`local.L_ItemData`)))
          (:`NewEnumerator0`
            (`self.ModifyItemCharge` (`local.L_SlotIndex`) _charge_2))
          (:`NewEnumerator1`
            (`self.ModifyItemAmount` (`local.L_SlotIndex`) _amount_2))))
      (:`then_2`
        (`/Game/UI/Inventory/W_InventorySlot.UpdateDisplayInfo` (`local.L_W_SelectedSlot`))
        (`self.ItemAdded` (`local.L_SlotIndex`))
        (return true)))
    (else
      (return false))))

(fn `ClearCombine`
  (locals (L_W_Inventory :type "/Game/UI/Inventory/W_Inventory Object Reference"))
  (set `local.L_W_Inventory` (`/Game/Base/Blueprints/BP_HUD_Base.Inventory_Widget` (`/Game/Libs/BP_GlobalGetters.GetHudByActor` (`self.GetOwner`))))
  (for _array_element (`|MakeArray` (`self.FirstItemIndexToCombine`) (`self.SecondItemIndexToCombine`))
    (bind (_out _found) (`/Game/UI/Inventory/W_Inventory.GetSlot` (`local.L_W_Inventory`) _array_element))
    (if _found
      (`/Game/UI/Inventory/W_InventorySlot.ResetCombineModeOutline` _out)))
  (bind _output_get (set `self.FirstItemIndexToCombine` -1))
  (set `self.SecondItemIndexToCombine` _output_get))

(fn `CombineItems`
  (locals (L_W_Inventory :type "/Game/UI/Inventory/W_Inventory Object Reference") (L_CombineSicceeded :type Boolean :default false) (L_SecondItemDataBackup :type "/Game/Data/Structs/S_InventoryItemData Structure") (L_SecondItemDataRest :type "/Game/Data/Structs/S_InventoryItemData Structure"))
  (bind (_id _name _description _type _image _cells _placement _isstackable _chargelimit _charge _amount) (break `/Game/Data/Structs/S_InventoryItemData` (`local.L_SecondItemDataBackup`)))
  (bind _out (`self.GetItem` (`self.SecondItemIndexToCombine`)))
  (bind (_out_2 _found) (`self.GetItem` (`self.FirstItemIndexToCombine`)))
  (bind (_out_3 _found_2) (`self.GetItem` (`self.SecondItemIndexToCombine`)))
  (bind _out_4 (`/Game/Libs/BP_GlobalGetters.GetHudByActor` (`self.GetOwner`)))
  (bind (_id_2 _name_2 _description_2 _type_2 _image_2 _cells_2 _placement_2 _isstackable_2 _chargelimit_2 _charge_2 _amount_2 _actions _realitemclass _inventoryitemclass _actorbridge _combinerule) (break `/Game/Data/Structs/S_InventoryItemData` _out_2))
  (bind (_id_3 _name_3 _description_3 _type_3 _image_3 _cells_3 _placement_3 _isstackable_3 _chargelimit_3 _charge_3 _amount_3) (break `/Game/Data/Structs/S_InventoryItemData` _out))
  (`|ExecutionSequence`
    (:`then_0`
      (if (and _found _found_2)
        (set `local.L_SecondItemDataBackup` _out_3)
        (`/Engine/EditorBlueprintResources/StandardMacros.IsValid` _combinerule
          (:`Is Valid`
            (bind _combinesucceeded (`/Game/Blueprints/Inventory/CombineRules/BP_Base_CombineRule.CombineItems` _combinerule (`self.FirstItemIndexToCombine`) (`self.SecondItemIndexToCombine`) self))
            (set `local.L_CombineSicceeded` _combinesucceeded)))))
    (:`then_1`
      (if (`local.L_CombineSicceeded`)
        ;[1 1 1] Remove item if its amount is zero
        (if (== _amount_3 0)
          (`self.RemoveItem` (`self.SecondItemIndexToCombine`))
          (else
            ;[1 1 1] Dublicate item if combination proccess produced the rest
            (if (and (!= _charge _charge_3) (> _amount 1))
              (set `local.L_SecondItemDataRest` _out)
              (`|ExecutionSequence`
                (:`then_0`
                  (bind _structout (setmembers `/Game/Data/Structs/S_InventoryItemData` :`StructRef` (`|Copy` (`local.L_SecondItemDataRest`)) :`Charge` _charge :`Amount` (- _amount_3 1)))
                  (`self.RewriteItem` (`self.SecondItemIndexToCombine`) _structout))
                (:`then_1`
                  (bind _structout_2 (setmembers `/Game/Data/Structs/S_InventoryItemData` :`StructRef` (`|Copy` (`local.L_SecondItemDataRest`)) :`Amount` 1))
                  (bind _itemadded (`self.AddItem` _structout_2))
                  (if (not _itemadded)
                    (`self.SpawnItem` _structout_2)))))))))
    (:`then_2`
      (`/Engine/EditorBlueprintResources/StandardMacros.IsValid` _out_4
        (:`Is Valid`
          (set `local.L_W_Inventory` (`/Game/Base/Blueprints/BP_HUD_Base.Inventory_Widget` _out_4))
          (for _array_element (`|MakeArray` (`self.FirstItemIndexToCombine`) (`self.SecondItemIndexToCombine`))
            (bind (_out_5 _found_3) (`/Game/UI/Inventory/W_Inventory.GetSlot` (`local.L_W_Inventory`) _array_element))
            (if _found_3
              (`/Game/UI/Inventory/W_InventorySlot.UpdateDisplayInfo` _out_5)))
          (`/Game/UI/Inventory/W_Inventory.UpdateEquipmentDisplayInfo` (`local.L_W_Inventory`)))))
    (:`then_3`
      (`self.CombineFinished` (`self.FirstItemIndexToCombine`) (`self.SecondItemIndexToCombine`))
      (bind _output_get (set `self.FirstItemIndexToCombine` -1))
      (set `self.SecondItemIndexToCombine` _output_get))))

(fn `DisarmHandgunSlot`
  (`self.HandgunSlotDisarmed` (`self.HandgunSlot`))
  (set `self.HandgunSlot` null))

(fn `DisarmRifleSlotOne`
  (`self.SlotOneDisarmed` (`self.RifleSlotOne`))
  (set `self.RifleSlotOne` null))

(fn `DisarmRifleSlotTwo`
  (`self.SlotTwoDisarmed` (`self.RifleSlotTwo`))
  (set `self.RifleSlotTwo` null))

(fn `EquipRifleToSlotOne`
  (params (RifleToEquip :type "/Game/Blueprints/Interfaces/BP_TwoHandedWeapon_Interface Interface"))
  (bind _output_get (set `self.RifleSlotOne` RifleToEquip))
  (`self.SlotOneEquipped` _output_get))

(fn `EquipRifleToSlotTwo`
  (params (RifleToEquip :type "/Game/Blueprints/Interfaces/BP_TwoHandedWeapon_Interface Interface"))
  (bind _output_get (set `self.RifleSlotTwo` RifleToEquip))
  (`self.SlotTwoEquipped` _output_get))

(fn `EquipToHandgunSlot`
  (params (HandgunToEquip :type "/Game/Blueprints/Interfaces/BP_OneHandedWeapon_Interface Interface"))
  (bind _output_get (set `self.HandgunSlot` HandgunToEquip))
  (`self.HandgunSlotEquipped` _output_get))

(fn `GetEquippedArmorItemCharge`
  (returns (Out :type Integer))
  (locals (L_W_Inventory :type "/Game/UI/Inventory/W_Inventory Object Reference"))
  (bind _armorslotindex (`self.ArmorSlotIndex`))
  (bind (_out _found) (`self.GetItem` _armorslotindex))
  (if (!= -1 _armorslotindex)
    (if _found
      (return (`.Charge_12_3F5CFC6849447618911FE689586EBF3B` (break `/Game/Data/Structs/S_InventoryItemData` _out)))
      (else
        _)))
  (return 0))

(fn `GetFromHandgunSlot`
  (returns (Handgun :type "/Game/Blueprints/Interfaces/BP_OneHandedWeapon_Interface Interface") (ItemIndex :type Integer))
  (return (`self.HandgunSlot`) (`self.WeaponSlot3Index`)))

(fn `GetItem`
  (params (Index :type Integer))
  (returns (Out :type "/Game/Data/Structs/S_InventoryItemData Structure") (Found :type Boolean))
  (bind (_value _returnvalue) (`BlueprintMapLibrary.Map_Find` (`self.Items`) Index))
  (return _value _returnvalue))

(fn `GetItemsById`
  (params (In :type String))
  (returns (Out :type "Array of Integer"))
  (locals (L_ItemIds :type "Array of Integer"))
  (bind _keys (`BlueprintMapLibrary.Map_Keys` (`self.Items`)))
  (for _array_element _keys
    (bind (_out _found) (`self.GetItem` _array_element))
    (if (and _found (`KismetStringLibrary.EqualEqual_StrStr` (`.ID_33_C85DBAA343F73909462E21B0374A3722` (break `/Game/Data/Structs/S_InventoryItemData` _out)) In))
      (`KismetArrayLibrary.Array_Add` (`local.L_ItemIds`) _array_element)))
  (return (`local.L_ItemIds`)))

(fn `GetRifleFromSlotOne`
  (returns (Rifle :type "/Game/Blueprints/Interfaces/BP_TwoHandedWeapon_Interface Interface") (ItemIndex :type Integer))
  (return (`self.RifleSlotOne`) (`self.WeaponSlot1Index`)))

(fn `GetRifleFromSlotTwo`
  (returns (Rifle :type "/Game/Blueprints/Interfaces/BP_TwoHandedWeapon_Interface Interface") (ItemIndex :type Integer))
  (return (`self.RifleSlotTwo`) (`self.WeaponSlot2Index`)))

(fn `InitSubscriptions`
  (bind _w_inventory (`self.W_Inventory`))
  (set `self.W_Inventory` (`/Game/Base/Blueprints/BP_HUD_Base.Inventory_Widget` (`/Game/Libs/BP_GlobalGetters.GetHudByActor` (`self.GetOwner`))))
  (for _array_element (`|MakeArray` (`/Game/UI/Inventory/W_Inventory.W_WeaponSlot1` _w_inventory) (`/Game/UI/Inventory/W_Inventory.W_WeaponSlot2` _w_inventory) (`/Game/UI/Inventory/W_Inventory.W_WeaponSlot3` _w_inventory) (`/Game/UI/Inventory/W_Inventory.W_ArmorSlot` _w_inventory))
    (add `/Game/UI/Inventory/W_InventorySlot.ItemAssigned` _array_element (`|CreateDelegate` :!event `OnItemAssignedToSlot`))
    (add `/Game/UI/Inventory/W_InventorySlot.ItemRemoved` _array_element (`|CreateDelegate` :!event `OnItemRemovedFromSlot`))))

(fn `IsCombineModeEnabled`
  (returns (Out :type Boolean))
  (return (!= (`self.FirstItemIndexToCombine`) -1)))

(fn `ModifyItemAmount`
  (params (ItemIndex :type Integer) (Quantity :type Integer))
  (bind _value (`BlueprintMapLibrary.Map_Find` (`self.Items`) ItemIndex))
  (bind _returnvalue (+ (`.Amount_16_1F1E155B4AA399D443274FA1A73C83C4` (break `/Game/Data/Structs/S_InventoryItemData` _value)) Quantity))
  (bind _structout (setmembers `/Game/Data/Structs/S_InventoryItemData` :`StructRef` _value :`Amount` (`KismetMathLibrary.SelectInt` _returnvalue 0 (>= _returnvalue 0))))
  (`BlueprintMapLibrary.Map_Add` (`self.Items`) ItemIndex _structout))

(fn `ModifyItemCharge`
  (params (ItemIndex :type Integer) (Quantity :type Integer))
  (bind _value (`BlueprintMapLibrary.Map_Find` (`self.Items`) ItemIndex))
  (bind _returnvalue (+ (`.Charge_12_3F5CFC6849447618911FE689586EBF3B` (break `/Game/Data/Structs/S_InventoryItemData` _value)) Quantity))
  (bind _structout (setmembers `/Game/Data/Structs/S_InventoryItemData` :`StructRef` _value :`Charge` (`KismetMathLibrary.SelectInt` _returnvalue 0 (>= _returnvalue 0))))
  (`BlueprintMapLibrary.Map_Add` (`self.Items`) ItemIndex _structout))

(fn `OnItemAssignedToSlot`
  (params (ItemIndex :type Integer) (SlotType :type "/Game/Data/Enums/E_InventorySlotType Enum" :default "NewEnumerator0") (SlotName :type String))
  (locals (L_ItemIndex :type Integer) (L_SlotName :type String))
  (bind _l_itemindex (`local.L_ItemIndex`))
  (set `local.L_ItemIndex` ItemIndex)
  (set `local.L_SlotName` SlotName)
  (if (`|EnumEquality` SlotType "NewEnumerator1")
    (switch `string` (`local.L_SlotName`)
      (:`W_WeaponSlot1`
        (set `self.WeaponSlot1Index` _l_itemindex))
      (:`W_WeaponSlot2`
        (set `self.WeaponSlot2Index` _l_itemindex))
      (:`W_WeaponSlot3`
        (set `self.WeaponSlot3Index` _l_itemindex))
      (:`W_ArmorSlot`
        (set `self.ArmorSlotIndex` _l_itemindex)))))

(fn `OnItemRemovedFromSlot`
  (params (ItemIndex :type Integer) (SlotType :type "/Game/Data/Enums/E_InventorySlotType Enum" :default "NewEnumerator0") (SlotName :type String))
  (locals (L_ItemIndex :type Integer) (L_SlotName :type String))
  (bind _l_itemindex (`local.L_ItemIndex`))
  (set `local.L_ItemIndex` -1)
  (set `local.L_SlotName` SlotName)
  (if (`|EnumEquality` SlotType "NewEnumerator1")
    (switch `string` (`local.L_SlotName`)
      (:`W_WeaponSlot1`
        (set `self.WeaponSlot1Index` _l_itemindex))
      (:`W_WeaponSlot2`
        (set `self.WeaponSlot2Index` _l_itemindex))
      (:`W_WeaponSlot3`
        (set `self.WeaponSlot3Index` _l_itemindex))
      (:`W_ArmorSlot`
        (set `self.ArmorSlotIndex` _l_itemindex)))))

(fn `RemoveItem`
  (params (ItemIndex :type Integer))
  (returns (ItemRemoved :type Boolean))
  (locals (L_W_Inventory :type "/Game/UI/Inventory/W_Inventory Object Reference"))
  (bind _out (`/Game/Libs/BP_GlobalGetters.GetHudByActor` (`self.GetOwner`)))
  (bind _returnvalue (`BlueprintMapLibrary.Map_Remove` (`self.Items`) ItemIndex))
  (`/Engine/EditorBlueprintResources/StandardMacros.IsValid` _out
    (:`Is Valid`
      (`/Game/UI/Inventory/W_Inventory.RemoveItem` (`/Game/Base/Blueprints/BP_HUD_Base.Inventory_Widget` _out) ItemIndex)
      (return _returnvalue))))

(fn `RewriteItem`
  (params (ItemIndex :type Integer) (ItemData :type "/Game/Data/Structs/S_InventoryItemData Structure"))
  (`BlueprintMapLibrary.Map_Add` (`self.Items`) ItemIndex ItemData))

(fn `SetFirstSlotToCombine`
  (params (ItemIndex :type Integer))
  (set `self.FirstItemIndexToCombine` ItemIndex))

(fn `SetSecondSlotToCombine`
  (params (ItemIndex :type Integer))
  (set `self.SecondItemIndexToCombine` ItemIndex))

(fn `SpawnItem`
  (params (ItemData :type "/Game/Data/Structs/S_InventoryItemData Structure"))
  (returns (ItemSpawned :type Boolean))
  (locals (LocationToSpawn :type "Vector Structure") (RotationIterationAmount :type Integer :default 8) (ForwardVectorMultiplier :type Integer :default 75) (LocationFound :type Boolean))
  (bind _returnvalue (`self.GetOwner`))
  (bind _rotationiterationamount (`local.RotationIterationAmount`))
  (bind _returnvalue_2 (`Actor.K2_GetActorLocation` _returnvalue))
  (`|ExecutionSequence`
    (:`then_0`
      (for _index (range _rotationiterationamount)
        (bind _returnvalue_3 (+ (`KismetMathLibrary.GreaterGreater_VectorRotator` (* (`Actor.GetActorForwardVector` _returnvalue) (`local.ForwardVectorMultiplier`)) (`KismetMathLibrary.MakeRotator` 0.0 0.0 (`KismetMathLibrary.Conv_IntToDouble` (* _index (/ 360 _rotationiterationamount))))) _returnvalue_2))
        (bind (_outhit _returnvalue_4) (`KismetSystemLibrary.LineTraceSingleForObjects` _returnvalue_2 _returnvalue_3 (`|MakeArray` "ObjectTypeQuery1" "ObjectTypeQuery3" :!type "EObjectTypeQuery Enum")))
        (if (not _returnvalue_4)
          (set `local.LocationToSpawn` _returnvalue_3)
          (set `local.LocationFound` true)
          (break))))
    (:`then_1`
      (if (`local.LocationFound`)
        (bind _returnvalue_5 (`|SpawnActorFromClass` (`.InventoryItemClass_39_8B96CBE6411954AA93AE15AC43F7D8A8` (break `/Game/Data/Structs/S_InventoryItemData` ItemData)) (`KismetMathLibrary.MakeTransform` (`local.LocationToSpawn`)) "Undefined" "OverrideRootScale" null null))
        (bind _asbp_item_base (cast `/Game/Blueprints/Items/Common/BP_Item_Base` _returnvalue_5)
          (:`then`
            (set `/Game/Blueprints/Items/Common/BP_Item_Base.ItemData` ItemData _asbp_item_base))
          (:`CastFailed`
            (set `local.LocationFound` false)))))
    (:`then_2`
      (return (`local.LocationFound`)))))

(fn `SpawnTwoHandedWeapon`
  (params (ItemIndex :type Integer))
  (returns (Out :type "/Game/Blueprints/Interfaces/BP_TwoHandedWeapon_Interface Interface") (Success :type Boolean))
  (bind (_out _found) (`self.GetItem` ItemIndex))
  (bind (_id _name _description _type _image _cells _placement _isstackable _chargelimit _charge _amount _actions _realitemclass) (break `/Game/Data/Structs/S_InventoryItemData` _out))
  (if _found
    (bind _returnvalue (`|SpawnActorFromClass` _realitemclass (`Actor.GetTransform` (`self.GetOwner`)) "Undefined" "OverrideRootScale" null null))
    (bind _asbp_firearm (cast `/Game/Blueprints/Weapons/BP_Firearm` _returnvalue)
      (:`then`
        (set `/Game/Blueprints/Weapons/BP_Firearm.BulletAmount` _charge _asbp_firearm)
        (set `/Game/Blueprints/Weapons/BP_Weapon.WeaponOwner` (`self.GetOwner`) _asbp_firearm)
        (bind _asbp_rifle (cast `/Game/Blueprints/Weapons/BP_Rifle` _returnvalue)
          (:`then`
            (return _asbp_rifle true))
          (:`CastFailed`
            (bind _asbp_shotgun (cast `/Game/Blueprints/Weapons/BP_Shotgun` _returnvalue)
              (:`then`
                (return _asbp_shotgun true))
              (:`CastFailed`
                (return null false))))))
      (:`CastFailed`
        _)))
  (return null false))

(fn `TakeItem`
  (params (In :type "/Game/Blueprints/Interfaces/BP_InventoryItem_Interface Interface"))
  (returns (ItemTaken :type Boolean))
  (bind _out (`/Game/Blueprints/Interfaces/BP_InventoryItem_Interface.GetItemData` In))
  (bind _itemadded (`self.AddItem` _out))
  (return _itemadded))

(fn `ThrowAwayEquippedItems`
  (bind (_rifle _itemindex) (`self.GetRifleFromSlotOne`))
  (bind (_rifle_2 _itemindex_2) (`self.GetRifleFromSlotTwo`))
  (bind (_handgun _itemindex_3) (`self.GetFromHandgunSlot`))
  (`|ExecutionSequence`
    (:`then_0`
      (if (!= -1 _itemindex)
        (`self.DisarmRifleSlotOne`)
        (`self.ThrowAwayItem` _itemindex)))
    (:`then_1`
      (if (!= -1 _itemindex_2)
        (`self.DisarmRifleSlotTwo`)
        (`self.ThrowAwayItem` _itemindex_2)))
    (:`then_2`
      (if (!= -1 _itemindex_3)
        (`self.DisarmHandgunSlot`)
        (`self.ThrowAwayItem` _itemindex_3)))))

(fn `ThrowAwayItem`
  (params (ItemIndex :type Integer :default -1))
  (returns (ItemTrownAway :type Boolean))
  (locals (L_ItemIndex :type Integer))
  (bind (_out _found) (`self.GetItem` ItemIndex))
  (set `local.L_ItemIndex` ItemIndex)
  (if _found
    (bind _itemspawned (`self.SpawnItem` _out))
    (if _itemspawned
      (`self.RemoveItem` (`local.L_ItemIndex`))
      (return true)
      (else
        _)))
  (return false))