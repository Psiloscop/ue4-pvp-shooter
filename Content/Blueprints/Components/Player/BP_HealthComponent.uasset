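; Player health component that tracks health and death state and handles damage, healing and resurrection.
; Damage and healing update Health and fire dispatchers for damaged, healed or dead, with an IsDead flag so death is announced only once.
; Resurrection restores the class default Health, as does healing past a hardcoded cap of 100.
; A helper reports when health is low enough to need healing.
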(fn `DamageHealth`
  (params (Damage :type "Float (double-precision)"))
  (bind _returnvalue (- (`self.Health`) Damage))
  (if (> _returnvalue 0.0)
    (bind _output_get (set `self.Health` _returnvalue))
    (`self.CharacterDamaged` _output_get)
    (else
      (set `self.Health` 0.0)
      (if (not (`self.IsDead`))
        (`self.CharacterDead`)
        (set `self.IsDead` true)))))

(fn `DoesItNeedToBeHealed`
  (returns (Out :type Boolean))
  (return (<= (`self.Health`) 30.0)))

(fn `HealHealth`
  (params (Heal :type "Float (double-precision)"))
  (bind _returnvalue (+ Heal (`self.Health`)))
  (bind _output_get (set `self.Health` (select `bool` (> _returnvalue 100.0) :`false` _returnvalue :`true` (defaults `/Game/Blueprints/Components/Player/BP_HealthComponent` "BP_HealthComponent_C"))))
  (`self.CharacterHealed` _output_get))

(fn `Resurrect`
  (set `self.Health` (defaults `/Game/Blueprints/Components/Player/BP_HealthComponent` "BP_HealthComponent_C"))
  (set `self.IsDead` false))