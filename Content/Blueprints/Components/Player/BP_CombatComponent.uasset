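; Player combat component that manages combat state (Disarmed, Armed, Aiming) and Auto/Manual targeting.
; It tracks detected characters, dropping dead ones, and cycles to the next or nearest on-screen target with a clear line trace from the weapon muzzle.
; In Auto mode, Tick turns controller and owner yaw toward the target, interpolated when Armed, and falls back to Manual without a visible target.
; Mode changes fire dispatchers, and target switches update the HUD crosshair.
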(event `self.ReceiveBeginPlay`
  (add `/Game/Blueprints/Components/Player/BP_WeaponManagerComponent.FirearmTaken` (`/Game/Blueprints/Characters/Player/BP_Character.BP_WeaponManagerComponent` (`/Game/Libs/BP_GlobalGetters.GetCharacterByActor` (`self.GetOwner`))) (`|CreateDelegate` :!event `OnFirearmTaken`)))

(event `self.ReceiveTick`
  (params (DeltaSeconds :type "Float (single-precision)"))
  (if (`|EnumEquality` "NewEnumerator0" (`self.CombatModeType`))
    (`/Engine/EditorBlueprintResources/StandardMacros.IsValid` (`self.AimedCharacter`)
      (:`Is Valid`
        ;[1 1 1] Check if aimed char is still within the visible area
        (if (`self.IsLocationOnTheScreen` (`Actor.K2_GetActorLocation` (`self.AimedCharacter`))) :!label _label
          (`self.FaceToAim`)
          (else
            (`self.SwitchCombatType` :!label _label_2))))
      (:`Is Not Valid`
        (if (> (`KismetArrayLibrary.Array_Length` (`self.DetectedCharacters`)) 0)
          (`self.SwitchAim`)
          (`/Engine/EditorBlueprintResources/StandardMacros.IsValid` (`self.AimedCharacter`)
            (:`Is Valid`
              (goto _label))
            (:`Is Not Valid`
              (goto _label_2)))
          (else
            (goto _label_2)))))))

(fn `AddAim`
  (params (Character :type "/Game/Blueprints/Characters/BP_Base_Character Object Reference"))
  (`|ExecutionSequence`
    (:`then_0`
      (if (== (`KismetArrayLibrary.Array_Find` (`self.DetectedCharacters`) Character) -1)
        (`KismetArrayLibrary.Array_Add` (`self.DetectedCharacters`) Character)
        (add `/Game/Blueprints/Characters/BP_Base_Character.CharacterDead` Character (`|CreateDelegate` :!event `OnCharacterDeath`))))))

(fn `ChangeCombayState`
  (params (NewCombatState :type "/Game/Data/Enums/E_CharacterAnimState Enum" :default "NewEnumerator0"))
  (bind _output_get (set `self.CombatState` NewCombatState))
  (`self.CombatStateChanged` _output_get))

(fn `FaceToAim`
  (bind _returnvalue (`self.GetOwner`))
  (bind _out (`/Game/Libs/BP_GlobalGetters.GetControllerByCharacter` (`/Game/Libs/BP_GlobalGetters.GetCharacterByActor` (`self.GetOwner`))))
  (bind _returnvalue_2 (`Controller.GetControlRotation` _out))
  (bind _yaw (.yaw (`KismetMathLibrary.FindLookAtRotation` (`Actor.K2_GetActorLocation` _returnvalue) (`Actor.K2_GetActorLocation` (`self.AimedCharacter`)))))
  (bind _returnvalue_3 (`KismetMathLibrary.MakeRotator` 0.0 0.0 _yaw))
  (bind _returnvalue_4 (`KismetMathLibrary.MakeRotator` (.roll _returnvalue_2) (.pitch _returnvalue_2) _yaw))
  (if (`|EnumEquality` (`self.CombatState`) "NewEnumerator1")
    (`Controller.SetControlRotation` _out (`KismetMathLibrary.RInterpTo` _returnvalue_2 _returnvalue_4 (`GameplayStatics.GetWorldDeltaSeconds`) 3.0))
    (`Actor.K2_SetActorRotation` _returnvalue (`KismetMathLibrary.RInterpTo` (`Actor.K2_GetActorRotation` _returnvalue) _returnvalue_3 (`GameplayStatics.GetWorldDeltaSeconds`) 3.0) false)
    (else
      (`Controller.SetControlRotation` _out _returnvalue_4)
      (`Actor.K2_SetActorRotation` _returnvalue _returnvalue_3 false))))

(fn `GetWeaponLocation`
  (returns (Out :type "Vector Structure"))
  (`/Engine/EditorBlueprintResources/StandardMacros.IsValid` (`KismetSystemLibrary.Conv_InterfaceToObject` (`self.Weapon`))
    (:`Is Valid`
      (bind _out (`/Game/Blueprints/Interfaces/BP_SpecificFirearmWeapon_Interface.GetFireshotTransform` (cast `/Game/Blueprints/Interfaces/BP_SpecificFirearmWeapon_Interface` (`KismetSystemLibrary.Conv_InterfaceToObject` (`self.Weapon`)) :!pure true)))
      (return (.location _out)))
    (:`Is Not Valid`
      (return (0.0 0.0 0.0)))))

(fn `IsAimVisible`
  (params (Character :type "Character Object Reference"))
  (returns (Out :type Boolean))
  (locals (L_PlayerLocation :type "Vector Structure" :default (0.0 0.0 0.0)))
  (bind _returnvalue (`Actor.K2_GetActorLocation` Character))
  (if (and (`self.IsLocationOnTheScreen` _returnvalue) (`self.IsWayToAimClear` (`Actor.K2_GetActorLocation` (`self.GetOwner`)) _returnvalue Character))
    (return true)
    (else
      (return false))))

(fn `IsLocationOnTheScreen`
  (params (In :type "Vector Structure"))
  (returns (Out :type Boolean))
  (bind (_returnvalue_x _returnvalue_y) (`KismetMathLibrary.BreakVector2D` (`WidgetLayoutLibrary.GetViewportSize`)))
  (bind _screenlocation (`PlayerController.ProjectWorldLocationToScreen` (`/Game/Libs/BP_GlobalGetters.GetControllerByCharacter` (`/Game/Libs/BP_GlobalGetters.GetCharacterByActor` (`self.GetOwner`))) In false))
  (return (and (> (`KismetMathLibrary.BreakVector2D` _screenlocation) 0.0) (> (`.Y` (`KismetMathLibrary.BreakVector2D` _screenlocation)) 0.0) (< (`KismetMathLibrary.BreakVector2D` _screenlocation) _returnvalue_x) (< (`.Y` (`KismetMathLibrary.BreakVector2D` _screenlocation)) _returnvalue_y))))

(fn `IsWayToAimClear`
  (params (From :type "Vector Structure") (To :type "Vector Structure") (ExpectedAim :type "Actor Object Reference"))
  (returns (Out :type Boolean))
  (bind _outhit (`KismetSystemLibrary.LineTraceSingleForObjects` From To (`|MakeArray` "ObjectTypeQuery1" "ObjectTypeQuery1" "ObjectTypeQuery3" :!type "EObjectTypeQuery Enum") false (`|MakeArray` (`self.GetOwner`))))
  (return (== ExpectedAim (`.HitActor` (`GameplayStatics.BreakHitResult` _outhit)))))

(fn `OnCharacterDeath`
  (params (Character :type "/Game/Blueprints/Characters/BP_Base_Character Object Reference"))
  (remove `/Game/Blueprints/Characters/BP_Base_Character.CharacterDead` Character (`|CreateDelegate` :!event `OnCharacterDeath`))
  (`self.RemoveAim` Character)
  (if (> (`KismetArrayLibrary.Array_Length` (`self.DetectedCharacters`)) 0)
    (`self.SwitchAim`)
    (else
      (set `self.AimedCharacter` null)
      (if (`|EnumEquality` (`self.CombatModeType`) "NewEnumerator0")
        (`self.SwitchCombatType`)))))

(fn `OnFirearmTaken`
  (params (Weapon :type "/Game/Blueprints/Interfaces/BP_Weapon_Interface Interface") (FirearmType :type "/Game/Data/Enums/E_FirearmType Enum" :default "NewEnumerator0") (ItemIndex :type Integer))
  (set `self.Weapon` Weapon))

(fn `RemoveAim`
  (params (Character :type "/Game/Blueprints/Characters/BP_Base_Character Object Reference"))
  (bind _returnvalue (`KismetArrayLibrary.Array_RemoveItem` (`self.DetectedCharacters`) Character))
  (if (and _returnvalue (== Character (`self.AimedCharacter`)))
    (set `self.AimedCharacter` null)))

(fn `SwitchAim`
  (locals (L_PlayerLocation :type "Vector Structure" :default (0.0 0.0 0.0)) (L_NearestCharacter :type "Character Object Reference"))
  (bind _detectedcharacters (`self.DetectedCharacters`))
  (bind _l_nearestcharacter (`local.L_NearestCharacter`))
  (bind _l_nearestcharacter_2 (`local.L_NearestCharacter`))
  (bind _aimedcharacter (`self.AimedCharacter`))
  (bind _detectedcharacters_2 (`self.DetectedCharacters`))
  (bind _l_playerlocation (`local.L_PlayerLocation`))
  (bind _returnvalue (`KismetArrayLibrary.Array_Length` _detectedcharacters))
  (bind _returnvalue_2 (`Actor.K2_GetActorLocation` _l_nearestcharacter))
  (bind _returnvalue_3 (+ (`KismetArrayLibrary.Array_Find` _detectedcharacters _aimedcharacter) 1))
  (if (`|EnumEquality` "NewEnumerator0" (`self.CombatModeType`))
    (`|ExecutionSequence`
      (:`then_0`
        (`/Engine/EditorBlueprintResources/StandardMacros.IsValid` _aimedcharacter
          (:`Is Valid`
            (if (!= _returnvalue_3 _returnvalue)
              (for _index (range _returnvalue_3 _returnvalue)
                (bind _output (`|GetArrayItem` (`self.DetectedCharacters`) _index))
                (bind _returnvalue_4 (`Actor.K2_GetActorLocation` _output))
                (if (and (`self.IsLocationOnTheScreen` _returnvalue_4) (`self.IsWayToAimClear` (`self.GetWeaponLocation`) _returnvalue_4 _output))
                  (set `local.L_NearestCharacter` _output)
                  (break)))
              (`/Engine/EditorBlueprintResources/StandardMacros.IsValid` _l_nearestcharacter_2
                (:`Is Valid`
                  (set `self.AimedCharacter` _l_nearestcharacter_2))
                (:`Is Not Valid`
                  (set `local.L_PlayerLocation` (`Actor.K2_GetActorLocation` (`self.GetOwner` self)) :!label _label)
                  (set `local.L_NearestCharacter` (`|GetArrayItem` _detectedcharacters_2))
                  (for _array_element _detectedcharacters_2
                    (bind _returnvalue_5 (`Actor.K2_GetActorLocation` _array_element))
                    (if (and (!= _array_element (`self.AimedCharacter`)) (`self.IsLocationOnTheScreen` _returnvalue_5) (`self.IsWayToAimClear` (`self.GetWeaponLocation`) _returnvalue_5 _array_element) (< (`KismetMathLibrary.VSize` (- _returnvalue_5 _l_playerlocation)) (`KismetMathLibrary.VSize` (- (`Actor.K2_GetActorLocation` (`local.L_NearestCharacter`)) _l_playerlocation))))
                      (set `local.L_NearestCharacter` _array_element)))
                  (if (and (`self.IsLocationOnTheScreen` _returnvalue_2) (`self.IsWayToAimClear` (`self.GetWeaponLocation`) _returnvalue_2 _l_nearestcharacter))
                    (set `self.AimedCharacter` _l_nearestcharacter))))
              (else
                (goto _label))))
          (:`Is Not Valid`
            (goto _label))))
      (:`then_1`
        (`/Game/Base/Blueprints/BP_HUD_Base.UpdateAutoCrosshairData` (`/Game/Libs/BP_GlobalGetters.GetHudByActor` (`self.GetOwner`)) (`self.AimedCharacter`))))))

(fn `SwitchCombatType`
  (switch `/Game/Data/Enums/E_CombatModeType` (`self.CombatModeType`)
    (:`NewEnumerator0`
      (bind _output_get (set `self.CombatModeType` "NewEnumerator1"))
      (`self.CombatModeSwitched` _output_get))
    (:`NewEnumerator1`
      (bind _output_get_2 (set `self.CombatModeType` "NewEnumerator0"))
      (`self.CombatModeSwitched` _output_get_2)
      (set `self.AimedCharacter` null))))

(fn `ToggleCombatMode`
  (params (Enable :type Boolean))
  (if Enable
    (bind _output_get (set `self.CombatState` "NewEnumerator1"))
    (`self.CombatStateChanged` _output_get)
    (else
      (bind _output_get_2 (set `self.CombatModeType` "NewEnumerator1"))
      (`self.CombatModeSwitched` _output_get_2)
      (set `self.AimedCharacter` null)
      (bind _output_get_3 (set `self.CombatState` "NewEnumerator0"))
      (`self.CombatStateChanged` _output_get_3))))

(fn `ToggleCombatState`
  (switch `/Game/Data/Enums/E_CharacterAnimState` (`self.CombatState`)
    (:`NewEnumerator1`
      (bind _output_get (set `self.CombatState` "NewEnumerator2"))
      (`self.CombatStateChanged` _output_get))
    (:`NewEnumerator2`
      (bind _output_get_2 (set `self.CombatState` "NewEnumerator1"))
      (`self.CombatStateChanged` _output_get_2))))