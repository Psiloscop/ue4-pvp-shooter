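; Player component that manages the owning character's pose (stand, crouch, prone, jump) and its sprint, jump and aim actions.
; Action calls update an action stack that sets movement permission flags and walk speed.
; Removing an action reapplies the latest remaining Sprint or Aim, or clears restrictions when the stack is empty.
; Tick syncs the Jump pose with the movement component's falling state; aiming parameters are an empty stub.
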(event `self.ReceiveBeginPlay`
  (bind _out (`/Game/Libs/BP_GlobalGetters.GetCharacterByActor` (`self.GetOwner`)))
  (set `self.MovementComponent` (`Pawn.GetMovementComponent` _out))
  (set `self.Character` _out))

(event `self.ReceiveTick`
  (params (DeltaSeconds :type "Float (single-precision)"))
  (`self.UpdatePose`))

(fn `Aim`
  (params (Start :type Boolean))
  (if Start
    (if (`self.IsAbleToChangePose`)
      (`self.ProcessActionStack` "NewEnumerator4" true))
    (else
      (`self.ProcessActionStack` "NewEnumerator4"))))

(fn `CancelAllRestrictions`
  (set `self.IsAbleToMove` true)
  (set `self.IsAbleToSprint` true)
  (set `self.IsAbleToJump` true)
  (set `self.IsAbleToAim` true))

(fn `ChangePose`
  (params (NewPose :type "/Game/Data/Enums/E_CharacterPoseState Enum" :default "NewEnumerator0"))
  (if (not (`|EnumInequality` NewPose "NewEnumerator0"))
    (set `self.IsAbleToChangePose` true))
  (switch `/Game/Data/Enums/E_CharacterPoseState` NewPose
    (:`NewEnumerator0`
      _)
    (:`NewEnumerator1`
      (set `self.IsAbleToChangePose` false :!label _label))
    (:`NewEnumerator2`
      (goto _label))
    (:`NewEnumerator3`
      (goto _label)))
  (set `self.PoseState` NewPose))

(fn `Crouch`
  (params (Start :type Boolean))
  (if Start
    (if (`self.IsAbleToChangePose`)
      (`self.ChangePose` "NewEnumerator1")
      (`self.ProcessActionStack` "NewEnumerator5" true))
    (else
      (`self.ChangePose` "NewEnumerator0")
      (`self.ProcessActionStack` "NewEnumerator5"))))

(fn `Jump`
  (params (Start :type Boolean))
  (bind _movementcomponent (`self.MovementComponent`))
  (if Start
    (if (`self.IsAbleToChangePose`)
      (`self.ChangePose` "NewEnumerator3")
      (`self.ProcessActionStack` "NewEnumerator1" true)
      (`Character.Jump` (`self.Character`))
      (bind _ascharacter_movement_component (cast `CharacterMovementComponent` _movementcomponent :!label _label))
      (if (> (`KismetMathLibrary.VSize` (`MovementComponent.Velocity` _movementcomponent)) 0.0)
        (set `CharacterMovementComponent.JumpZVelocity` 400.0 _ascharacter_movement_component)
        (else
          (set `CharacterMovementComponent.JumpZVelocity` 400.0 _ascharacter_movement_component))))
    (else
      (`self.ChangePose` "NewEnumerator0")
      (`self.ProcessActionStack` "NewEnumerator1")
      (`Character.StopJumping` (`self.Character`))
      (goto _label))))

(fn `ProcessActionStack`
  (params (ActionName :type "/Game/Data/Enums/E_CharacterAction Enum" :default "NewEnumerator0") (AddIt :type Boolean))
  (bind _currentactions (`self.CurrentActions`))
  (if AddIt
    (`KismetArrayLibrary.Array_Add` (`self.CurrentActions`) ActionName)
    (switch `/Game/Data/Enums/E_CharacterAction` ActionName
      (:`NewEnumerator0`
        (if (`self.IsAbleToSprint`)
          (`self.SetupSprintParams` true)
          (`self.SetupSprintRestrictions`)))
      (:`NewEnumerator1`
        (if (`self.IsAbleToJump`)
          (`self.SetupJumpRestrictions`)))
      (:`NewEnumerator4`
        (if (`self.IsAbleToAim`)
          (`self.SetupAimingParams` true)
          (`self.SetupAimRestrictions`)))
      (:`NewEnumerator5`
        (`self.SetupCrouchRestrictions`))
      (:`NewEnumerator6`
        (`self.SetupProneRestrictions`)))
    (else
      (`KismetArrayLibrary.Array_RemoveItem` _currentactions ActionName)
      (`|ExecutionSequence`
        (:`then_0`
          (switch `/Game/Data/Enums/E_CharacterAction` ActionName
            (:`NewEnumerator0`
              (`self.SetupSprintParams` false))
            (:`NewEnumerator4`
              (`self.SetupAimingParams` false))))
        (:`then_1`
          (if (== (`KismetArrayLibrary.Array_Length` _currentactions) 0)
            (`self.CancelAllRestrictions`)
            (else
              (switch `/Game/Data/Enums/E_CharacterAction` (`|GetArrayItem` _currentactions (`KismetArrayLibrary.Array_LastIndex` _currentactions))
                (:`NewEnumerator0`
                  (`self.SetupSprintParams` true)
                  (`self.SetupSprintRestrictions`))
                (:`NewEnumerator4`
                  (`self.SetupAimingParams` true)
                  (`self.SetupAimRestrictions`))))))))))

(fn `Prone`
  (params (Start :type Boolean))
  (if Start
    (if (`self.IsAbleToChangePose`)
      (`self.ChangePose` "NewEnumerator2")
      (`self.ProcessActionStack` "NewEnumerator6" true))
    (else
      (`self.ChangePose` "NewEnumerator0")
      (`self.ProcessActionStack` "NewEnumerator6"))))

(fn `SetupAimingParams`
  (params (Activate :type Boolean)))

(fn `SetupAimRestrictions`
  (set `self.IsAbleToMove` true)
  (set `self.IsAbleToSprint` false)
  (`self.SetupSprintParams` false))

(fn `SetupCrouchRestrictions`
  (set `self.IsAbleToMove` true)
  (set `self.IsAbleToSprint` false)
  (set `self.IsAbleToJump` false)
  (set `self.IsAbleToAim` true))

(fn `SetupJumpRestrictions`
  (set `self.IsAbleToMove` false)
  (set `self.IsAbleToSprint` false)
  (set `self.IsAbleToJump` false)
  (set `self.IsAbleToAim` false))

(fn `SetupProneRestrictions`
  (set `self.IsAbleToMove` false)
  (set `self.IsAbleToSprint` false)
  (set `self.IsAbleToJump` false)
  (set `self.IsAbleToAim` true))

(fn `SetupSprintParams`
  (params (Activate :type Boolean))
  (bind _movementcomponent (`/Game/Libs/BP_GlobalGetters.GetMovementComponent`))
  (if Activate
    (set `CharacterMovementComponent.MaxWalkSpeed` (`self.SprintSpeed`) _movementcomponent)
    (else
      (set `CharacterMovementComponent.MaxWalkSpeed` (`self.WalkSpeed`) _movementcomponent))))

(fn `SetupSprintRestrictions`
  (set `self.IsAbleToMove` true)
  (set `self.IsAbleToSprint` true)
  (set `self.IsAbleToJump` true)
  (set `self.IsAbleToAim` true))

(fn `SetupStandRestrictions`
  (set `self.IsAbleToMove` true)
  (set `self.IsAbleToSprint` true)
  (set `self.IsAbleToJump` true)
  (set `self.IsAbleToAim` true))

(fn `Sprint`
  (params (Start :type Boolean))
  (if (`self.IsAbleToChangePose`)
    (`self.ProcessActionStack` "NewEnumerator0" Start)))

(fn `UpdatePose`
  (if (and (`|EnumEquality` "NewEnumerator3" (`self.PoseState`)) (not (`NavMovementComponent.IsFalling` (`self.MovementComponent`))))
    (`self.ChangePose` "NewEnumerator0")
    (`self.SetupStandRestrictions`)
    (elif (and (`|EnumInequality` "NewEnumerator3" (`self.PoseState`)) (`NavMovementComponent.IsFalling` (`self.MovementComponent`)))
      (`self.ChangePose` "NewEnumerator3")
      (`self.SetupJumpRestrictions`))))