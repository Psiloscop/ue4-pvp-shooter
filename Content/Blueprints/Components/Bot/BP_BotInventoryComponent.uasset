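; Inventory component for bots that stores items and automates weapon and armor loadout choices.
; AddItem merges pickups into matching entries by charge or stack amount, otherwise creating a new entry.
; EquipWeapons spawns loaded or ammo-backed two-handed weapons into empty rifle slots, matched by hold type; the handgun slot is checked but never filled.
; Other routines disarm weapons lacking reserve ammo, discard nearly depleted armor and pick the highest-charge armor as an equip candidate.
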(fn `AddItem`
  (params (ItemData :type "/Game/Data/Structs/S_InventoryItemData Structure"))
  (returns (ItemAdded :type Boolean))
  (locals (L_ItemData :type "/Game/Data/Structs/S_InventoryItemData Structure") (L_SlotIndex :type Integer))
  (bind (_id _name _description _type _image _cells _placement _isstackable _chargelimit _charge _amount) (break `/Game/Data/Structs/S_InventoryItemData` (`local.L_ItemData`)))
  (bind _output_get (set `local.L_ItemData` ItemData))
  (bind (_indextoplace _actiontoplace) (`self.FindIndexToPlace` _output_get))
  (set `local.L_SlotIndex` _indextoplace)
  (`|ExecutionSequence`
    (:`then_0`
      (switch `/Game/Data/Enums/E_InventorySlotModifyOption` _actiontoplace
        (:`NewEnumerator2`
          (return false))
        (:`NewEnumerator3`
          (`BlueprintMapLibrary.Map_Add` (`self.Items`) (`local.L_SlotIndex`) (`local.L_ItemData`)))
        (:`NewEnumerator0`
          (`self.ModifyItemCharge` (`local.L_SlotIndex`) _charge))
        (:`NewEnumerator1`
          (`self.ModifyItemAmount` (`local.L_SlotIndex`) _amount))))
    (:`then_1`
      (`self.ItemAdded` (`local.L_SlotIndex`))
      (return true))))

(fn `DisarmEmptyWeapons`
  (for _array_element (`|MakeArray` (`self.WeaponSlot1Index`) (`self.WeaponSlot2Index`) (`self.WeaponSlot3Index`))
    (if (not (`self.HasWeaponBullets` _array_element))
      (switch `int` _array_element
        (:`1`
          (`self.DisarmRifleSlotOne`))
        (:`2`
          (`self.DisarmRifleSlotTwo`))
        (:`3`
          (`self.DisarmHandgunSlot`))))))

(fn `EquipArmor`
  (locals (CurrentArmorCharge :type Integer :default 0) (OwnedArmor :type "Array of Integer") (BestOffer :type Integer))
  (bind _items (`self.Items`))
  (bind _items_2 (`self.Items`))
  (bind (_value _returnvalue) (`BlueprintMapLibrary.Map_Find` (`self.Items`) (`self.ArmorSlotIndex`)))
  (`|ExecutionSequence`
    (:`then_0`
      (if _returnvalue
        (set `local.CurrentArmorCharge` (`.Charge_12_3F5CFC6849447618911FE689586EBF3B` (break `/Game/Data/Structs/S_InventoryItemData` _value)))))
    (:`then_1`
      (bind _keys (`BlueprintMapLibrary.Map_Keys` _items))
      (for _array_element _keys
        (if (`|EnumEquality` (`.Type_55_4FF7FFC44917CA832BB2249BB30345EC` (break `/Game/Data/Structs/S_InventoryItemData` (`BlueprintMapLibrary.Map_Find` _items _array_element))) "NewEnumerator1")
          (`KismetArrayLibrary.Array_Add` (`local.OwnedArmor`) _array_element))))
    (:`then_2`
      (if (> (`KismetArrayLibrary.Array_Length` (`local.OwnedArmor`)) 0)
        (set `local.BestOffer` (`|GetArrayItem` (`local.OwnedArmor`)))
        (for _array_element_2 (`local.OwnedArmor`)
          (if (> (`.Charge_12_3F5CFC6849447618911FE689586EBF3B` (break `/Game/Data/Structs/S_InventoryItemData` (`BlueprintMapLibrary.Map_Find` _items_2 _array_element_2))) (`.Charge_12_3F5CFC6849447618911FE689586EBF3B` (break `/Game/Data/Structs/S_InventoryItemData` (`BlueprintMapLibrary.Map_Find` _items_2 (`local.BestOffer`)))))
            (set `local.BestOffer` _array_element_2)))))
    (:`then_3`
      (if (> (`.ChargeLimit_32_70D8CD844ADA26FC121DA18A08B98E32` (break `/Game/Data/Structs/S_InventoryItemData` (`BlueprintMapLibrary.Map_Find` (`self.Items`) (`local.BestOffer`)))) (`local.CurrentArmorCharge`))
        (set `self.ArmorSlotIndex` (`local.BestOffer`))))))

(fn `EquipWeapons`
  (locals (L_HoldTypes :type "Map of Integer to Name") (L_EmptySlotNumbers :type "Array of Integer") (L_EquippedItems :type "Array of Integer") (L_Weapon :type "/Game/Blueprints/Interfaces/BP_TwoHandedWeapon_Interface Interface"))
  (`|ExecutionSequence`
    (:`then_0`
      (`BlueprintMapLibrary.Map_Add` (`local.L_HoldTypes`) 1 "two_handed")
      (`BlueprintMapLibrary.Map_Add` (`local.L_HoldTypes`) 2 "two_handed")
      (`BlueprintMapLibrary.Map_Add` (`local.L_HoldTypes`) 3 "one_handed"))
    (:`then_1`
      (for (_array_element _array_index) (`|MakeArray` (`.ItemIndex` (`self.GetRifleFromSlotOne`)) (`.ItemIndex` (`self.GetRifleFromSlotTwo`)) (`.ItemIndex` (`self.GetFromHandgunSlot`)))
        (if (== _array_element -1)
          (`KismetArrayLibrary.Array_Add` (`local.L_EmptySlotNumbers`) (+ _array_index 1)))))
    (:`then_2`
      (for _array_element_2 (`local.L_EmptySlotNumbers`)
        (bind _keys (`BlueprintMapLibrary.Map_Keys` (`self.Items`)))
        (for _array_element_3 _keys
          (if (not (`KismetArrayLibrary.Array_Contains` (`|MakeArray` (`self.WeaponSlot1Index`) (`self.WeaponSlot2Index`)) _array_element_3))
            (bind (_id _name _description _type _image _cells _placement _isstackable _chargelimit _charge _amount _actions _realitemclass _inventoryitemclass _actorbridge _combinerule _properties) (break `/Game/Data/Structs/S_InventoryItemData` (`BlueprintMapLibrary.Map_Find` (`self.Items`) _array_element_3)))
            (if (`|EnumEquality` _type "NewEnumerator0")
              (if (and (or (`self.HasWeaponBullets` _array_element_3) (> _charge 0)) (== (`BlueprintMapLibrary.Map_Find` _properties "hold_type") (`BlueprintMapLibrary.Map_Find` (`local.L_HoldTypes`) _array_element_2)) (== (`KismetArrayLibrary.Array_Find` (`local.L_EquippedItems`) _array_element_3) -1))
                (switch `int` _array_element_2
                  (:`1`
                    (bind _output_get (set `self.WeaponSlot1Index` _array_element_3))
                    (bind _out (`self.SpawnTwoHandedWeapon` _output_get))
                    (bind _output_get_2 (set `local.L_Weapon` _out))
                    (`self.EquipRifleToSlotOne` _output_get_2))
                  (:`2`
                    (bind _output_get_3 (set `self.WeaponSlot2Index` _array_element_3))
                    (bind _out_2 (`self.SpawnTwoHandedWeapon` _output_get_3))
                    (bind _output_get_4 (set `local.L_Weapon` _out_2))
                    (`self.EquipRifleToSlotTwo` _output_get_4)))
                (`/Game/Blueprints/Inventory/ActorBridges/BP_Base_ActorBridge.AssignObservable` _actorbridge (cast `Actor` (`KismetSystemLibrary.Conv_InterfaceToObject` (`local.L_Weapon`)) :!pure true) _array_element_3 self)
                (`KismetArrayLibrary.Array_Add` (`local.L_EquippedItems`) _array_element_3)))))))))

(fn `FindIndexToPlace`
  (params (ItemData :type "/Game/Data/Structs/S_InventoryItemData Structure"))
  (returns (IndexToPlace :type Integer) (ActionToPlace :type "/Game/Data/Enums/E_InventorySlotModifyOption Enum"))
  (locals (L_ItemID :type String) (L_ItemChargeLimit :type Integer) (L_ItemCharge :type Integer) (L_ItemCount :type Integer) (L_CurrentSlotIndex :type Integer))
  (bind (_id _name _description _type _image _cells _placement _isstackable _chargelimit _charge) (break `/Game/Data/Structs/S_InventoryItemData` ItemData))
  (bind _returnvalue (`BlueprintMapLibrary.Map_Length` (`self.Items`)))
  (set `local.L_ItemID` _id)
  (set `local.L_ItemChargeLimit` _chargelimit)
  (set `local.L_ItemCharge` _charge)
  (set `local.L_ItemCount` _returnvalue)
  (for _index (range (`local.L_ItemCount`))
    (bind _output_get (set `local.L_CurrentSlotIndex` _index))
    (bind (_out _found) (`self.GetItem` _output_get))
    (bind (_id_2 _name_2 _description_2 _type_2 _image_2 _cells_2 _placement_2 _isstackable_2 _chargelimit_2 _charge_2) (break `/Game/Data/Structs/S_InventoryItemData` _out))
    (if (and (`KismetStringLibrary.EqualEqual_StrStr` (`local.L_ItemID`) _id_2) _found)
      (`|ExecutionSequence`
        (:`then_0`
          (if (and (<= (+ _charge_2 (`local.L_ItemCharge`)) _chargelimit_2) (!= _chargelimit_2 0))
            (return (`local.L_CurrentSlotIndex`) "NewEnumerator0")))
        (:`then_1`
          (if (and _isstackable (== _chargelimit_2 _charge_2) (== (`local.L_ItemChargeLimit`) (`local.L_ItemCharge`)))
            (return (`local.L_CurrentSlotIndex`) "NewEnumerator1"))))))
  (return _returnvalue "NewEnumerator3"))

(fn `HasWeaponBullets`
  (params (ItemIndex :type Integer))
  (returns (Out :type Boolean))
  (for _array_element (`KismetStringLibrary.ParseIntoArray` (`KismetStringLibrary.Conv_NameToString` (`BlueprintMapLibrary.Map_Find` (`.Properties_63_2E93C90741D16E8EF8CBB8B002440FBA` (break `/Game/Data/Structs/S_InventoryItemData` (`self.GetItem` ItemIndex))) "ammo_item_ids")) ",")
    (for _array_element_2 (`self.GetItemsById` _array_element)
      (bind (_out _found) (`self.GetItem` _array_element_2))
      (if (and (> (`.Charge_12_3F5CFC6849447618911FE689586EBF3B` (break `/Game/Data/Structs/S_InventoryItemData` _out)) 0) _found)
        (return true)))
    (return false))
  (return false))

(fn `ThrowAwayWasteItems`
  (bind _keys (`BlueprintMapLibrary.Map_Keys` (`self.Items`)))
  (for _array_element _keys
    (bind (_id _name _description _type _image _cells _placement _isstackable _chargelimit _charge) (break `/Game/Data/Structs/S_InventoryItemData` (`BlueprintMapLibrary.Map_Find` (`self.Items`) _array_element)))
    (if (and (`|EnumEquality` _type "NewEnumerator1") (<= _charge 10))
      (`self.RemoveItem` _array_element))))