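; Bot patrol component that walks its AI-controlled owner along the points of BP_Spline actors gathered at BeginPlay.
; StartPatrolling picks the current spline's nearest point and a direction, then issues SimpleMoveToLocation; StopPatrolling halts movement.
; Helpers detect arrival by distance, step the point index, cycle splines or pick one randomly.
; The draft logic chaining these into a continuous patrol is disconnected, and Tick is empty.
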(event `self.ReceiveTick`
  (params (DeltaSeconds :type "Float (single-precision)"))
  ;[1 1 1] Draft
)

(event `self.ReceiveBeginPlay`
  (bind _outactors (`GameplayStatics.GetAllActorsOfClass` "/Game/Blueprints/Utility/BP_Spline.BP_Spline_C"))
  (set `self.Splines` _outactors))

(fn `FindNextPoint`
  (returns (Found :type Boolean))
  (if (`self.IsMovingForward`)
    (if (< (`self.CurrentSplinePointIndex`) (`SplineComponent.GetNumberOfSplinePoints` (`/Game/Blueprints/Utility/BP_Spline.Spline` (`|GetArrayItem` (`self.Splines`) (`self.CurrentSplineIndex`)))))
      (`/Engine/EditorBlueprintResources/StandardMacros.IncrementInt` (`self.CurrentSplinePointIndex`)
        (:`  `
          (return true)))
      (else
        _))
    (elif (> (`self.CurrentSplinePointIndex`) 0)
      (`/Engine/EditorBlueprintResources/StandardMacros.DecrementInt` (`self.CurrentSplinePointIndex`)
        (:`  `
          (return true)))
      (else
        _)))
  (return false))

(fn `GetNearesSplinePointIndex`
  (params (SplineIndex :type Integer) (CharacterLocation :type "Vector Structure"))
  (returns (Out :type Integer) (ShouldMoveForward :type Boolean))
  (locals (L_NearestSplitePoint :type Integer) (L_ShortestLength :type "Float (double-precision)"))
  (bind _spline (`/Game/Blueprints/Utility/BP_Spline.Spline` (`|GetArrayItem` (`self.Splines`) SplineIndex)))
  (bind _returnvalue (`SplineComponent.GetNumberOfSplinePoints` _spline))
  (set `local.L_NearestSplitePoint` 1)
  (set `local.L_ShortestLength` (`KismetMathLibrary.VSize` (- CharacterLocation (`SplineComponent.GetLocationAtSplinePoint` _spline 0 "World"))))
  (for _index (range (+ _returnvalue 1))
    (bind _returnvalue_2 (`KismetMathLibrary.VSize` (- CharacterLocation (`SplineComponent.GetLocationAtSplinePoint` _spline _index "World"))))
    (if (< _returnvalue_2 (`local.L_ShortestLength`))
      (set `local.L_NearestSplitePoint` _index)
      (set `local.L_ShortestLength` _returnvalue_2)))
  (return (`local.L_NearestSplitePoint`) (< (`local.L_NearestSplitePoint`) (/ _returnvalue 2))))

(fn `MoveToPoint`
  (`AIBlueprintHelperLibrary.SimpleMoveToLocation` (`AIBlueprintHelperLibrary.GetAIController` (`self.GetOwner`)) (`SplineComponent.GetLocationAtSplinePoint` (`/Game/Blueprints/Utility/BP_Spline.Spline` (`|GetArrayItem` (`self.Splines`) (`self.CurrentSplineIndex`))) (`self.CurrentSplinePointIndex`) "World")))

(fn `SelectRandomSpline`
  (set `self.CurrentSplineIndex` (`KismetMathLibrary.RandomIntegerInRange` 0 (- (`KismetArrayLibrary.Array_Length` (`self.Splines`)) 1))))

(fn `StartPatrolling`
  (bind (_out _shouldmoveforward) (`self.GetNearesSplinePointIndex` (`self.CurrentSplineIndex`) (`Actor.K2_GetActorLocation` (`self.GetOwner`))))
  (set `self.CurrentSplinePointIndex` _out)
  (set `self.IsMovingForward` _shouldmoveforward)
  (`self.MoveToPoint`)
  (set `self.IsPatrolling` true))

(fn `StopPatrolling`
  (`Controller.StopMovement` (`AIBlueprintHelperLibrary.GetAIController` (`self.GetOwner`)))
  (set `self.IsPatrolling` false))

(fn `SwitchToNextSpline`
  (if (< (`self.CurrentSplineIndex`) (- (`KismetArrayLibrary.Array_Length` (`self.Splines`)) 1))
    (`/Engine/EditorBlueprintResources/StandardMacros.IncrementInt` (`self.CurrentSplineIndex`))
    (else
      (set `self.CurrentSplineIndex` 0))))

(fn `WasPointReached`
  (returns (Out :type Boolean))
  (locals (L_OffsetLocation :type "Float (double-precision)" :default 125.0))
  (if (`self.IsPatrolling`)
    (return (<= (`KismetMathLibrary.VSize` (- (`Actor.K2_GetActorLocation` (`self.GetOwner`)) (`SplineComponent.GetLocationAtSplinePoint` (`/Game/Blueprints/Utility/BP_Spline.Spline` (`|GetArrayItem` (`self.Splines`) (`self.CurrentSplineIndex`))) (`self.CurrentSplinePointIndex`) "World"))) (`local.L_OffsetLocation`)))
    (else
      (return false))))