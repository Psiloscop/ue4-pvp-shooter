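; Bot combat component that picks, tracks and turns toward targets among detected characters.
; SwitchAim cycles to the next detected character with a clear line from the weapon, falling back to a nearest-target search.
; FaceToAim yaws controller and actor toward the target, interpolated in one combat state and instant otherwise.
; Added targets are watched for death and dropped when killed, and the torso socket supplies the point to shoot at.
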(event `self.ReceiveBeginPlay`
  (add `/Game/Blueprints/Components/Player/BP_WeaponManagerComponent.FirearmTaken` (`/Game/Blueprints/Characters/Bot/BP_Bot.BP_BotWeaponManagerComponent` (`/Game/Libs/BP_GlobalGetters_Bot.GetBotCharacterByActor` (`self.GetOwner`))) (`|CreateDelegate` :!event `OnFirearmTaken`)))

(event `self.ReceiveTick`
  (params (DeltaSeconds :type "Float (single-precision)")))

(event `self.SwitchAim`
  (`self.SwitchAimOverridden`))

(event `self.FaceToAim`
  (`self.FaceToAimOverridden`))

(event `self.AddAim`
  (params (Character :type "/Game/Blueprints/Characters/BP_Base_Character Object Reference"))
  (add `/Game/Blueprints/Characters/BP_Base_Character.CharacterDead` Character (`|CreateDelegate` :!event `OnCharacterDead`))
  (`parent.AddAim` Character))

(event `self.RemoveAim`
  (params (Character :type "/Game/Blueprints/Characters/BP_Base_Character Object Reference"))
  (remove `/Game/Blueprints/Characters/BP_Base_Character.CharacterDead` Character (`|CreateDelegate` :!event `OnCharacterDead`))
  (`parent.RemoveAim` Character))

(fn `FaceToAimOverridden`
  (bind _returnvalue (`self.GetOwner`))
  (bind _returnvalue_2 (`Pawn.GetController` (`/Game/Libs/BP_GlobalGetters_Bot.GetBotCharacterByActor` (`self.GetOwner`))))
  (bind _returnvalue_3 (`Controller.GetControlRotation` _returnvalue_2))
  (bind _yaw (.yaw (`KismetMathLibrary.FindLookAtRotation` (`Actor.K2_GetActorLocation` _returnvalue) (`Actor.K2_GetActorLocation` (`self.AimedCharacter`)))))
  (bind _returnvalue_4 (`KismetMathLibrary.MakeRotator` 0.0 0.0 _yaw))
  (bind _returnvalue_5 (`KismetMathLibrary.MakeRotator` (.roll _returnvalue_3) (.pitch _returnvalue_3) _yaw))
  (if (`|EnumEquality` (`self.CombatState`) "NewEnumerator1")
    (`Controller.SetControlRotation` _returnvalue_2 (`KismetMathLibrary.RInterpTo` _returnvalue_3 _returnvalue_5 (`GameplayStatics.GetWorldDeltaSeconds`) 3.0))
    (`Actor.K2_SetActorRotation` _returnvalue (`KismetMathLibrary.RInterpTo` (`Actor.K2_GetActorRotation` _returnvalue) _returnvalue_4 (`GameplayStatics.GetWorldDeltaSeconds`) 3.0) false)
    (else
      (`Controller.SetControlRotation` _returnvalue_2 _returnvalue_5)
      (`Actor.K2_SetActorRotation` _returnvalue _returnvalue_4 false))))

(fn `FindNearestAim`
  (locals (L_OwnerLocation :type "Vector Structure" :default (0.0 0.0 0.0)) (L_NearestAimLocation :type "Float (double-precision)") (L_NearestAimIndex :type Integer :default -1))
  (set `local.L_OwnerLocation` (`Actor.K2_GetActorLocation` (`self.GetOwner`)))
  (if (> (`KismetArrayLibrary.Array_Length` (`self.DetectedCharacters`)) 0)
    (set `local.L_NearestAimLocation` (`KismetMathLibrary.VSize` (- (`local.L_OwnerLocation`) (`Actor.K2_GetActorLocation` (`|GetArrayItem` (`self.DetectedCharacters`))))))
    (for (_array_element _array_index) (`self.DetectedCharacters`)
      (bind _returnvalue (`KismetMathLibrary.VSize` (- (`local.L_OwnerLocation`) (`Actor.K2_GetActorLocation` _array_element))))
      (if (and (< _returnvalue (`local.L_NearestAimLocation`)) (`self.IsWayToAimClear` (`local.L_OwnerLocation`) (`Actor.K2_GetActorLocation` _array_element) _array_element))
        (set `local.L_NearestAimLocation` _returnvalue)
        (set `local.L_NearestAimIndex` _array_index)))
    (if (!= -1 (`local.L_NearestAimIndex`))
      (set `self.AimedCharacter` (`|GetArrayItem` (`self.DetectedCharacters`) (`local.L_NearestAimIndex`))))))

(fn `GetAimedCharacterPlaceToShoot`
  (returns (Out :type "Vector Structure"))
  (`/Engine/EditorBlueprintResources/StandardMacros.IsValid` (`self.AimedCharacter`)
    (:`Is Valid`
      (return (`SceneComponent.GetSocketLocation` (`Character.Mesh` (`self.AimedCharacter`)) "torso")))
    (:`Is Not Valid`
      (return (0.0 0.0 0.0)))))

(fn `HaveAimToAttack`
  (returns (Out :type Boolean))
  (return (> (`KismetArrayLibrary.Array_Length` (`self.DetectedCharacters`)) 0)))

(fn `OnCharacterDead`
  (params (Character :type "/Game/Blueprints/Characters/BP_Base_Character Object Reference"))
  (`self.RemoveAim` Character)
  (if (== Character (`self.AimedCharacter`))
    (set `self.AimedCharacter` null)))

(fn `SwitchAimOverridden`
  (locals (L_PlayerLocation :type "Vector Structure") (L_NearestCharacter :type "Character Object Reference"))
  (bind _detectedcharacters (`self.DetectedCharacters`))
  (bind _l_nearestcharacter (`local.L_NearestCharacter`))
  (bind _l_nearestcharacter_2 (`local.L_NearestCharacter`))
  (bind _aimedcharacter (`self.AimedCharacter`))
  (bind _detectedcharacters_2 (`self.DetectedCharacters`))
  (bind _l_playerlocation (`local.L_PlayerLocation`))
  (bind _returnvalue (`KismetArrayLibrary.Array_Length` _detectedcharacters))
  (bind _returnvalue_2 (+ (`KismetArrayLibrary.Array_Find` _detectedcharacters _aimedcharacter) 1))
  (`/Engine/EditorBlueprintResources/StandardMacros.IsValid` _aimedcharacter
    (:`Is Valid`
      (if (!= _returnvalue_2 _returnvalue)
        (for _index (range _returnvalue_2 _returnvalue)
          (bind _output (`|GetArrayItem` (`self.DetectedCharacters`) _index))
          (if (`self.IsWayToAimClear` (`self.GetWeaponLocation`) (`Actor.K2_GetActorLocation` _output) _output)
            (set `local.L_NearestCharacter` _output)
            (break)))
        (`/Engine/EditorBlueprintResources/StandardMacros.IsValid` _l_nearestcharacter_2
          (:`Is Valid`
            (set `self.AimedCharacter` _l_nearestcharacter_2))
          (:`Is Not Valid`
            (set `local.L_PlayerLocation` (`Actor.K2_GetActorLocation` (`self.GetOwner` self)) :!label _label)
            (set `local.L_NearestCharacter` (`|GetArrayItem` _detectedcharacters_2))
            (for _array_element _detectedcharacters_2
              (`/Engine/EditorBlueprintResources/StandardMacros.IsValid` _array_element
                (:`Is Valid`
                  (bind _returnvalue_3 (`Actor.K2_GetActorLocation` _array_element))
                  (if (and (!= _array_element (`self.AimedCharacter`)) (`self.IsWayToAimClear` (`self.GetWeaponLocation`) _returnvalue_3 _array_element) (< (`KismetMathLibrary.VSize` (- _returnvalue_3 _l_playerlocation)) (`KismetMathLibrary.VSize` (- (`Actor.K2_GetActorLocation` (`local.L_NearestCharacter`)) _l_playerlocation))))
                    (set `local.L_NearestCharacter` _array_element)))))
            (if (`self.IsWayToAimClear` (`self.GetWeaponLocation`) (`Actor.K2_GetActorLocation` _l_nearestcharacter) _l_nearestcharacter)
              (set `self.AimedCharacter` _l_nearestcharacter))))
        (else
          (goto _label))))
    (:`Is Not Valid`
      (goto _label))))