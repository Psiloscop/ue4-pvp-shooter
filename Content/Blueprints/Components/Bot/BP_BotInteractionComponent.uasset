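; Bot interaction component that keeps a list of detected interactables and a current target for a bot to act on.
; AddInteractable stores each unique interactable and binds to its OnDestroyed event, so OnInteractableDestroyed can unbind and drop it from the list.
; SetCurrentTarget sets the detected actor, while ApplyActiontoDetectedActor defers to the parent implementation.
; HaveItemsToInteractWith reports whether any detected interactables remain.
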(event `self.ReceiveBeginPlay`)

(event `self.ReceiveTick`
  (params (DeltaSeconds :type "Float (single-precision)")))

(event `self.ApplyActionToDetectedActor`
  (`parent.ApplyActionToDetectedActor`))

(fn `AddInteractable`
  (params (In :type "/Game/Blueprints/Common/BP_Interaction Object Reference"))
  (if (== (`KismetArrayLibrary.Array_Find` (`self.DetectedInteractables`) In) -1)
    (add `Actor.OnDestroyed` In (`|CreateDelegate` :!event `OnInteractableDestroyed`))
    (`KismetArrayLibrary.Array_Add` (`self.DetectedInteractables`) In)))

(fn `HaveItemsToInteractWith`
  (returns (Out :type Boolean))
  (return (> (`KismetArrayLibrary.Array_Length` (`self.DetectedInteractables`)) 0)))

(fn `OnInteractableDestroyed`
  (params (Actor :type "Actor Object Reference"))
  (remove `Actor.OnDestroyed` Actor (`|CreateDelegate` :!event `OnInteractableDestroyed`))
  (`KismetArrayLibrary.Array_RemoveItem` (`self.DetectedInteractables`) (cast `/Game/Blueprints/Common/BP_Interaction` Actor :!pure true)))

(fn `SetCurrentTarget`
  (params (In :type "/Game/Blueprints/Common/BP_Interaction Object Reference"))
  (set `self.DetectedInteractableActor` In))