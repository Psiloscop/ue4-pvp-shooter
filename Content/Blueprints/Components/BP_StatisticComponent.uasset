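; Character component that records PVP kills, deaths, shots and hits on the BP_PlayerState_PVP of the relevant player.
; Deaths and shots go to the owner, while kills and hits are credited to the stored LastShootInstigator.
; Kill and death changes fire update dispatchers on the affected character's component; shots and hits update silently.
; GetAllStats reads all four counters; ClearStats is empty and BeginPlay does nothing.
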(event `self.ReceiveBeginPlay`)

(fn `ClearStats`)

(fn `GetAllStats`
  (returns (KIlls :type Integer) (Deaths :type Integer) (Shots :type Integer) (Hits :type Integer))
  (bind _out (`self.GetPlayerState`))
  (return (`/Game/Base/Blueprints/BP_PlayerState_PVP.KIlls` _out) (`/Game/Base/Blueprints/BP_PlayerState_PVP.Deaths` _out) (`/Game/Base/Blueprints/BP_PlayerState_PVP.Shots` _out) (`/Game/Base/Blueprints/BP_PlayerState_PVP.Hits` _out)))

(fn `GetPlayerState`
  (returns (Out :type "/Game/Base/Blueprints/BP_PlayerState_PVP Object Reference"))
  (bind _asbp_base_character (cast `/Game/Blueprints/Characters/BP_Base_Character` (`self.GetOwner`)))
  (bind _asbp_player_state_pvp (cast `/Game/Base/Blueprints/BP_PlayerState_PVP` (`Pawn.PlayerState` _asbp_base_character)))
  (return _asbp_player_state_pvp))

(fn `IncreaseDeathsValue`
  (bind _result (`/Engine/EditorBlueprintResources/StandardMacros.IncrementInt` (`/Game/Base/Blueprints/BP_PlayerState_PVP.Deaths` (`self.GetPlayerState`)))
    (:`  `
      (`self.DeathsStatUpdated` _result))))

(fn `IncreaseHitsValueValueForInstigator`
  (`/Engine/EditorBlueprintResources/StandardMacros.IsValid` (`self.LastShootInstigator`)
    (:`Is Valid`
      (bind _asbp_player_state_pvp (cast `/Game/Base/Blueprints/BP_PlayerState_PVP` (`Pawn.PlayerState` (`self.LastShootInstigator`))))
      (`/Engine/EditorBlueprintResources/StandardMacros.IncrementInt` (`/Game/Base/Blueprints/BP_PlayerState_PVP.Hits` _asbp_player_state_pvp)))))

(fn `IncreaseKillsValueForInstigator`
  (`/Engine/EditorBlueprintResources/StandardMacros.IsValid` (`self.LastShootInstigator`)
    (:`Is Valid`
      (bind _asbp_player_state_pvp (cast `/Game/Base/Blueprints/BP_PlayerState_PVP` (`Pawn.PlayerState` (`self.LastShootInstigator`))))
      (bind _result (`/Engine/EditorBlueprintResources/StandardMacros.IncrementInt` (`/Game/Base/Blueprints/BP_PlayerState_PVP.KIlls` _asbp_player_state_pvp))
        (:`  `
          (`self.KillsStatUpdated` (`/Game/Blueprints/Characters/BP_Base_Character.BP_StatisticComponent` (`self.LastShootInstigator`)) _result))))))

(fn `IncreaseShotsValue`
  (`/Engine/EditorBlueprintResources/StandardMacros.IncrementInt` (`/Game/Base/Blueprints/BP_PlayerState_PVP.Shots` (`self.GetPlayerState`))))

(fn `SetShotInstigator`
  (params (Character :type "/Game/Blueprints/Characters/BP_Base_Character Object Reference"))
  (set `self.LastShootInstigator` Character))