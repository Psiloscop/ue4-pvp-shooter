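; Bullet actor that applies point damage to what it hits, then destroys itself.
; Damage multiplies weapon and bullet factors, with BulletOwner passed as the damage causer.
; A timer set in the Construction Script also destroys it after Lifetime, and Destroy clears that timer.
; A SpawnDecal helper, not called in this graph, attaches a temporary impact decal oriented to the surface normal; an unconnected draft spawns decal actors instead.
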(event `self.ReceiveHit`
  (params (MyComp :type "PrimitiveComponent Object Reference") (Other :type "Actor Object Reference") (OtherComp :type "PrimitiveComponent Object Reference") (bSelfMoved :type Boolean) (HitLocation :type "Vector Structure") (HitNormal :type "Vector Structure") (NormalImpulse :type "Vector Structure") (Hit :type "HitResult Structure (by ref)"))
  (bind (_bblockinghit _binitialoverlap _time _distance _location _impactpoint _normal _impactnormal _physmat _hitactor _hitcomponent _hitbonename _hititem _faceindex _tracestart _traceend) (`GameplayStatics.BreakHitResult` Hit))
  (`GameplayStatics.ApplyPointDamage` Other (* (`self.DamageByWeapon`) (`self.DamageByBullet`)) (`KismetMathLibrary.GetDirectionUnitVector` _traceend _tracestart) Hit (`self.GetInstigatorController`) (`self.BulletOwner`))
  (`self.Destroy`))

(fn `Destroy`
  (`KismetSystemLibrary.K2_ClearAndInvalidateTimerHandle` (`self.DestroyTimer`))
  (`self.K2_DestroyActor`))

(fn `SpawnDecal`
  (params (HitComponent :type "SceneComponent Object Reference") (HitLocation :type "Vector Structure") (HitNormal :type "Vector Structure") (HitScale :type "Vector Structure") (Material :type "Material Object Reference"))
  (locals (RandomStream :type "RandomStream Structure"))
  (bind _returnvalue (`GameplayStatics.SpawnDecalAttached` Material HitScale HitComponent "None" HitLocation (`KismetMathLibrary.Conv_VectorToRotator` HitNormal) "KeepWorldPosition" 30.0))
  (`DecalComponent.SetFadeScreenSize` _returnvalue 0.001))

(fn `UserConstructionScript`
  (bind _returnvalue (`KismetSystemLibrary.K2_SetTimer` null "Destroy" (`self.Lifetime`)))
  (set `self.DestroyTimer` _returnvalue))