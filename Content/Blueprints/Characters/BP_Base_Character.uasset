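; Base character Blueprint that binds handlers for point damage, death and destruction on BeginPlay.
; Bullet hits whose damage causer is another base character record that instigator in BPStatisticComponent and credit it with a hit.
; Death disables movement and mesh collision, then updates death and kill stats; destruction also destroys attached actors.
; Armor, health and alive getters are stubs returning zero or false.
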(event `self.ReceiveBeginPlay`
  (add `self.OnTakePointDamage` (`|CreateDelegate` :!event `OnTakeBulletDamage`))
  (add `self.CharacterDead` (`|CreateDelegate` :!event `OnBaseCharacterDead`))
  (add `self.OnDestroyed` (`|CreateDelegate` :!event `OnActorDestroyed`)))

(fn `GetArmorValue`
  (returns (Out :type "Float (double-precision)"))
  (return 0.0))

(fn `GetHealthValue`
  (returns (Out :type "Float (double-precision)"))
  (return 0.0))

(fn `IsAlive`
  (returns (Out :type Boolean))
  (return false))

(fn `OnActorDestroyed`
  (params (Actor :type "Actor Object Reference"))
  (bind _children (`/DatasmithContent/Blueprints/FBXImporter/FBXImporterUtils.GetAllAttachedActors` Actor))
  (for _array_element _children
    (`self.K2_DestroyActor` _array_element)))

(fn `OnBaseCharacterDead`
  (params (Character :type "/Game/Blueprints/Characters/BP_Base_Character Object Reference"))
  (`|ExecutionSequence`
    (:`then_0`
      (`CharacterMovementComponent.DisableMovement` (`Character.CharacterMovement` Character))
      (`PrimitiveComponent.SetCollisionEnabled` (`Character.Mesh` Character) "NoCollision"))
    (:`then_1`
      (`/Game/Blueprints/Components/BP_StatisticComponent.IncreaseDeathsValue` (`self.BP_StatisticComponent`))
      (`/Game/Blueprints/Components/BP_StatisticComponent.IncreaseKillsValueForInstigator` (`self.BP_StatisticComponent`)))))

(fn `OnTakeBulletDamage`
  (params (DamagedActor :type "Actor Object Reference") (Damage :type "Float (double-precision)") (InstigatedBy :type "Controller Object Reference") (HitLocation :type "Vector Structure") (FHitComponent :type "PrimitiveComponent Object Reference") (BoneName :type Name) (ShotFromDirection :type "Vector Structure") (DamageType :type "DamageType Object Reference") (DamageCauser :type "Actor Object Reference"))
  (bind _asbp_base_character (cast `/Game/Blueprints/Characters/BP_Base_Character` DamageCauser))
  (`/Game/Blueprints/Components/BP_StatisticComponent.SetShotInstigator` (`self.BP_StatisticComponent`) _asbp_base_character)
  (`/Game/Blueprints/Components/BP_StatisticComponent.IncreaseHitsValueValueForInstigator` (`self.BP_StatisticComponent`)))

(fn `UserConstructionScript`)