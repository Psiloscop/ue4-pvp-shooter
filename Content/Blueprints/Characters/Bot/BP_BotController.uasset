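; BP_BotController is the AI controller for bot characters, starting their behavior when it possesses a pawn.
; On possess it sets up the BB_Bot blackboard and runs the BT_Bot behavior tree.
; It then seeds the BotState and BotEntityPriority enum keys with initial values, leaving all further decision-making to the tree.
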(event `self.ReceivePossess`
  (params (PossessedPawn :type "Pawn Object Reference"))
  (`|ExecutionSequence`
    (:`then_0`
      (`self.UseBlackboard` "/Game/Blueprints/AI/BB_Bot.BB_Bot")
      (`self.RunBehaviorTree` "/Game/Blueprints/AI/BT_Bot.BT_Bot"))
    (:`then_1`
      (`BlackboardComponent.SetValueAsEnum` (`AIBlueprintHelperLibrary.GetBlackboard` null) "BotState" (enumliteral `/Game/Blueprints/AI/Data/E_BotState` "NewEnumerator0"))
      (`BlackboardComponent.SetValueAsEnum` (`AIBlueprintHelperLibrary.GetBlackboard` null) "BotEntityPriority" (enumliteral `/Game/Blueprints/AI/Data/BotEntityPriority` "NewEnumerator1")))))

(fn `UserConstructionScript`)