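; Inventory item actor for the AS Val suppressed rifle, defining its item data and world mesh.
; On BeginPlay it fills ItemData with display info, slot size, charge, actions, rifle and item classes, and properties for two-handed hold and compatible magazine.
; It constructs a firearm actor bridge and an AS Val combine rule as helper objects stored in that data.
; Outline highlighting toggles custom depth on the static mesh.
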(event `self.ReceiveBeginPlay`
  (`parent.ReceiveBeginPlay`)
  (`|ExecutionSequence`
    (:`then_0`
      (bind _returnvalue (`|GenericCreateObject` "/Game/Blueprints/Inventory/ActorBridges/BP_Firearm_ActorBridge.BP_Firearm_ActorBridge_C" self))
      (setmembers `/Game/Data/Structs/S_InventoryItemData` :`StructRef` (`self.ItemData`) :`ID` "item_rifle_asval" :`Name` "Rifle AS Val" :`Description` "The AS Val  is a Soviet-designed rifle featuring an integrated suppressor. Development of a special rifle (AS) \"Shaft\" began in the first half of the 1980s in the Central Research Institute of Precision Engineering (TSNIITOCHMASH), in the city of Klimovsk, Moscow region. The lead designer of the rifle is Pyotr Serdyukov." :`Type` "NewEnumerator0" :`Image` "/Game/Assets/ItemsIcons/T_Item_asval.T_Item_asval" :`Cells` 2 :`Placement` "NewEnumerator0" :`IsStackable` false :`ChargeLimit` 20 :`Charge` 20 :`Amount` 1 :`Actions` (`|MakeArray` "NewEnumerator0" "NewEnumerator3" "NewEnumerator2" "NewEnumerator4" :!type "/Game/Data/Enums/E_InventoryItemAction Enum") :`RealItemClass` "/Game/Blueprints/Weapons/BP_Rifle_asval.BP_Rifle_asval_C" :`InventoryItemClass` "BP_Item_asval_C" :`ActorBridge` _returnvalue :`Properties` (`|MakeMap` "hold_type" "two_handed" "ammo_item_ids" "item_mag_asval" :!type "Name" :!valuetype "Name")))
    (:`then_1`
      (bind _returnvalue_2 (`|GenericCreateObject` "/Game/Blueprints/Inventory/CombineRules/BP_RifleAsval_CombineRule.BP_RifleAsval_CombineRule_C" self))
      (setmembers `/Game/Data/Structs/S_InventoryItemData` :`StructRef` (`self.ItemData`) :`CombineRule` _returnvalue_2))))

(event `/Game/Blueprints/Interfaces/BP_Intercation_Interface.ToggleOutline`
  (params (Enable :type Boolean))
  (`PrimitiveComponent.SetRenderCustomDepth` (`self.StaticMesh`) Enable))

(fn `GetItemMesh`
  (returns (Out :type "StaticMesh Object Reference"))
  (return (`StaticMeshComponent.StaticMesh` (`self.StaticMesh`))))

(fn `UserConstructionScript`)