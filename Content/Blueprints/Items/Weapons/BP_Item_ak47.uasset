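; Inventory item actor for the AK-47 rifle, representing the weapon as an item and linking it to its real rifle class.
; On BeginPlay it fills the ItemData struct with display info, charge, actions, hold type and compatible magazine.
; It constructs a firearm actor bridge and an AK-47 combine rule object and stores both in that data.
; It also exposes its static mesh and toggles an outline through custom depth.
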(event `self.ReceiveBeginPlay`
  (`parent.ReceiveBeginPlay`)
  (`|ExecutionSequence`
    (:`then_0`
      (bind _returnvalue (`|GenericCreateObject` "/Game/Blueprints/Inventory/ActorBridges/BP_Firearm_ActorBridge.BP_Firearm_ActorBridge_C" self))
      (setmembers `/Game/Data/Structs/S_InventoryItemData` :`StructRef` (`self.ItemData`) :`ID` "item_rifle_ak47" :`Name` "Rifle AK47" :`Description` "The AK-47, officially known as the Avtomat Kalashnikova, is a gas-operated, 7.62×39mm assault rifle, developed in the Soviet Union by Mikhail Kalashnikov. It is the originating firearm of the Kalashnikov rifle (or \"AK\") family." :`Type` "NewEnumerator0" :`Image` "/Game/Assets/ItemsIcons/T_Item_ak47.T_Item_ak47" :`Cells` 2 :`Placement` "NewEnumerator0" :`IsStackable` false :`ChargeLimit` 30 :`Charge` 30 :`Amount` 1 :`Actions` (`|MakeArray` "NewEnumerator0" "NewEnumerator3" "NewEnumerator2" "NewEnumerator4" :!type "/Game/Data/Enums/E_InventoryItemAction Enum") :`RealItemClass` "/Game/Blueprints/Weapons/BP_Rifle_ak47.BP_Rifle_ak47_C" :`InventoryItemClass` "BP_Item_ak47_C" :`ActorBridge` _returnvalue :`Properties` (`|MakeMap` "hold_type" "two_handed" "ammo_item_ids" "item_mag_ak47" :!type "Name" :!valuetype "Name")))
    (:`then_1`
      (bind _returnvalue_2 (`|GenericCreateObject` "/Game/Blueprints/Inventory/CombineRules/BP_RifleAk47_CombineRule.BP_RifleAk47_CombineRule_C" self))
      (setmembers `/Game/Data/Structs/S_InventoryItemData` :`StructRef` (`self.ItemData`) :`CombineRule` _returnvalue_2))))

(event `/Game/Blueprints/Interfaces/BP_Intercation_Interface.ToggleOutline`
  (params (Enable :type Boolean))
  (`PrimitiveComponent.SetRenderCustomDepth` (`self.StaticMesh`) Enable))

(fn `GetItemMesh`
  (returns (Out :type "StaticMesh Object Reference"))
  (return (`StaticMeshComponent.StaticMesh` (`self.StaticMesh`))))

(fn `UserConstructionScript`)