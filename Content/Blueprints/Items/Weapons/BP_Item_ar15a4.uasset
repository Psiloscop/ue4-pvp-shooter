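; Inventory item actor for the AR15A4 rifle, defining how it appears and behaves as an item.
; On BeginPlay it fills ItemData with display info, charge, actions, the rifle and item classes, two-handed hold type and compatible magazine ID.
; It constructs a firearm actor bridge and a rifle-specific combine rule as helper objects within that data.
; It also exposes its static mesh and toggles an outline through custom depth rendering.
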(event `self.ReceiveBeginPlay`
  (`parent.ReceiveBeginPlay`)
  (`|ExecutionSequence`
    (:`then_0`
      (bind _returnvalue (`|GenericCreateObject` "/Game/Blueprints/Inventory/ActorBridges/BP_Firearm_ActorBridge.BP_Firearm_ActorBridge_C" self))
      (setmembers `/Game/Data/Structs/S_InventoryItemData` :`StructRef` (`self.ItemData`) :`ID` "item_rifle_ar15a4" :`Name` "Rifle AR15A4" :`Description` "Rifle desc" :`Type` "NewEnumerator0" :`Image` "/Game/Assets/ItemsIcons/T_Item_ar15a4.T_Item_ar15a4" :`Cells` 2 :`Placement` "NewEnumerator0" :`IsStackable` false :`ChargeLimit` 30 :`Charge` 30 :`Amount` 1 :`Actions` (`|MakeArray` "NewEnumerator0" "NewEnumerator3" "NewEnumerator2" "NewEnumerator4" :!type "/Game/Data/Enums/E_InventoryItemAction Enum") :`RealItemClass` "/Game/Blueprints/Weapons/BP_Rifle_ar15a4.BP_Rifle_ar15a4_C" :`InventoryItemClass` "BP_Item_ar15a4_C" :`ActorBridge` _returnvalue :`Properties` (`|MakeMap` "hold_type" "two_handed" "ammo_item_ids" "item_mag_ar15a4" :!type "Name" :!valuetype "Name")))
    (:`then_1`
      (bind _returnvalue_2 (`|GenericCreateObject` "/Game/Blueprints/Inventory/CombineRules/BP_RifleAr15a4_CombineRule.BP_RifleAr15a4_CombineRule_C" self))
      (setmembers `/Game/Data/Structs/S_InventoryItemData` :`StructRef` (`self.ItemData`) :`CombineRule` _returnvalue_2))))

(event `/Game/Blueprints/Interfaces/BP_Intercation_Interface.ToggleOutline`
  (params (Enable :type Boolean))
  (`PrimitiveComponent.SetRenderCustomDepth` (`self.StaticMesh`) Enable))

(fn `GetItemMesh`
  (returns (Out :type "StaticMesh Object Reference"))
  (return (`StaticMeshComponent.StaticMesh` (`self.StaticMesh`))))

(fn `UserConstructionScript`)