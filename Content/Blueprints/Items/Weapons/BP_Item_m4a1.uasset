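; BP_Item_m4a1 is the inventory item actor for the M4A1 rifle.
; On BeginPlay it fills ItemData with the rifle's display info, charge, actions, item classes and properties for two-handed hold and compatible magazine.
; It constructs a firearm actor bridge and a rifle-specific combine rule into that data.
; It also exposes its static mesh and toggles custom depth on it for outlining.
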(event `self.ReceiveBeginPlay`
  (`parent.ReceiveBeginPlay`)
  (`|ExecutionSequence`
    (:`then_0`
      (bind _returnvalue (`|GenericCreateObject` "/Game/Blueprints/Inventory/ActorBridges/BP_Firearm_ActorBridge.BP_Firearm_ActorBridge_C" self))
      (setmembers `/Game/Data/Structs/S_InventoryItemData` :`StructRef` (`self.ItemData`) :`ID` "item_rifle_m4a1" :`Name` "Rifle M4A1" :`Description` "The M4A1 carbine is a fully automatic variant of the basic M4 carbine intended for special operations use. The M4A1 was introduce in May 1991 with improvements. and was in service in 1994." :`Type` "NewEnumerator0" :`Image` "/Game/Assets/ItemsIcons/T_Item_m4a1.T_Item_m4a1" :`Cells` 2 :`Placement` "NewEnumerator0" :`IsStackable` false :`ChargeLimit` 20 :`Charge` 20 :`Amount` 1 :`Actions` (`|MakeArray` "NewEnumerator0" "NewEnumerator3" "NewEnumerator2" "NewEnumerator4" :!type "/Game/Data/Enums/E_InventoryItemAction Enum") :`RealItemClass` "/Game/Blueprints/Weapons/BP_Rifle_m4a1.BP_Rifle_m4a1_C" :`InventoryItemClass` "BP_Item_m4a1_C" :`ActorBridge` _returnvalue :`Properties` (`|MakeMap` "hold_type" "two_handed" "ammo_item_ids" "item_mag_m4a1" :!type "Name" :!valuetype "Name")))
    (:`then_1`
      (bind _returnvalue_2 (`|GenericCreateObject` "/Game/Blueprints/Inventory/CombineRules/BP_RifleM4a1_CombineRule.BP_RifleM4a1_CombineRule_C" self))
      (setmembers `/Game/Data/Structs/S_InventoryItemData` :`StructRef` (`self.ItemData`) :`CombineRule` _returnvalue_2))))

(event `/Game/Blueprints/Interfaces/BP_Intercation_Interface.ToggleOutline`
  (params (Enable :type Boolean))
  (`PrimitiveComponent.SetRenderCustomDepth` (`self.StaticMesh`) Enable))

(fn `GetItemMesh`
  (returns (Out :type "StaticMesh Object Reference"))
  (return (`StaticMeshComponent.StaticMesh` (`self.StaticMesh`))))

(fn `UserConstructionScript`)