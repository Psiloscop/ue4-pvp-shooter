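; Remington 870 shell box item Blueprint, a world item under the weapons category.
; On BeginPlay it calls the parent logic and appends two extra entries to its ItemData action list.
; ToggleOutline switches custom depth rendering on its static mesh for highlighting, and GetItemMesh returns that mesh's asset.
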(event `self.ReceiveBeginPlay`
  (bind (_itemdata_id _itemdata_name _itemdata_description _itemdata_type _itemdata_image _itemdata_cells _itemdata_placement _itemdata_isstackable _itemdata_chargelimit _itemdata_charge _itemdata_amount _itemdata_actions) (break `/Game/Data/Structs/S_InventoryItemData` (`self.ItemData`)))
  (`parent.ReceiveBeginPlay`)
  (`KismetArrayLibrary.Array_Add` _itemdata_actions "NewEnumerator3")
  (`KismetArrayLibrary.Array_Add` _itemdata_actions "NewEnumerator4"))

(event `/Game/Blueprints/Interfaces/BP_Intercation_Interface.ToggleOutline`
  (params (Enable :type Boolean))
  (`PrimitiveComponent.SetRenderCustomDepth` (`self.StaticMesh`) Enable))

(fn `GetItemMesh`
  (returns (Out :type "StaticMesh Object Reference"))
  (return (`StaticMeshComponent.StaticMesh` (`self.StaticMesh`))))

(fn `UserConstructionScript`)