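; Base Blueprint for pickup items that players and AI bots collect into their inventories through an interaction action.
; ApplyAction branches on controller type, destroying the actor when the inventory accepts it.
; Bots throw away waste items and retry a failed take, then disarm empty weapons and re-equip after success.
; It also shows the item name as a HUD action-hand label and exposes type, data and an empty mesh getter.
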(event `/Game/Blueprints/Interfaces/BP_Intercation_Interface.ApplyAction`
  (bind _bp_botinventorycomponent (`/Game/Blueprints/Characters/Bot/BP_Bot.BP_BotInventoryComponent` (`/Game/Libs/BP_GlobalGetters_Bot.GetBotCharacterByBotController` (`self.InteractionController`))))
  (if (`.bSuccess` (cast `AIController` (`self.InteractionController`) :!pure true))
    (bind _itemtaken (`/Game/Blueprints/Components/Player/BP_InventoryComponent.TakeItem` _bp_botinventorycomponent self))
    (if _itemtaken
      (`self.K2_DestroyActor` :!label _label)
      (`/Game/Blueprints/Components/Bot/BP_BotInventoryComponent.DisarmEmptyWeapons` _bp_botinventorycomponent)
      (`/Game/Blueprints/Components/Bot/BP_BotInventoryComponent.EquipWeapons` _bp_botinventorycomponent)
      (else
        (`/Game/Blueprints/Components/Bot/BP_BotInventoryComponent.ThrowAwayWasteItems` _bp_botinventorycomponent)
        (bind _itemtaken_2 (`/Game/Blueprints/Components/Player/BP_InventoryComponent.TakeItem` _bp_botinventorycomponent self))
        (if _itemtaken_2
          (goto _label))))
    (else
      (bind _itemtaken_3 (`/Game/Blueprints/Components/Player/BP_InventoryComponent.TakeItem` (`/Game/Blueprints/Characters/Player/BP_Character.BP_InventoryComponent` (`/Game/Libs/BP_GlobalGetters.GetCharacterByController` (`self.InteractionController`))) self))
      (if _itemtaken_3
        (`self.K2_DestroyActor`)))))

(event `self.OnActionHandDisplayed`
  (params (ActonHand :type "/Game/Data/Enums/E_ActionHandType Enum" :default "NewEnumerator0"))
  (bind (_itemdata_id _itemdata_name) (break `/Game/Data/Structs/S_InventoryItemData` (`self.ItemData`)))
  (if (`|EnumEquality` ActonHand "NewEnumerator1")
    (`/Game/Base/Blueprints/BP_HUD_Base.SetActionHandLabel` (`/Game/Libs/BP_GlobalGetters.GetHudByController` (`self.InteractionController`)) (`KismetStringLibrary.Conv_NameToString` _itemdata_name))))

(fn `GetItemData`
  (returns (Out :type "/Game/Data/Structs/S_InventoryItemData Structure"))
  (return (`self.ItemData`)))

(fn `GetItemMesh`
  (returns (Out :type "StaticMesh Object Reference"))
  (return null))

(fn `GetType`
  (returns (Out :type "/Game/Data/Enums/E_ObjectType Enum"))
  (return "NewEnumerator0"))

(fn `UserConstructionScript`)