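; Medium medkit item for the inventory system, built on a parent item class.
; On BeginPlay it calls the parent, then fills its ItemData struct with identity, description, icon, type, placement, charge, allowed actions, its own class and a medkit-type property.
; ToggleOutline switches custom depth rendering on the static mesh for highlighting.
; GetItemMesh returns the mesh asset from that component.
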(event `self.ReceiveBeginPlay`
  (`parent.ReceiveBeginPlay`)
  (setmembers `/Game/Data/Structs/S_InventoryItemData` :`StructRef` (`self.ItemData`) :`ID` "item_medkit_medium" :`Name` "Medkit (medium)" :`Description` "A first aid kit is a collection of supplies and equipment that is used to give medical treatment." :`Type` "NewEnumerator2" :`Image` "/Game/Assets/ItemsIcons/T_Item_medkit.T_Item_medkit" :`Cells` 1 :`Placement` "NewEnumerator1" :`IsStackable` false :`ChargeLimit` 0 :`Charge` 25 :`Amount` 1 :`Actions` (`|MakeArray` "NewEnumerator1" "NewEnumerator2" "NewEnumerator4" :!type "/Game/Data/Enums/E_InventoryItemAction Enum") :`RealItemClass` null :`InventoryItemClass` (`GameplayStatics.GetObjectClass` self) :`ActorBridge` null :`CombineRule` null :`Properties` (`|MakeMap` "medkit_type" "medium" :!type "Name" :!valuetype "Name")))

(event `/Game/Blueprints/Interfaces/BP_Intercation_Interface.ToggleOutline`
  (params (Enable :type Boolean))
  (`PrimitiveComponent.SetRenderCustomDepth` (`self.StaticMesh`) Enable))

(fn `GetItemMesh`
  (returns (Out :type "StaticMesh Object Reference"))
  (return (`StaticMeshComponent.StaticMesh` (`self.StaticMesh`))))

(fn `UserConstructionScript`)