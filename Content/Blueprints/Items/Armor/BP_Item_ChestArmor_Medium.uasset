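; Medium chest armor inventory item, a child item Blueprint that defines its own data when play begins.
; BeginPlay fills the ItemData struct with identity, icon, placement, charge, available actions, its own class and a new BP_Armor_ActorBridge object.
; A second sequence step constructs another bridge and overwrites the first in ItemData.
; ToggleOutline switches custom depth rendering on the static mesh to show or hide an outline.
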(event `self.ReceiveBeginPlay`
  (`parent.ReceiveBeginPlay`)
  (`|ExecutionSequence`
    (:`then_0`
      (bind _returnvalue (`|GenericCreateObject` "/Game/Blueprints/Inventory/ActorBridges/BP_Armor_ActorBridge.BP_Armor_ActorBridge_C" self))
      (setmembers `/Game/Data/Structs/S_InventoryItemData` :`StructRef` (`self.ItemData`) :`ID` "item_chest_armor_medium" :`Name` "Armor (medium)" :`Description` "Chest armor descritptipn" :`Type` "NewEnumerator1" :`Image` "/Game/Assets/Items/ChestArmor/M_Item_ChestArmor.M_Item_ChestArmor" :`Cells` 2 :`Placement` "NewEnumerator1" :`IsStackable` false :`ChargeLimit` 50 :`Charge` 50 :`Amount` 1 :`Actions` (`|MakeArray` "NewEnumerator5" "NewEnumerator2" "NewEnumerator4" :!type "/Game/Data/Enums/E_InventoryItemAction Enum") :`RealItemClass` null :`InventoryItemClass` (`GameplayStatics.GetObjectClass` self) :`ActorBridge` _returnvalue :`CombineRule` null))
    (:`then_1`
      (bind _returnvalue_2 (`|GenericCreateObject` "/Game/Blueprints/Inventory/ActorBridges/BP_Armor_ActorBridge.BP_Armor_ActorBridge_C" self))
      (setmembers `/Game/Data/Structs/S_InventoryItemData` :`StructRef` (`self.ItemData`) :`ActorBridge` _returnvalue_2))))

(event `/Game/Blueprints/Interfaces/BP_Intercation_Interface.ToggleOutline`
  (params (Enable :type Boolean))
  (`PrimitiveComponent.SetRenderCustomDepth` (`self.StaticMesh`) Enable))

(fn `UserConstructionScript`
  (`parent.UserConstructionScript`))