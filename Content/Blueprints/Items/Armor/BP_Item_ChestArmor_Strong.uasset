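; Strong chest armor inventory item, built on a parent item class.
; On BeginPlay it fills ItemData with identity, icon, cell size, placement, charge and actions, and links a new BP_Armor_ActorBridge.
; A second sequence branch constructs another bridge and sets it as ItemData's ActorBridge again.
; The static mesh supplies the item mesh and toggles custom depth rendering for outlines.
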(event `self.ReceiveBeginPlay`
  (`parent.ReceiveBeginPlay`)
  (`|ExecutionSequence`
    (:`then_0`
      (bind _returnvalue (`|GenericCreateObject` "/Game/Blueprints/Inventory/ActorBridges/BP_Armor_ActorBridge.BP_Armor_ActorBridge_C" self))
      (setmembers `/Game/Data/Structs/S_InventoryItemData` :`StructRef` (`self.ItemData`) :`ID` "item_chest_armor_strong" :`Name` "Armor (strong)" :`Description` "Armor is a protective covering that is used to prevent damage from being inflicted to an object, individual or vehicle by direct contact weapons or projectiles." :`Type` "NewEnumerator1" :`Image` "/Game/Assets/ItemsIcons/T_Item_armor.T_Item_armor" :`Cells` 2 :`Placement` "NewEnumerator1" :`IsStackable` false :`ChargeLimit` 100 :`Charge` 100 :`Amount` 1 :`Actions` (`|MakeArray` "NewEnumerator5" "NewEnumerator2" "NewEnumerator4" :!type "/Game/Data/Enums/E_InventoryItemAction Enum") :`RealItemClass` null :`InventoryItemClass` (`GameplayStatics.GetObjectClass` self) :`ActorBridge` _returnvalue :`CombineRule` null))
    (:`then_1`
      (bind _returnvalue_2 (`|GenericCreateObject` "/Game/Blueprints/Inventory/ActorBridges/BP_Armor_ActorBridge.BP_Armor_ActorBridge_C" self))
      (setmembers `/Game/Data/Structs/S_InventoryItemData` :`StructRef` (`self.ItemData`) :`ActorBridge` _returnvalue_2))))

(event `/Game/Blueprints/Interfaces/BP_Intercation_Interface.ToggleOutline`
  (params (Enable :type Boolean))
  (`PrimitiveComponent.SetRenderCustomDepth` (`self.StaticMesh`) Enable))

(fn `GetItemMesh`
  (returns (Out :type "StaticMesh Object Reference"))
  (return (`StaticMeshComponent.StaticMesh` (`self.StaticMesh`))))

(fn `UserConstructionScript`
  (`parent.UserConstructionScript`))