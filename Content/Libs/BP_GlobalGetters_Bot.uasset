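; Blueprint library of global getters that resolve bot characters and controllers from related objects.
; Each function is a single cast that returns the typed result, or nothing when the cast fails.
; Bot characters come from a controller's controlled pawn or a given actor, cast to BP_Bot.
; The controller getter casts the character's controller to BP_PlayerController, despite its bot-controller name.
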(fn `GetBotCharacterByActor`
  (params (In :type "Actor Object Reference"))
  (returns (Out :type "/Game/Blueprints/Characters/Bot/BP_Bot Object Reference"))
  (bind _asbp_bot (cast `/Game/Blueprints/Characters/Bot/BP_Bot` In)
    (:`then`
      (return _asbp_bot))
    (:`CastFailed`
      (return null))))

(fn `GetBotCharacterByBotController`
  (params (In :type "Controller Object Reference"))
  (returns (Out :type "/Game/Blueprints/Characters/Bot/BP_Bot Object Reference"))
  (bind _asbp_bot (cast `/Game/Blueprints/Characters/Bot/BP_Bot` (`Controller.K2_GetPawn` In))
    (:`then`
      (return _asbp_bot))
    (:`CastFailed`
      (return null))))

(fn `GetBotControllerByBotCharacter`
  (params (Character :type "/Game/Blueprints/Characters/Player/BP_Character Object Reference"))
  (returns (Out :type "/Game/Blueprints/Characters/Player/BP_PlayerController Object Reference"))
  (bind _asbp_player_controller (cast `/Game/Blueprints/Characters/Player/BP_PlayerController` (`Pawn.GetController` Character))
    (:`then`
      (return _asbp_player_controller))
    (:`CastFailed`
      (return null))))