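; Base game mode that spawns, tracks and removes player and bot characters for faction-based sessions.
; Players in shuffled order and per-faction bot counts each take a free BP_PlayerStart_Base owned by their faction, which performs the spawn.
; Spawned characters are kept in separate player and bot lists, pruned through bindable death events and used to unpossess and destroy pawns.
; It also exposes the session state from BP_GameState_Base.
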(fn `BindToCharacterDeathEvent`
  (`|ExecutionSequence`
    (:`then_0`
      (for _array_element (`self.SpawnedPlayers`)
        (add `/Game/Blueprints/Characters/BP_Base_Character.CharacterDead` _array_element (`|CreateDelegate` :!event `OnCharacterDead`))))
    (:`then_1`
      (for _array_element_2 (`self.SpawnedBots`)
        (add `/Game/Blueprints/Characters/BP_Base_Character.CharacterDead` _array_element_2 (`|CreateDelegate` :!event `OnCharacterDead`))))))

(fn `GetSessionState`
  (returns (SessionState :type "/Game/Base/Blueprints/E_SessionState Enum"))
  (return (`/Game/Base/Blueprints/BP_GameState_Base.SessionState` (cast `/Game/Base/Blueprints/BP_GameState_Base` (`GameplayStatics.GetGameState`) :!pure true))))

(fn `GetSpawnPoints`
  (returns (Out :type "Array of /Game/Base/Blueprints/Bp_PlayerStart_Base Object Reference"))
  (locals (L_FreeSpawnPoints :type "Array of /Game/Base/Blueprints/Bp_PlayerStart_Base Object Reference"))
  (bind _outactors (`GameplayStatics.GetAllActorsOfClass` "/Game/Base/Blueprints/Bp_PlayerStart_Base.BP_PlayerStart_Base_C"))
  (for _array_element _outactors
    (if (`/Game/Base/Blueprints/Bp_PlayerStart_Base.IsFree` _array_element)
      (`KismetArrayLibrary.Array_Add` (`local.L_FreeSpawnPoints`) _array_element)))
  (return (`local.L_FreeSpawnPoints`)))

(fn `OnCharacterDead`
  (params (Character :type "/Game/Blueprints/Characters/BP_Base_Character Object Reference"))
  (if (`Pawn.IsBotControlled` Character)
    (`KismetArrayLibrary.Array_RemoveItem` (`self.SpawnedBots`) Character)
    (else
      (`KismetArrayLibrary.Array_RemoveItem` (`self.SpawnedPlayers`) Character))))

(fn `RemovePawns`
  (`|ExecutionSequence`
    (:`then_0`
      (for _array_element (`self.SpawnedPlayers`)
        (`/Engine/EditorBlueprintResources/StandardMacros.IsValid` _array_element
          (:`Is Valid`
            (`Controller.UnPossess` (`Pawn.GetController` _array_element))
            (`self.K2_DestroyActor` _array_element)))))
    (:`then_1`
      (for _array_element_2 (`self.SpawnedBots`)
        (`/Engine/EditorBlueprintResources/StandardMacros.IsValid` _array_element_2
          (:`Is Valid`
            (`Controller.UnPossess` (`Pawn.GetController` _array_element_2))
            (`self.K2_DestroyActor` _array_element_2)))))))

(fn `SpawnBots`
  (params (BotCount :type "Map of /Game/Data/Enums/E_CharacterFaction Enum to Integer" :default _))
  (locals (L_FreeSpawnPoints :type "Array of /Game/Base/Blueprints/Bp_PlayerStart_Base Object Reference") (L_SpawnPointIndex :type Integer))
  (`|ExecutionSequence`
    (:`then_0`
      (set `local.L_FreeSpawnPoints` (`self.GetSpawnPoints`)))
    (:`then_1`
      (bind _keys (`BlueprintMapLibrary.Map_Keys` BotCount))
      (for _array_element _keys
        (for _ (range 1 (+ (`BlueprintMapLibrary.Map_Find` BotCount _array_element) 1))
          (for _array_element_2 (`local.L_FreeSpawnPoints`)
            (if (and (`/Game/Base/Blueprints/Bp_PlayerStart_Base.IsFree` _array_element_2) (`|EnumEquality` (`/Game/Base/Blueprints/Bp_PlayerStart_Base.FactionOwner` _array_element_2) _array_element))
              (bind _out (`/Game/Base/Blueprints/Bp_PlayerStart_Base.SpawnBot` _array_element_2 _array_element))
              (`KismetArrayLibrary.Array_Add` (`self.SpawnedBots`) _out)
              (break))))))))

(fn `SpawnPlayers`
  (locals (L_FreeSpawnPoints :type "Array of /Game/Base/Blueprints/Bp_PlayerStart_Base Object Reference"))
  (bind _playerarray (`GameStateBase.PlayerArray` (`GameplayStatics.GetGameState`)))
  (`|ExecutionSequence`
    (:`then_0`
      (set `local.L_FreeSpawnPoints` (`self.GetSpawnPoints`)))
    (:`then_1`
      (`KismetArrayLibrary.Array_Shuffle` _playerarray)
      (for _array_element _playerarray
        (bind _returnvalue (`self.GetOwner` _array_element))
        (bind _asplayer_controller (cast `PlayerController` _returnvalue))
        (for _array_element_2 (`local.L_FreeSpawnPoints`)
          (bind _faction (`/Game/Base/Blueprints/BP_PlayerState_PVP.Faction` (cast `/Game/Base/Blueprints/BP_PlayerState_PVP` (`Controller.PlayerState` (cast `Controller` _returnvalue :!pure true)) :!pure true)))
          (if (and (`/Game/Base/Blueprints/Bp_PlayerStart_Base.IsFree` _array_element_2) (`|EnumEquality` (`/Game/Base/Blueprints/Bp_PlayerStart_Base.FactionOwner` _array_element_2) _faction))
            (bind _out (`/Game/Base/Blueprints/Bp_PlayerStart_Base.SpawnPlayer` _array_element_2 _faction _asplayer_controller))
            (`KismetArrayLibrary.Array_Add` (`self.SpawnedPlayers`) _out)
            (break)))))))

(fn `UnbindFromCharacterDeathEvent`
  (`|ExecutionSequence`
    (:`then_0`
      (for _array_element (`self.SpawnedPlayers`)
        (`/Engine/EditorBlueprintResources/StandardMacros.IsValid` _array_element
          (:`Is Valid`
            (remove `/Game/Blueprints/Characters/BP_Base_Character.CharacterDead` _array_element (`|CreateDelegate` :!event `OnCharacterDead`))))))
    (:`then_1`
      (for _array_element_2 (`self.SpawnedBots`)
        (`/Engine/EditorBlueprintResources/StandardMacros.IsValid` _array_element_2
          (:`Is Valid`
            (remove `/Game/Blueprints/Characters/BP_Base_Character.CharacterDead` _array_element_2 (`|CreateDelegate` :!event `OnCharacterDead`))))))))

(fn `UserConstructionScript`)