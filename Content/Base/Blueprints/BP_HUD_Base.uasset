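; Base HUD that manages the HUD and inventory widgets, showing manual/auto crosshairs and an interaction hand icon.
; CreateHUD binds to the pawn's combat and interaction components, whose events drive widget visibility and icons.
; GetActiveCrosshairLocation returns a camera-trace hit or the auto-aimed actor's location, also updating crosshair health and armor.
; It tracks the aimed character's damage event to paint the crosshair on hits; the session-state handler is empty.
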(event `self.ReceiveBeginPlay`
  (add `/Game/Base/Blueprints/BP_GameState_Base.SessionStateChanged` (cast `/Game/Base/Blueprints/BP_GameState_Base` (`GameplayStatics.GetGameState`) :!pure true) (`|CreateDelegate` :!event `OnSessionStateChanged`)))

(fn `AssignAimedActor`
  (params (Actor :type "Actor Object Reference"))
  (`|ExecutionSequence`
    (:`then_0`
      (`/Engine/EditorBlueprintResources/StandardMacros.IsValid` (`self.AimedActor`)
        (:`Is Valid`
          (remove `self.OnTakePointDamage` (`self.AimedActor`) (`|CreateDelegate` :!event `OnAimActorTakeBulletDamage`)))))
    (:`then_1`
      (bind _output_get (set `self.AimedActor` Actor))
      (add `self.OnTakePointDamage` _output_get (`|CreateDelegate` :!event `OnAimActorTakeBulletDamage`)))))

(fn `CreateHUD`
  (bind _bp_interactioncomponent (`/Game/Blueprints/Characters/Player/BP_Character.BP_InteractionComponent` (`/Game/Libs/BP_GlobalGetters.GetCharacterByActor` (`self.GetOwningPawn`))))
  (bind _bp_combatcomponent (`/Game/Blueprints/Characters/Player/BP_Character.BP_CombatComponent` (`/Game/Libs/BP_GlobalGetters.GetCharacterByActor` (`self.GetOwningPawn`))))
  (`|ExecutionSequence`
    (:`then_0`
      (bind _returnvalue (`|CreateWidget` (`self.HUD_Class`) (`self.GetOwningPlayerController`)))
      (bind _output_get (set `self.HUD_Widget` _returnvalue))
      (`UserWidget.AddToViewport` _output_get 0)
      (`Widget.SetVisibility` (`/Game/UI/HUD/W_HUD.W_HUD_Crosshair_Manual` (`self.HUD_Widget`)) "Hidden")
      (`Widget.SetVisibility` (`/Game/UI/HUD/W_HUD.W_HUD_Crosshair_Auto` (`self.HUD_Widget`)) "Hidden")
      (`Widget.SetVisibility` (`/Game/UI/HUD/W_HUD.W_HUD_ActionHand` (`self.HUD_Widget`)) "Hidden"))
    (:`then_1`
      (bind _returnvalue_2 (`|CreateWidget` (`self.Inventory_Class`) (`self.GetOwningPlayerController`)))
      (bind _output_get_2 (set `self.Inventory_Widget` _returnvalue_2))
      (`UserWidget.AddToViewport` _output_get_2 0)
      (`Widget.SetVisibility` (`self.Inventory_Widget`) "Hidden")
      (`/Game/UI/HUD/W_HUD_StatusBar.InitSubscriptions` (`/Game/UI/HUD/W_HUD.W_HUD_StatusBar` (`self.HUD_Widget`)) (`self.Inventory_Widget`)))
    (:`then_2`
      (add `/Game/Blueprints/Components/Player/BP_InteractionComponent.InteractionModeToggled` _bp_interactioncomponent (`|CreateDelegate` :!event `OnInteractionModeToggled`))
      (add `/Game/Blueprints/Components/Player/BP_InteractionComponent.InteractableActorDetected` _bp_interactioncomponent (`|CreateDelegate` :!event `OnInteractableActorDetected`))
      (add `/Game/Blueprints/Components/Player/BP_InteractionComponent.InteractableActorIgnored` _bp_interactioncomponent (`|CreateDelegate` :!event `InteractableActorIgnored`)))
    (:`then_3`
      (add `/Game/Blueprints/Components/Player/BP_CombatComponent.CombatStateChanged` _bp_combatcomponent (`|CreateDelegate` :!event `OnCombatStateChanged`))
      (add `/Game/Blueprints/Components/Player/BP_CombatComponent.CombatModeSwitched` _bp_combatcomponent (`|CreateDelegate` :!event `OnCombatModeSwitched`)))))

(fn `DestroyHUD`
  (`|ExecutionSequence`
    (:`then_0`
      (`/Engine/EditorBlueprintResources/StandardMacros.IsValid` (`self.HUD_Widget`)
        (:`Is Valid`
          (`Widget.RemoveFromParent` (`self.HUD_Widget`)))))
    (:`then_1`
      (`/Engine/EditorBlueprintResources/StandardMacros.IsValid` (`self.Inventory_Widget`)
        (:`Is Valid`
          (`Widget.RemoveFromParent` (`self.Inventory_Widget`)))))))

(fn `GetActionHandLocation`
  (returns (Out :type "Vector Structure"))
  (return (`GameplayStatics.DeprojectScreenToWorld` (`self.GetOwningPlayerController`) (`SlateBlueprintLibrary.LocalToAbsolute` (`Widget.GetCachedGeometry` (`/Game/UI/HUD/W_HUD.W_HUD_ActionHand` (`self.HUD_Widget`)))))))

(fn `GetActiveCrosshairLocation`
  (returns (Out :type "Vector Structure"))
  (bind _hud_widget (`self.HUD_Widget`))
  (bind _aimedactor (`self.AimedActor`))
  (bind _camera (`/Game/Blueprints/Characters/Player/BP_Character.Camera` (`/Game/Libs/BP_GlobalGetters.GetCharacterByActor` (`self.GetOwningPawn`))))
  (if (`Widget.IsVisible` (`/Game/UI/HUD/W_HUD.W_HUD_Crosshair_Manual` _hud_widget))
    (bind _outhit (`KismetSystemLibrary.LineTraceSingleForObjects` (`SceneComponent.K2_GetComponentLocation` _camera) (+ (`GameplayStatics.DeprojectScreenToWorld` (`self.GetOwningPlayerController`) (`SlateBlueprintLibrary.LocalToAbsolute` (`Widget.GetCachedGeometry` (`/Game/UI/HUD/W_HUD.W_HUD_Crosshair_Manual` (`self.HUD_Widget`))))) (* (`SceneComponent.GetForwardVector` _camera) 10000)) (`|MakeArray` "ObjectTypeQuery1" "ObjectTypeQuery1" "ObjectTypeQuery3" :!type "EObjectTypeQuery Enum") false (`|MakeArray` (`self.GetOwningPawn`) :!type "Actor Object Reference")))
    (`self.UpdateManualCrosshairData` (`.HitActor` (`GameplayStatics.BreakHitResult` _outhit)))
    (return (`.Location` (`GameplayStatics.BreakHitResult` _outhit)))
    (elif (and (`Widget.IsVisible` (`/Game/UI/HUD/W_HUD.W_HUD_Crosshair_Auto` _hud_widget)) (`KismetSystemLibrary.IsValid` (`self.AimedActor`)))
      (`self.UpdateAutoCrosshairData` _aimedactor)
      (return (`self.K2_GetActorLocation` _aimedactor)))))

(fn `InteractableActorIgnored`
  (`/Game/UI/HUD/W_HUD_ActionHand.SetupActionHandImage` (`/Game/UI/HUD/W_HUD.W_HUD_ActionHand` (`self.HUD_Widget`)) "NewEnumerator0"))

(fn `OnAimActorTakeBulletDamage`
  (params (DamagedActor :type "Actor Object Reference") (Damage :type "Float (double-precision)") (InstigatedBy :type "Controller Object Reference") (HitLocation :type "Vector Structure") (FHitComponent :type "PrimitiveComponent Object Reference") (BoneName :type Name) (ShotFromDirection :type "Vector Structure") (DamageType :type "DamageType Object Reference") (DamageCauser :type "Actor Object Reference"))
  (bind _hud_widget (`self.HUD_Widget`))
  (bind _w_hud_crosshair_manual (`/Game/UI/HUD/W_HUD.W_HUD_Crosshair_Manual` _hud_widget))
  (if (`Widget.IsVisible` _w_hud_crosshair_manual)
    (`/Game/UI/HUD/W_HUD_Crosshair_Base.PaintCrosshair` _w_hud_crosshair_manual)
    (else
      (`/Game/UI/HUD/W_HUD_Crosshair_Base.PaintCrosshair` (`/Game/UI/HUD/W_HUD.W_HUD_Crosshair_Auto` _hud_widget)))))

(fn `OnCombatModeSwitched`
  (params (Enabled :type "/Game/Data/Enums/E_CombatModeType Enum" :default "NewEnumerator0"))
  (if (`|EnumEquality` Enabled "NewEnumerator0")
    (`Widget.SetVisibility` (`/Game/UI/HUD/W_HUD.W_HUD_Crosshair_Auto` (`self.HUD_Widget`)) "Visible")
    (else
      (`Widget.SetVisibility` (`/Game/UI/HUD/W_HUD.W_HUD_Crosshair_Auto` (`self.HUD_Widget`)) "Hidden"))))

(fn `OnCombatStateChanged`
  (params (CombatState :type "/Game/Data/Enums/E_CharacterAnimState Enum" :default "NewEnumerator0"))
  (if (`|EnumEquality` CombatState "NewEnumerator2")
    (`self.ToggleManualCrosshair` true)
    (else
      (`self.ToggleManualCrosshair` false))))

(fn `OnInteractableActorDetected`
  (params (In :type "/Game/Blueprints/Interfaces/BP_Intercation_Interface Interface"))
  (bind _out (`/Game/Blueprints/Interfaces/BP_Intercation_Interface.GetType` In))
  (switch `/Game/Data/Enums/E_ObjectType` _out
    (:`NewEnumerator0`
      (`/Game/UI/HUD/W_HUD_ActionHand.SetupActionHandImage` (`/Game/UI/HUD/W_HUD.W_HUD_ActionHand` (`self.HUD_Widget`)) "NewEnumerator1")
      (`self.ActionHandDisplayed` "NewEnumerator1"))))

(fn `OnInteractionModeToggled`
  (params (Enable :type Boolean))
  (if Enable
    (`Widget.SetVisibility` (`/Game/UI/HUD/W_HUD.W_HUD_ActionHand` (`self.HUD_Widget`)) "Visible")
    (else
      (`Widget.SetVisibility` (`/Game/UI/HUD/W_HUD.W_HUD_ActionHand` (`self.HUD_Widget`)) "Hidden"))))

(fn `OnSessionStateChanged`
  (params (NewSessionState :type "/Game/Base/Blueprints/E_SessionState Enum" :default "NewEnumerator0")))

(fn `SetActionHandLabel`
  (params (In :type String))
  (bind _bottomtext (`/Game/UI/HUD/W_HUD_ActionHand.BottomText` (`/Game/UI/HUD/W_HUD.W_HUD_ActionHand` (`self.HUD_Widget`))))
  (`TextBlock.SetText` _bottomtext (`KismetTextLibrary.Conv_StringToText` In))
  (`Widget.SetVisibility` _bottomtext "Visible"))

(fn `ToggleAutoCrosshair`
  (params (Show :type Boolean))
  (if Show
    (`UserWidget.AddToViewport` (`/Game/UI/HUD/W_HUD.W_HUD_Crosshair_Auto` (`self.HUD_Widget`)) 0)
    (else
      (`Widget.RemoveFromParent` (`/Game/UI/HUD/W_HUD.W_HUD_Crosshair_Auto` (`self.HUD_Widget`))))))

(fn `ToggleInventory`
  (if (not (`Widget.IsVisible` (`self.Inventory_Widget`)))
    (`Widget.SetVisibility` (`self.Inventory_Widget`) "Visible")
    (`WidgetBlueprintLibrary.SetInputMode_UIOnlyEx` (`self.GetOwningPlayerController`) (`self.Inventory_Widget`))
    (else
      (`Widget.SetVisibility` (`self.Inventory_Widget`) "Hidden")
      (`WidgetBlueprintLibrary.SetInputMode_GameOnly` (`self.GetOwningPlayerController`)))))

(fn `ToggleManualCrosshair`
  (params (Show :type Boolean))
  (if Show
    (`Widget.SetVisibility` (`/Game/UI/HUD/W_HUD.W_HUD_Crosshair_Manual` (`self.HUD_Widget`)) "Visible")
    (else
      (`Widget.SetVisibility` (`/Game/UI/HUD/W_HUD.W_HUD_Crosshair_Manual` (`self.HUD_Widget`)) "Hidden"))))

(fn `UpdateAutoCrosshairData`
  (params (Actor :type "Actor Object Reference"))
  (locals (BaseCharacter :type "/Game/Blueprints/Characters/BP_Base_Character Object Reference"))
  (bind _returnvalue (`KismetSystemLibrary.DoesImplementInterface` Actor "/Game/Blueprints/Interfaces/BP_Character_Interface.BP_Character_Interface_C"))
  (bind _w_hud_crosshair_auto (`/Game/UI/HUD/W_HUD.W_HUD_Crosshair_Auto` (`self.HUD_Widget`)))
  (bind _w_hud_crosshair_auto_2 (`/Game/UI/HUD/W_HUD.W_HUD_Crosshair_Auto` (`self.HUD_Widget`)))
  (set `local.BaseCharacter` (cast `/Game/Blueprints/Characters/BP_Base_Character` Actor :!pure true))
  (`|ExecutionSequence`
    (:`then_0`
      (if _returnvalue
        (`|ExecutionSequence`
          (:`then_0`
            (bind _out (`/Game/Blueprints/Interfaces/BP_Character_Interface.GetHealthValue` (`local.BaseCharacter`)))
            (`/Game/UI/HUD/W_HUD_Crosshair_Base.SetHealthProgress` _w_hud_crosshair_auto _out))
          (:`then_1`
            (bind _out_2 (`/Game/Blueprints/Interfaces/BP_Character_Interface.GetArmorValue` (`local.BaseCharacter`)))
            (`/Game/UI/HUD/W_HUD_Crosshair_Base.SetArmorProgress` _w_hud_crosshair_auto _out_2)))
        (else
          (`/Game/UI/HUD/W_HUD_Crosshair_Base.SetHealthProgress` _w_hud_crosshair_auto_2 0.0)
          (`/Game/UI/HUD/W_HUD_Crosshair_Base.SetArmorProgress` _w_hud_crosshair_auto_2 0.0))))
    (:`then_1`
      (if _returnvalue
        (`self.AssignAimedActor` (`local.BaseCharacter`))
        (set `/Game/UI/HUD/W_HUD_Crosshair_Auto.Location` (`self.K2_GetActorLocation` (`local.BaseCharacter`)) (`/Game/UI/HUD/W_HUD.W_HUD_Crosshair_Auto` (`self.HUD_Widget`)))))))

(fn `UpdateManualCrosshairData`
  (params (Actor :type "Actor Object Reference"))
  (locals (BaseCharacter :type "/Game/Blueprints/Characters/BP_Base_Character Object Reference"))
  (bind _returnvalue (`KismetSystemLibrary.DoesImplementInterface` Actor "/Game/Blueprints/Interfaces/BP_Character_Interface.BP_Character_Interface_C"))
  (bind _w_hud_crosshair_manual (`/Game/UI/HUD/W_HUD.W_HUD_Crosshair_Manual` (`self.HUD_Widget`)))
  (bind _w_hud_crosshair_manual_2 (`/Game/UI/HUD/W_HUD.W_HUD_Crosshair_Manual` (`self.HUD_Widget`)))
  (set `local.BaseCharacter` (cast `/Game/Blueprints/Characters/BP_Base_Character` Actor :!pure true))
  (`|ExecutionSequence`
    (:`then_0`
      (if _returnvalue
        (`|ExecutionSequence`
          (:`then_0`
            (bind _out (`/Game/Blueprints/Interfaces/BP_Character_Interface.GetHealthValue` (`local.BaseCharacter`)))
            (`/Game/UI/HUD/W_HUD_Crosshair_Base.SetHealthProgress` _w_hud_crosshair_manual_2 _out))
          (:`then_1`
            (bind _out_2 (`/Game/Blueprints/Interfaces/BP_Character_Interface.GetArmorValue` (`local.BaseCharacter`)))
            (`/Game/UI/HUD/W_HUD_Crosshair_Base.SetArmorProgress` _w_hud_crosshair_manual_2 _out_2)))
        (else
          (`/Game/UI/HUD/W_HUD_Crosshair_Base.SetHealthProgress` _w_hud_crosshair_manual 0.0)
          (`/Game/UI/HUD/W_HUD_Crosshair_Base.SetArmorProgress` _w_hud_crosshair_manual 0.0))))
    (:`then_1`
      (if _returnvalue
        (`self.AssignAimedActor` (`local.BaseCharacter`))))))

(fn `UserConstructionScript`)