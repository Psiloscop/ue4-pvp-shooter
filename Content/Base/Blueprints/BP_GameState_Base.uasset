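; Base game state that drives the round lifecycle and tracks match time.
; It starts in Before Round, broadcasts session, time and reset changes through event dispatchers, and advances the timer on a one-second tick during In Round.
; Its handlers tell the game mode to spawn players and bots from preparation data, manage death bindings and remove pawns afterwards.
; Replay reloads the current level, a temporary solution until multiplayer.
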(event `self.ReceiveBeginPlay`
  (`|ExecutionSequence`
    (:`then_0`
      (add `self.TimeChanged` (`|CreateDelegate` :!event `OnTimeChanged`))
      (add `self.SessionStateChanged` (`|CreateDelegate` :!event `OnSessionStateChanged`))
      (add `self.RoundResetted` (`|CreateDelegate` :!event `OnRoundResetted`)))
    (:`then_1`
      ;[1 1 1] Trigger game initialization
      (`self.ChangeSessionState` "NewEnumerator0"))))

(event `self.ReceiveTick`
  (params (DeltaSeconds :type "Float (single-precision)"))
  (switch `/Game/Base/Blueprints/E_SessionState` (`self.SessionState`)
    (:`NewEnumerator1`
      (`self.TickTime`))))

(fn `AssignPreparationData`
  (params (PreparationData :type "/Game/Base/Blueprints/S_PreparationData Structure"))
  (set `self.PreparationData` PreparationData))

(fn `ChangeSessionState`
  (params (NewState :type "/Game/Base/Blueprints/E_SessionState Enum" :default "NewEnumerator0"))
  (bind _output_get (set `self.SessionState` NewState))
  (`self.SessionStateChanged` _output_get))

(fn `GetTime`
  (returns (Out :type "Timespan Structure"))
  (return (`self.MatchTime`)))

(fn `OnRoundResetted`
  ;[1 1 1] Temporary solution before develop multiplayer mode
  (bind _returnvalue (`GameplayStatics.GetCurrentLevelName` true))
  (`GameplayStatics.OpenLevel` (`KismetStringLibrary.Conv_StringToName` _returnvalue)))

(fn `OnSessionStateChanged`
  (params (SessionState :type "/Game/Base/Blueprints/E_SessionState Enum" :default "NewEnumerator0"))
  (locals (L_GameMode_Base :type "/Game/Base/Blueprints/BP_GameMode_Base Object Reference"))
  (bind (_selectedteam _humanbotcount _cyborgbotcount) (break `/Game/Base/Blueprints/S_PreparationData` (`self.PreparationData`)))
  (bind _asbp_game_mode_base (cast `/Game/Base/Blueprints/BP_GameMode_Base` (`GameplayStatics.GetGameMode`)))
  (set `local.L_GameMode_Base` _asbp_game_mode_base)
  (switch `/Game/Base/Blueprints/E_SessionState` SessionState
    (:`NewEnumerator1`
      (`/Game/Base/Blueprints/BP_GameMode_Base.SpawnPlayers` (`local.L_GameMode_Base`))
      (`/Game/Base/Blueprints/BP_GameMode_Base.SpawnBots` (`local.L_GameMode_Base`) (`|MakeMap` "NewEnumerator0" _humanbotcount "NewEnumerator1" _cyborgbotcount :!type "/Game/Data/Enums/E_CharacterFaction Enum"))
      (`/Game/Base/Blueprints/BP_GameMode_Base.BindToCharacterDeathEvent` (`local.L_GameMode_Base`)))
    (:`NewEnumerator2`
      (`/Game/Base/Blueprints/BP_GameMode_Base.UnbindFromCharacterDeathEvent` (`local.L_GameMode_Base`))
      (`/Game/Base/Blueprints/BP_GameMode_Base.RemovePawns` (`local.L_GameMode_Base`)))))

(fn `OnTimeChanged`
  (params (CurrentTime :type "Timespan Structure")))

(fn `ReplayRound`
  (`self.RoundResetted`)
  (for _array_element (`GameStateBase.PlayerArray` (`GameplayStatics.GetGameState`))
    (set `/Game/Base/Blueprints/BP_PlayerState_Base.IsValid` false (cast `/Game/Base/Blueprints/BP_PlayerState_Base` _array_element :!pure true))))

(fn `TickTime`
  (bind _output_get (set `self.MatchTime` (+ (`self.MatchTime`) (`KismetMathLibrary.MakeTimespan` 0 0 0 1))))
  (`self.TimeChanged` _output_get))

(fn `UserConstructionScript`)