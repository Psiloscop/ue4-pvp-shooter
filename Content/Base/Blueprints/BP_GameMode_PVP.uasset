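; PVP game mode that respawns dead bots and players while the session is in the required state.
; Bots queue with a death time polled on Tick, while players get a HUD countdown and a Delay.
; RespawnCharacter destroys the old pawn, then respawns its controller at the first spawn point matching its faction, rebinding the death event.
; The previous skeletal mesh is handed to spawn points beforehand.
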(event `self.ReceiveTick`
  (params (DeltaSeconds :type "Float (single-precision)"))
  (`parent.ReceiveTick` DeltaSeconds)
  (for _array_element (`self.RespawnCharacters`)
    (bind (_character _deathtime) (break `/Game/Base/Blueprints/S_RespawnCharacter` _array_element))
    (if (and (>= (`KismetMathLibrary.GetSeconds` (- (`KismetMathLibrary.Now`) _deathtime)) (`self.RespawnTime`)) (`|EnumEquality` "NewEnumerator1" (`self.GetSessionState`)))
      (`self.RespawnCharacter` _character)
      (`KismetArrayLibrary.Array_RemoveItem` (`self.RespawnCharacters`) _array_element))))

(event `self.OnCharacterDead`
  (params (Character :type "/Game/Blueprints/Characters/BP_Base_Character Object Reference"))
  (`parent.OnCharacterDead` Character)
  (if (`Pawn.IsBotControlled` Character)
    (`KismetArrayLibrary.Array_Add` (`self.RespawnCharacters`) (make `/Game/Base/Blueprints/S_RespawnCharacter` Character (`KismetMathLibrary.Now`)))
    (else
      (bind _asbp_hud_pvp (cast `/Game/Base/Blueprints/BP_HUD_PVP` (`/Game/Libs/BP_GlobalGetters.GetHudByActor` Character)))
      (`/Game/Base/Blueprints/BP_HUD_PVP.ShowRespawnWidget` _asbp_hud_pvp (`self.RespawnTime`))
      (`KismetSystemLibrary.Delay` (`KismetMathLibrary.Conv_IntToDouble` (`self.RespawnTime`)))
      (if (`|EnumEquality` "NewEnumerator1" (`self.GetSessionState`))
        (`/Game/Base/Blueprints/BP_HUD_PVP.HideRespawnWidget` _asbp_hud_pvp)
        (`self.RespawnCharacter` Character)))))

(fn `RespawnCharacter`
  (params (In :type "/Game/Blueprints/Characters/BP_Base_Character Object Reference"))
  (locals (L_Controller :type "Controller Object Reference") (L_UsedSkeletalMesh :type "SkeletalMesh Object Reference"))
  (bind _faction (`/Game/Base/Blueprints/BP_PlayerState_PVP.Faction` (cast `/Game/Base/Blueprints/BP_PlayerState_PVP` (`Controller.PlayerState` (`local.L_Controller`)) :!pure true)))
  (bind _output_get (set `local.L_Controller` (`Pawn.GetController` In)))
  (`/Engine/EditorBlueprintResources/StandardMacros.IsValid` _output_get
    (:`Is Valid`
      (`Controller.UnPossess` (`local.L_Controller`))
      (set `local.L_UsedSkeletalMesh` (`/Game/Blueprints/Characters/BP_Base_Character.UsedSkeletalMesh` In))
      (`self.K2_DestroyActor` In)
      (for _array_element (`self.GetSpawnPoints`)
        (`|ExecutionSequence`
          (:`then_0`
            (`/Engine/EditorBlueprintResources/StandardMacros.IsValid` (`local.L_UsedSkeletalMesh`)
              (:`Is Valid`
                (`/Game/Base/Blueprints/Bp_PlayerStart_Base.SetPrevSkeletalMesh` _array_element (`local.L_UsedSkeletalMesh`)))))
          (:`then_1`
            (if (`|EnumEquality` (`/Game/Base/Blueprints/Bp_PlayerStart_Base.FactionOwner` _array_element) _faction)
              (if (`.bSuccess` (cast `AIController` (`local.L_Controller`) :!pure true))
                (bind _out (`/Game/Base/Blueprints/Bp_PlayerStart_Base.RespawnBot` _array_element _faction (`local.L_Controller`)))
                (`KismetArrayLibrary.Array_Add` (`self.SpawnedBots`) _out)
                (add `/Game/Blueprints/Characters/BP_Base_Character.CharacterDead` _out (`|CreateDelegate` :!event `OnCharacterDead`))
                (else
                  (bind _out_2 (`/Game/Base/Blueprints/Bp_PlayerStart_Base.SpawnPlayer` _array_element _faction (`local.L_Controller`)))
                  (`KismetArrayLibrary.Array_Add` (`self.SpawnedPlayers`) _out_2)
                  (add `/Game/Blueprints/Characters/BP_Base_Character.CharacterDead` _out_2 (`|CreateDelegate` :!event `OnCharacterDead`))))
              (return))))))))

(fn `UserConstructionScript`
  (`parent.UserConstructionScript`))