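; PVP game state Blueprint that runs a timed round and records per-player results when it ends.
; It sets a five-minute match clock on start and round reset, counts it down by seconds in TickTime, and switches the session to AfterRound at zero.
; Entering AfterRound builds RoundStat from each player state's faction, pawn name, kills, deaths, shots, hits and computed accuracy.
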(event `self.ReceiveBeginPlay`
  (`parent.ReceiveBeginPlay`)
  (`self.SetupRoundTime`))

(event `self.ReceiveTick`
  (params (DeltaSeconds :type "Float (single-precision)"))
  (`parent.ReceiveTick` DeltaSeconds))

(event `self.TickTime`
  (bind _output_get (set `self.MatchTime` (- (`self.MatchTime`) (`KismetMathLibrary.MakeTimespan` 0 0 0 1))))
  (`self.TimeChanged` _output_get))

(event `self.OnTimeChanged`
  (params (CurrentTime :type "Timespan Structure"))
  (if (== CurrentTime (`KismetMathLibrary.MakeTimespan` 0))
    (`self.ChangeSessionState` "NewEnumerator2")))

(event `self.OnSessionStateChanged`
  (params (SessionState :type "/Game/Base/Blueprints/E_SessionState Enum" :default "NewEnumerator0"))
  (`|ExecutionSequence`
    (:`then_0`
      (switch `/Game/Base/Blueprints/E_SessionState` SessionState
        (:`NewEnumerator2`
          (`self.CollectRoundStat`))))
    (:`then_1`
      (`parent.OnSessionStateChanged` SessionState))))

(event `self.OnRoundResetted`
  (`parent.OnRoundResetted`)
  (`self.SetupRoundTime`)
  (`self.ChangeSessionState` "NewEnumerator1"))

(fn `CollectRoundStat`
  (for _array_element (`self.PlayerArray`)
    (bind _asbp_player_state_pvp (cast `/Game/Base/Blueprints/BP_PlayerState_PVP` _array_element :!pure true))
    (bind _shots (`/Game/Base/Blueprints/BP_PlayerState_PVP.Shots` _asbp_player_state_pvp))
    (bind _hits (`/Game/Base/Blueprints/BP_PlayerState_PVP.Hits` _asbp_player_state_pvp))
    (`KismetArrayLibrary.Array_Add` (`self.RoundStat`) (make `/Game/Base/Blueprints/S_RoundStat_PVP` (`/Game/Base/Blueprints/BP_PlayerState_PVP.Faction` _asbp_player_state_pvp) (`KismetSystemLibrary.GetDisplayName` (`PlayerState.PawnPrivate` _asbp_player_state_pvp)) (`/Game/Base/Blueprints/BP_PlayerState_PVP.KIlls` _asbp_player_state_pvp) (`/Game/Base/Blueprints/BP_PlayerState_PVP.Deaths` _asbp_player_state_pvp) _shots _hits (`KismetMathLibrary.Round` (* _hits (/ 100.0 (`KismetMathLibrary.Conv_IntToDouble` _shots))))))))

(fn `SetupRoundTime`
  (bind _output_get (set `self.DefaultMatchTime` (`KismetMathLibrary.MakeTimespan` 0 0 5)))
  (set `self.MatchTime` _output_get))

(fn `UserConstructionScript`
  (`parent.UserConstructionScript`))