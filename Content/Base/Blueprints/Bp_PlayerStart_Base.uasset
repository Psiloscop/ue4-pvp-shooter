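; Base player start that spawns players and bots for a faction-based PVP mode, at its own transform.
; SpawnPlayer and RespawnBot possess a new pawn with the passed controller, while SpawnBot creates an AI running BT_Bot.
; Each picks a random Human or Cyborg mesh, writes the faction to the PlayerState and stores the character.
; IsFree reports the start as available when that stored character is invalid.
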(fn `IsFree`
  (returns (Out :type Boolean))
  (return (not (`KismetSystemLibrary.IsValid` (`self.Character`)))))

(fn `RespawnBot`
  (params (Faction :type "/Game/Data/Enums/E_CharacterFaction Enum" :default "NewEnumerator0") (Controller :type "Controller Object Reference"))
  (returns (Out :type "/Game/Blueprints/Characters/BP_Base_Character Object Reference"))
  (bind _returnvalue (`|SpawnActorFromClass` "/Game/Blueprints/Characters/Bot/BP_Bot.BP_Bot_C" (`self.GetTransform`) "Undefined" "OverrideRootScale" null null))
  (`SkinnedMeshComponent.SetSkinnedAssetAndUpdate` (`Character.Mesh` _returnvalue) (`self.SelectSkeletalMeshToSpawn` Faction) true)
  (set `self.Character` _returnvalue)
  (`Controller.Possess` Controller (`self.Character`))
  (set `/Game/Base/Blueprints/BP_PlayerState_PVP.Faction` Faction (cast `/Game/Base/Blueprints/BP_PlayerState_PVP` (`Controller.PlayerState` Controller) :!pure true))
  (return (`self.Character`)))

(fn `SelectSkeletalMeshToSpawn`
  (params (Faction :type "/Game/Data/Enums/E_CharacterFaction Enum" :default "NewEnumerator0"))
  (returns (Out :type "SkeletalMesh Object Reference"))
  (locals (L_SkeletalMesh :type "SkeletalMesh Object Reference"))
  (switch `/Game/Data/Enums/E_CharacterFaction` Faction
    (:`NewEnumerator0`
      (switch `int` (`KismetMathLibrary.RandomIntegerInRange` 1 4)
        (:`1`
          (set `local.L_SkeletalMesh` "/Game/Assets/Characters/MilitaryCharSilver/MW_Style1_Male.MW_Style1_Male"))
        (:`2`
          (set `local.L_SkeletalMesh` "/Game/Assets/Characters/MilitaryCharSilver/MW_Style1_Female.MW_Style1_Female"))
        (:`3`
          (set `local.L_SkeletalMesh` "/Game/Assets/Characters/MilitaryCharDark/MW_Style2_Male.MW_Style2_Male"))
        (:`4`
          (set `local.L_SkeletalMesh` "/Game/Assets/Characters/MilitaryCharDark/MW_Style2_Female.MW_Style2_Female"))))
    (:`NewEnumerator1`
      (switch `int` (`KismetMathLibrary.RandomIntegerInRange` 1 2)
        (:`1`
          (set `local.L_SkeletalMesh` "/Game/Assets/Characters/ProtoCharacters/SK_PrototypeM.SK_PrototypeM"))
        (:`2`
          (set `local.L_SkeletalMesh` "/Game/Assets/Characters/ProtoCharacters/SK_PrototypeF.SK_PrototypeF")))))
  (return (`local.L_SkeletalMesh`)))

(fn `SpawnBot`
  (params (Faction :type "/Game/Data/Enums/E_CharacterFaction Enum" :default "NewEnumerator0"))
  (returns (Out :type "/Game/Blueprints/Characters/BP_Base_Character Object Reference"))
  (bind _returnvalue (`AIBlueprintHelperLibrary.SpawnAIFromClass` "/Game/Blueprints/Characters/Bot/BP_Bot.BP_Bot_C" "/Game/Blueprints/AI/BT_Bot.BT_Bot" (.location (`self.GetTransform`)) (.rotation (`self.GetTransform`))))
  (bind _asbp_base_character (cast `/Game/Blueprints/Characters/BP_Base_Character` _returnvalue :!pure true))
  (`SkinnedMeshComponent.SetSkinnedAssetAndUpdate` (`Character.Mesh` _asbp_base_character) (`self.SelectSkeletalMeshToSpawn` Faction) true)
  (set `self.Character` _asbp_base_character)
  (set `/Game/Base/Blueprints/BP_PlayerState_PVP.Faction` Faction (cast `/Game/Base/Blueprints/BP_PlayerState_PVP` (`Controller.PlayerState` (`Pawn.GetController` _asbp_base_character)) :!pure true))
  (return (`self.Character`)))

(fn `SpawnPlayer`
  (params (Faction :type "/Game/Data/Enums/E_CharacterFaction Enum" :default "NewEnumerator0") (Controller :type "Controller Object Reference"))
  (returns (Out :type "/Game/Blueprints/Characters/BP_Base_Character Object Reference"))
  (bind _returnvalue (`|SpawnActorFromClass` "/Game/Blueprints/Characters/Player/BP_Character.BP_Character_C" (`self.GetTransform`) "Undefined" "OverrideRootScale" null null))
  (`SkinnedMeshComponent.SetSkinnedAssetAndUpdate` (`Character.Mesh` _returnvalue) (`self.SelectSkeletalMeshToSpawn` Faction) true)
  (set `self.Character` _returnvalue)
  (`Controller.Possess` Controller (`self.Character`))
  (set `/Game/Base/Blueprints/BP_PlayerState_PVP.Faction` Faction (cast `/Game/Base/Blueprints/BP_PlayerState_PVP` (`Controller.PlayerState` Controller) :!pure true))
  (return (`self.Character`)))

(fn `UserConstructionScript`)